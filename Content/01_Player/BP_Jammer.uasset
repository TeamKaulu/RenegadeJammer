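; Player-driven Chaos wheeled vehicle with color-coded boosts, drifting and a self-centering spring-arm camera.
; Tick pushes the mesh forward with speed-capped forces instead of throttle, prioritizing green (blue and yellow held together), blue, yellow, then normal acceleration.
; BoostState engages near each boost's top speed and recolors the placeholder character.
; Drift swaps friction on wheels 2 and 3, while speed and RPM feed dashboard materials and a HUD widget.
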(event Custom|InterpsToOriginalRotation
  (bind _returnvalue (Utilities|Time|GetWorldDeltaSeconds))
  (bind _springarm (Variables|Default|GetSpringArm))
  (bind _relativerotation (Variables|/Script/Engine.SceneComponent|GetRelativeRotation _springarm))
  ;[1 1 1] camera realign
  (Transformation|SetRelativeRotation (Variables|Default|GetSpringArm) (Math|Rotator|MakeRotator 0.0 (Math|Interpolation|FInterpTo (.pitch _relativerotation) 0.0 _returnvalue 1.0) (Math|Interpolation|FInterpTo (.yaw _relativerotation) 0.0 _returnvalue 1.0)) false false))

(event EventBeginPlay
  (bind _aschaos_wheeled_vehicle_movement_component (Utilities|Casting|CastToChaosWheeledVehicleMovementComponent (Variables|Default|GetVehicleMovementComponent)))
  (Variables|Default|SetChaos%20Wheeled%20Vehicle%20Movement%20Component _aschaos_wheeled_vehicle_movement_component)
  (bind _returnvalue (UserInterface|CreateWidget "/Game/01_Player/UI/WBP_Speedometer.WBP_Speedometer_C"))
  (bind _output_get (Variables|Default|SetSpeedometer%20UI _returnvalue))
  (UserInterface|Viewport|AddtoViewport _output_get 0)
  (Variables|Default|SetInitialTransform (Transformation|GetWorldTransform (Variables|Character|GetMesh))))

(event EventTick
  (params (DeltaSeconds :type Float%20%28single-precision%29))
  (bind _speedinkmperh (Utilities|GetSpeedinKmPerH))
  (bind _speedinkmperh_2 (Utilities|GetSpeedinKmPerH))
  (bind _speedinkmperh_3 (Utilities|GetSpeedinKmPerH))
  (bind _mesh (Variables|Character|GetMesh))
  (bind _mesh_2 (Variables|Character|GetMesh))
  (bind _maxspeedgreenboost (Variables|Default|GetMaxSpeedGreenBoost))
  (bind _maxspeedsimpleboost (Variables|Default|GetMaxSpeedSimpleBoost))
  (bind _mesh_3 (Variables|Character|GetMesh))
  (bind _maxspeedsimpleboost_2 (Variables|Default|GetMaxSpeedSimpleBoost))
  (bind _mesh_4 (Variables|Character|GetMesh))
  (Development|PrintText (Utilities|Text|ToText(Integer) (Math|Conversions|ToInteger(Byte) (Variables|Default|GetBoostState))))
  (CallFunction|InterpstoOriginalRotation)
  (CallFunction|UpdateSpeed/RPM)
  ;[1 1 1] BoostLogic (needs to refactor to improve readability)
  (Utilities|FlowControl|Sequence
    (:then_0
      (bind _shoulduse (CallFunction|ShouldUseGreenBoost))
      (if _shoulduse
        (Utilities|FlowControl|Sequence
          (:then_0
            (if (< _speedinkmperh_3 _maxspeedgreenboost)
              (Physics|AddForce _mesh_2 (* (Math|Vector|Normalize (Math|Vector|GetForwardVector _mesh_2)) (Variables|Default|GetGreenBoostFactor)) "None" true)))
          (:then_1
            (if (> _speedinkmperh_3 (* _maxspeedgreenboost 0.95))
              (Variables|Default|SetBoostState "NewEnumerator3")
              (else
                (Variables|Default|SetBoostState "NewEnumerator0")))
            (CallFunction|ChangeMaterial)))
        (else
          (bind _shoulduse_2 (CallFunction|ShouldUseBlueBoost))
          (if _shoulduse_2
            (Utilities|FlowControl|Sequence
              (:then_0
                (if (< _speedinkmperh _maxspeedsimpleboost_2)
                  (Physics|AddForce _mesh_3 (* (Math|Vector|Normalize (Math|Vector|GetForwardVector _mesh_3)) (Variables|Default|GetSimpleBoostFactor)) "None" true)))
              (:then_1
                (if (> _speedinkmperh (* _maxspeedsimpleboost_2 0.8))
                  (Variables|Default|SetBoostState "NewEnumerator2")
                  (else
                    (Variables|Default|SetBoostState "NewEnumerator0")))
                (CallFunction|ChangeMaterial)))
            (else
              (bind _shoulduse_3 (CallFunction|ShouldUseYellowBoost))
              (if _shoulduse_3
                (Utilities|FlowControl|Sequence
                  (:then_0
                    (if (< _speedinkmperh_2 _maxspeedsimpleboost)
                      (Physics|AddForce _mesh_4 (* (Math|Vector|Normalize (Math|Vector|GetForwardVector _mesh_4)) (Variables|Default|GetSimpleBoostFactor)) "None" true)))
                  (:then_1
                    (if (> _speedinkmperh_2 (* _maxspeedsimpleboost 0.8))
                      (Variables|Default|SetBoostState "NewEnumerator1")
                      (else
                        (Variables|Default|SetBoostState "NewEnumerator0")))
                    (CallFunction|ChangeMaterial)))
                (else
                  (if (Variables|Default|GetAccelerating)
                    (if (< (Utilities|GetSpeedinKmPerH) (Variables|Default|GetMaxSpeedNoBoost))
                      (Physics|AddForce _mesh (* (Math|Vector|Normalize (Math|Vector|GetForwardVector _mesh)) (Variables|Default|GetDefaultAccelerationFactor)) "None" true)))
                  (Variables|Default|SetBoostState "NewEnumerator0")
                  (CallFunction|ChangeMaterial))))))))
    (:then_1
      (if (and (== (Variables|Default|GetBoostAmarillo) (Variables|Default|GetBoostAmarilloMax)) (== (Variables|Default|GetBoostAzul) (Variables|Default|GetBoostAzulMax)))
        (Variables|Default|SetBoostVerde (Variables|Default|GetBoostVerdeMax))))))

(event Input|ActionEvents|InputActionMoveForward
  (params (Key :type Key%20Structure :default "None"))
  ;[1 1 1] Input
  (:Pressed
    (Variables|Default|SetAccelerating true))
  (:Released
    (Variables|Default|SetAccelerating false)))

(event Input|ActionEvents|InputActionYellowBoost
  (params (Key :type Key%20Structure :default "None"))
  ;[1 1 1] Input
  (:Pressed
    (Variables|Default|SetYellowBoost true))
  (:Released
    (Variables|Default|SetYellowBoost false)))

(event Input|ActionEvents|InputActionBlueBoost
  (params (Key :type Key%20Structure :default "None"))
  ;[1 1 1] Input
  (:Pressed
    (Variables|Default|SetBlueBoost true))
  (:Released
    (Variables|Default|SetBlueBoost false)))

(event Input|ActionEvents|InputActionDrift
  (params (Key :type Key%20Structure :default "None"))
  ;[1 1 1] Drift
  (:Pressed
    (bind _aschaos_wheeled_vehicle_movement_component (Utilities|Casting|CastToChaosWheeledVehicleMovementComponent (Variables|Default|GetVehicleMovementComponent)))
    (Class|ChaosWheeledVehicleMovementComponent|SetWheelFrictionMultiplier _aschaos_wheeled_vehicle_movement_component 2 (Variables|Default|GetDriftingWheelFriction))
    (Class|ChaosWheeledVehicleMovementComponent|SetWheelFrictionMultiplier _aschaos_wheeled_vehicle_movement_component 3 (Variables|Default|GetDriftingWheelFriction)))
  (:Released
    (bind _aschaos_wheeled_vehicle_movement_component_2 (Utilities|Casting|CastToChaosWheeledVehicleMovementComponent (Variables|Default|GetVehicleMovementComponent)))
    (Class|ChaosWheeledVehicleMovementComponent|SetWheelFrictionMultiplier _aschaos_wheeled_vehicle_movement_component_2 2 (Variables|Default|GetDefaultWheelFriction))
    (Class|ChaosWheeledVehicleMovementComponent|SetWheelFrictionMultiplier _aschaos_wheeled_vehicle_movement_component_2 3 (Variables|Default|GetDefaultWheelFriction))))

(event Input|AxisEvents|InputAxisLookUp
  (params (AxisValue :type Float%20%28single-precision%29))
  (bind _springarm (Variables|Default|GetSpringArm))
  (bind _returnvalue (Transformation|GetRelativeTransform _springarm))
  (bind (_roll _pitch _yaw) (Math|Rotator|BreakRotator (.rotation _returnvalue)))
  ;[1 1 1] Input
  (Transformation|AddRelativeRotation _springarm (Math|Rotator|MakeRotator 0.0 AxisValue 0.0) false false)
  (Transformation|SetRelativeRotation _springarm (Math|Rotator|MakeRotator _roll (Math|Float|Clamp(Float) _pitch -5e+01 2e+01) _yaw) false false))

(event Input|AxisEvents|InputAxisLookRight
  (params (AxisValue :type Float%20%28single-precision%29))
  ;[1 1 1] Input
  (Transformation|AddRelativeRotation (Variables|Default|GetSpringArm) (Math|Rotator|MakeRotator 0.0 0.0 AxisValue) false false))

(event Input|AxisEvents|InputAxisBreak
  (params (AxisValue :type Float%20%28single-precision%29))
  ;[1 1 1] Input
  (Class|ChaosVehicleMovementComponent|SetBrakeInput (Variables|Default|GetVehicleMovementComponent) AxisValue))

(event Input|AxisEvents|InputAxisMoveRight
  (params (AxisValue :type Float%20%28single-precision%29))
  ;[1 1 1] Input
  (Class|ChaosVehicleMovementComponent|SetSteeringInput (Variables|Default|GetVehicleMovementComponent) AxisValue))

(event Input|KeyboardEvents|DebugKeyP
  (params (Key :type Key%20Structure :default "None") (ActionValue :type Input%20Action%20Value%20Structure))
  ;[1 1 1] Debug
  (:Pressed
    (bind _output_get (Variables|Debug|SetIsCarMeshVisible (not (Variables|Debug|GetIsCarMeshVisible))))
    (Rendering|SetVisibility (Variables|Character|GetMesh) _output_get false)
    (Development|PrintText "Car mesh visibility changed")))

(event Input|KeyboardEvents|DebugKeyR
  (params (Key :type Key%20Structure :default "None") (ActionValue :type Input%20Action%20Value%20Structure))
  ;[1 1 1] Debug
  (:Pressed
    (Transformation|SetWorldTransform (Variables|Character|GetMesh) (Variables|Default|GetInitialTransform) false true)
    (Components|Movement|StopMovementImmediately (Variables|Default|GetVehicleMovementComponent))))

(event Input|GamepadEvents|GamepadSpecialRight
  (params (Key :type Key%20Structure :default "None"))
  (:Pressed
    ;[1 1 1] Debug
    (Transformation|SetWorldTransform (Variables|Character|GetMesh) (Variables|Default|GetInitialTransform) false true)
    (Components|Movement|StopMovementImmediately (Variables|Default|GetVehicleMovementComponent))))

(fn ConstructionScript
  (bind _returnvalue (Rendering|Material|CreateDynamicMaterialInstance (Variables|Character|GetMesh) 3 0 "None" :!class /Script/Engine.PrimitiveComponent))
  (Variables|Default|SetSpeedometer _returnvalue)
  (bind _returnvalue_2 (Rendering|Material|CreateDynamicMaterialInstance (Variables|Character|GetMesh) 4 0 "None" :!class /Script/Engine.PrimitiveComponent))
  (Variables|Default|SetTachometer _returnvalue_2)
  (Rendering|Material|CreateDynamicMaterialInstance (Variables|Character|GetMesh) 2 0 "None" :!class /Script/Engine.PrimitiveComponent))

(fn UpdateSpeed/RPM
  (bind _vehiclemovementcomponent (Variables|Default|GetVehicleMovementComponent))
  (bind _chaos_wheeled_vehicle_movement_component (Variables|Default|GetChaos%20Wheeled%20Vehicle%20Movement%20Component))
  (bind _returnvalue (Vehicle|GetForwardSpeed _vehiclemovementcomponent))
  (bind _returnvalue_2 (Class|ChaosWheeledVehicleMovementComponent|GetEngineRotationSpeed _chaos_wheeled_vehicle_movement_component))
  (bind _returnvalue_3 (/ _returnvalue_2 6e+03))
  (bind _returnvalue_4 (* _returnvalue 0.036))
  (bind _returnvalue_5 (/ _returnvalue_4 2.4e+02))
  (bind _returnvalue_6 (Math|Float|Absolute(Float) _returnvalue_5))
  (Rendering|Material|SetScalarParameterValue (Variables|Default|GetSpeedometer) "Value" _returnvalue_6 :!class /Script/Engine.MaterialInstanceDynamic)
  (Rendering|Material|SetScalarParameterValue (Variables|Default|GetTachometer) "Value" _returnvalue_3 :!class /Script/Engine.MaterialInstanceDynamic)
  (Default|UpdateHUD (Variables|Default|GetSpeedometer%20UI) _returnvalue_6 _returnvalue_3))

(fn SpringArmPitch
  (bind _springarm (Variables|Default|GetSpringArm))
  (bind _relativerotation (Variables|/Script/Engine.SceneComponent|GetRelativeRotation _springarm))
  (if (or (> (.pitch _relativerotation) 0.2) (< (.pitch _relativerotation) -0.5))
    (return false)
    (else
      (Development|PrintString "canPitch")
      (return true))))

(fn VehicleComponentasChaosWheeled
  (bind _aschaos_wheeled_vehicle_movement_component (Utilities|Casting|CastToChaosWheeledVehicleMovementComponent (Variables|Default|GetVehicleMovementComponent)))
  (return _aschaos_wheeled_vehicle_movement_component))

(fn ApplyForwardForce
  (params (NewParam :type Boolean)))

(fn ShouldUseBlueBoost
  (return (Variables|Default|GetBlueBoost)))

(fn ShouldUseGreenBoost
  (return (and (Variables|Default|GetYellowBoost) (Variables|Default|GetBlueBoost))))

(fn ShouldUseYellowBoost
  (return (Variables|Default|GetYellowBoost)))

(fn ChangeMaterial
  (bind _characterplaceholder (Variables|Default|GetCharacterPlaceholder))
  (switch Utilities|FlowControl|Switch|SwitchonE_BoostStateEnum (Variables|Default|GetBoostState)
    (:NewEnumerator0
      (Rendering|Material|SetMaterial _characterplaceholder 0 "/Engine/BasicShapes/BasicShapeMaterial.BasicShapeMaterial"))
    (:NewEnumerator1
      (Rendering|Material|SetMaterial _characterplaceholder 0 "/Game/01_Player/Materials/YellowBoostMaterial.YellowBoostMaterial"))
    (:NewEnumerator2
      (Rendering|Material|SetMaterial _characterplaceholder 0 "/Game/01_Player/Materials/BlueBoostMaterial.BlueBoostMaterial"))
    (:NewEnumerator3
      (Rendering|Material|SetMaterial _characterplaceholder 0 "/Game/01_Player/Materials/GreenBoostMaterial.GreenBoostMaterial"))))