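; Player vehicle Blueprint driven by sphere physics, where a force on a collision sphere moves it along the mesh's forward direction.
; Each tick it lerps current speed toward a max speed that the MoveForward input sets or clears, then applies it as acceleration.
; MoveRight yaws the mesh directly to steer.
; FixRotation only traces downward and prints on a hit without correcting rotation; debug lines and speed printouts aid tuning.
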(event Custom|ApplyForces
  (params (DeltaSeconds :type Float%20%28double-precision%29))
  (bind _charactermesh (Variables|Default|GetCharacterMesh))
  (bind _returnvalue (Transformation|GetWorldLocation _charactermesh))
  ;[1 1 1] Custom events
  (bind _output_get (Variables|State|SetCurrentSpeed (Math|Float|Lerp (Variables|State|GetCurrentSpeed) (Variables|State|GetMaxSpeed) (* DeltaSeconds 5e+01))))
  (Physics|AddForce (Variables|Default|GetSphereCollision) (* (Math|Vector|GetForwardVector (Variables|Default|GetCharacterMesh)) _output_get) "None" true)
  (if (Variables|Default|GetIsDebugging)
    (Rendering|Debug|DrawDebugLine _returnvalue (+ _returnvalue (* (Math|Vector|GetForwardVector (Variables|Default|GetCharacterMesh)) _output_get)) "(R=1.000000,G=0.830686,B=0.000000,A=1.000000)" 0.1 5.0)))

(event Custom|FixRotation
  (bind _charactermesh (Variables|Default|GetCharacterMesh))
  (bind _returnvalue (Physics|GetCenterOfMass _charactermesh "None"))
  (bind _returnvalue_2 (Math|Vector|MakeVector (.x _returnvalue) (.y _returnvalue) (.z _returnvalue)))
  (bind _returnvalue_3 (- (.z _returnvalue) 5e+02))
  (bind _returnvalue_4 (Math|Vector|MakeVector (.x _returnvalue) (.y _returnvalue) _returnvalue_3))
  (if (Variables|Default|GetIsDebugging)
    (Rendering|Debug|DrawDebugLine _returnvalue_2 _returnvalue_4 "(R=0.000000,G=0.000000,B=0.000000,A=1.000000)" 3.0 4.0))
  ;[1 1 1] Custom events
  (bind _returnvalue_5 (Collision|LineTraceByChannel _returnvalue_2 _returnvalue_4 "TraceTypeQuery1" false 0 "None"))
  (if _returnvalue_5
    (Development|PrintText "Ouch" true true "(R=1.000000,G=0.000000,B=0.021420,A=1.000000)")))

(event EventTick
  (params (DeltaSeconds :type Float%20%28single-precision%29))
  (bind _charactermesh (Variables|Default|GetCharacterMesh))
  (bind _returnvalue (Transformation|GetWorldLocation _charactermesh))
  ;[1 1 1] Main events
  (CallFunction|FixRotation)
  (CallFunction|ApplyForces DeltaSeconds)
  (Development|PrintText (Utilities|Text|ToText(String) (Utilities|String|Append "CurrentSpeed: " (Utilities|String|ToString(Float) (Variables|State|GetCurrentSpeed)) ";  MaxSpeed" (Utilities|String|ToString(Float) (Variables|State|GetMaxSpeed)))))
  (Development|PrintText (Utilities|Text|ToText(Float) (Math|Vector|VectorLength (- _returnvalue (Variables|Default|GetLastPosition))) "HalfToEven"))
  (Variables|Default|SetLastPosition _returnvalue))

(event Input|ActionEvents|InputActionMoveForward
  (params (Key :type Key%20Structure :default "None"))
  ;[1 1 1] Input
  (:Pressed
    (Variables|State|SetMaxSpeed (Variables|Movement|GetAcceleration))
    (Variables|State|SetIsAccelerating true))
  (:Released
    (Variables|State|SetMaxSpeed 0.0)
    (Variables|State|SetIsAccelerating false)))

(event Input|AxisEvents|InputAxisMoveRight
  (params (AxisValue :type Float%20%28single-precision%29))
  ;[1 1 1] Input
  (Transformation|AddWorldRotation (Variables|Default|GetCharacterMesh) (Math|Rotator|MakeRotator 0.0 0.0 (* AxisValue (Variables|Movement|GetRotationRate))) false false))

(fn ConstructionScript)