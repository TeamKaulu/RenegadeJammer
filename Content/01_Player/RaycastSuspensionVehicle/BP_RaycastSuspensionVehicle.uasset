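; Player-driven physics vehicle built on one simulated cube with raycast suspension and Enhanced Input controls.
; Each tick, four arrow traces push up by compression ratio and cache surface hits; two of their normals adjust the forward vector for acceleration and braking forces.
; Turning applies torque, while a velocity-scaled lateral counterforce limits sliding, using a separate factor during drift.
; Holding drift charges a forward boost impulse, released on letting go.
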(event Custom|IncrementDriftingBoostFactor
  ;[1 1 1] Input
  (Variables|Physics|SetDriftingImpulseFactor (Math|Float|Clamp(Float) (+ (Variables|Physics|GetDriftingImpulseFactor) 0.1))))

(event Input|EnhancedActionEvents|EnhancedInputActionIA_Accelerate
  (params (ActionValue :type Boolean) (ElapsedSeconds :type Float%20%28double-precision%29) (TriggeredSeconds :type Float%20%28double-precision%29) (InputAction :type Input%20Action%20Object%20Reference :default "/Game/01_Player/RaycastSuspensionVehicle/Input/IA_Accelerate.IA_Accelerate"))
  ;[1 1 1] Input
  (:Triggered
    (Variables|State|SetIsAccelerating true)
    (Physics|ProcessAcceleration))
  (:Completed
    (Variables|State|SetIsAccelerating false)))

(event Input|EnhancedActionEvents|EnhancedInputActionIA_TurnRight
  (params (ActionValue :type Float%20%28double-precision%29) (ElapsedSeconds :type Float%20%28double-precision%29) (TriggeredSeconds :type Float%20%28double-precision%29) (InputAction :type Input%20Action%20Object%20Reference :default "/Game/01_Player/RaycastSuspensionVehicle/Input/IA_TurnRight.IA_TurnRight"))
  ;[1 1 1] Input
  (:Triggered
    (Physics|ProcessTurning ActionValue)))

(event Input|EnhancedActionEvents|EnhancedInputActionIA_Break
  (params (ActionValue :type Boolean) (ElapsedSeconds :type Float%20%28double-precision%29) (TriggeredSeconds :type Float%20%28double-precision%29) (InputAction :type Input%20Action%20Object%20Reference :default "/Game/01_Player/RaycastSuspensionVehicle/Input/IA_Break.IA_Break"))
  ;[1 1 1] Input
  (:Triggered
    (Physics|ProcessBreaking)))

(event Input|EnhancedActionEvents|EnhancedInputActionIA_Drift
  (params (ActionValue :type Boolean) (ElapsedSeconds :type Float%20%28double-precision%29) (TriggeredSeconds :type Float%20%28double-precision%29) (InputAction :type Input%20Action%20Object%20Reference :default "/Game/01_Player/RaycastSuspensionVehicle/Input/IA_Drift.IA_Drift"))
  ;[1 1 1] Input
  (:Started
    (Variables|State|SetIsDrifting true)
    (bind _returnvalue (Utilities|Time|SetTimerbyEvent (delegate Custom|IncrementDriftingBoostFactor) 0.1 true)))
  (:Completed
    (Variables|State|SetIsDrifting false)
    (Utilities|Time|ClearandInvalidateTimerbyHandle _returnvalue)
    (Physics|ApplyDriftingImpulse)
    (Variables|Physics|SetDriftingImpulseFactor 0.0)))

(event EventBeginPlay
  (Setup|SetUpMappingContext)
  (Setup|InitValues))

(event EventTick
  (params (DeltaSeconds :type Float%20%28single-precision%29))
  (Physics|ProcessRaycastSuspension)
  (Physics|ProcessCounterGlidingForce)
  (Setup|DrawDebugInfo))

(event Input|KeyboardEvents|DebugKeyP
  (params (Key :type Key%20Structure :default "None") (ActionValue :type Input%20Action%20Value%20Structure))
  (:Pressed
    (Rendering|ToggleVisibility (Variables|Default|GetPlayerMesh) false)))

(fn ConstructionScript)

(fn ProcessRaycastSuspension
  (bind _suspensionraycastinfo (Variables|Default|GetSuspensionRaycastInfo))
  (Utilities|FlowControl|Sequence
    (:then_0
      (bind (_surfaceimpactpoint _compressionratio _surfaceimpactnormal _hascollided) (Physics|ApplyRaycastSuspensionForce (Variables|Default|GetRaycastArrow1)))
      (if _hascollided
        (LocalVariables|SetNoneCollided false))
      (Utilities|Map|Add _suspensionraycastinfo 1 (Utilities|Struct|MakeS_SuspensionRaycastInfo _surfaceimpactpoint _compressionratio _surfaceimpactnormal)))
    (:then_1
      (bind (_surfaceimpactpoint_2 _compressionratio_2 _surfaceimpactnormal_2 _hascollided_2) (Physics|ApplyRaycastSuspensionForce (Variables|Default|GetRaycastArrow2)))
      (if _hascollided_2
        (LocalVariables|SetNoneCollided false))
      (Utilities|Map|Add _suspensionraycastinfo 3 (Utilities|Struct|MakeS_SuspensionRaycastInfo _surfaceimpactpoint_2 _compressionratio_2 _surfaceimpactnormal_2)))
    (:then_2
      (bind (_surfaceimpactpoint_3 _compressionratio_3 _surfaceimpactnormal_3 _hascollided_3) (Physics|ApplyRaycastSuspensionForce (Variables|Default|GetRaycastArrow3)))
      (if _hascollided_3
        (LocalVariables|SetNoneCollided false))
      (Utilities|Map|Add _suspensionraycastinfo 2 (Utilities|Struct|MakeS_SuspensionRaycastInfo _surfaceimpactpoint_3 _compressionratio_3 _surfaceimpactnormal_3)))
    (:then_3
      (bind (_surfaceimpactpoint_4 _compressionratio_4 _surfaceimpactnormal_4 _hascollided_4) (Physics|ApplyRaycastSuspensionForce (Variables|Default|GetRaycastArrow4)))
      (if _hascollided_4
        (LocalVariables|SetNoneCollided false))
      (Utilities|Map|Add _suspensionraycastinfo 0 (Utilities|Struct|MakeS_SuspensionRaycastInfo _surfaceimpactpoint_4 _compressionratio_4 _surfaceimpactnormal_4))
      (if (LocalVariables|GetNoneCollided)
        (Variables|State|SetIsInAir true)
        (else
          (Variables|State|SetIsInAir false))))))

(fn ProcessAcceleration
  (bind _basephysicscube (Variables|Default|GetBasePhysicsCube))
  (bind _returnvalue (Physics|GetCenterOfMass _basephysicscube "None"))
  (bind _projectedforwardvector (Utils|GetForwardVectorProjectedIntoSurface))
  (Physics|AddForce _basephysicscube (* _projectedforwardvector (Variables|Physics|GetAccelerationForce)) "None" true)
  (Rendering|Debug|DrawDebugArrow _returnvalue (+ _returnvalue (* _projectedforwardvector 5e+02)) 5.0 "(R=1.000000,G=0.944561,B=0.000000,A=1.000000)" 0.0 5.0))

(fn ApplyRaycastSuspensionForce
  (params (Arrow :type Arrow%20Component%20Object%20Reference))
  (bind (_start _end) (Utilities|GetArrowStartandEndPoint Arrow))
  (Rendering|Debug|DrawDebugLine _start _end "(R=1.000000,G=0.009182,B=0.000000,A=1.000000)" 0.0 3.0)
  (bind (_outhit _returnvalue) (Collision|LineTraceByChannel _start _end "TraceTypeQuery1" false 0 "None"))
  (if _returnvalue
    (Rendering|Debug|DrawDebugString _start (Utilities|String|ToString(Float) (Utilities|GetSuspensionRatio (.distance _outhit) (Variables|/Script/Engine.ArrowComponent|GetArrowLength Arrow))) 0 "(R=1.000000,G=1.000000,B=1.000000,A=1.000000)")
    (Class|PrimitiveComponent|AddForceatLocation (Variables|Default|GetBasePhysicsCube) (* (Math|Vector|MakeVector 0.0 0.0 (Variables|Physics|GetSuspensionForce)) (Utilities|GetSuspensionRatio (.distance _outhit) (Variables|/Script/Engine.ArrowComponent|GetArrowLength Arrow))) _start "None")
    (return (.location _outhit) (Utilities|GetSuspensionRatio (.distance _outhit) (Variables|/Script/Engine.ArrowComponent|GetArrowLength Arrow)) (.normal _outhit) true)
    (else
      (return "0, 0, 0" 0.0 "0, 0, 0" false))))

(fn InitValues
  (bind _basephysicscube (Variables|Default|GetBasePhysicsCube))
  (Utilities|FlowControl|Sequence
    (:then_0
      (Class|PrimitiveComponent|SetLinearDamping _basephysicscube (Variables|Physics|GetLinearDamping)))
    (:then_1
      (Class|PrimitiveComponent|SetAngularDamping _basephysicscube (Variables|Physics|GetAngularDamping)))
    (:then_2
      (Class|PrimitiveComponent|SetMassOverrideinKg _basephysicscube "None" (Variables|Physics|GetCubeMass) true))
    (:then_3
      (bind _output_get (Variables|/Script/Engine.ArrowComponent|SetArrowLength (Variables|Default|GetRaycastArrow1) (Variables|Physics|GetSuspensionRaycastLength)))
      (bind _output_get_2 (Variables|/Script/Engine.ArrowComponent|SetArrowLength (Variables|Default|GetRaycastArrow2) _output_get))
      (bind _output_get_3 (Variables|/Script/Engine.ArrowComponent|SetArrowLength (Variables|Default|GetRaycastArrow3) _output_get_2))
      (Variables|/Script/Engine.ArrowComponent|SetArrowLength (Variables|Default|GetRaycastArrow4) _output_get_3))
    (:then_4
      (Class|PrimitiveComponent|SetCenterOfMass (Variables|Default|GetBasePhysicsCube) (Math|Vector|MakeVector 0.0 0.0 (Variables|Physics|GetCenterOfMassZOffset)) "None"))))

(fn DrawDebugInfo
  (bind _basephysicscube (Variables|Default|GetBasePhysicsCube))
  (Rendering|Debug|DrawDebugString (Transformation|GetWorldLocation _basephysicscube) (Utilities|String|Append "Velocity: " (Utilities|String|ToString(Float) (Math|Vector|VectorLength (Transformation|GetComponentVelocity _basephysicscube)))) 0 "(R=1.000000,G=1.000000,B=1.000000,A=1.000000)")
  (Rendering|Debug|DrawDebugSphere (Physics|GetCenterOfMass (Variables|Default|GetBasePhysicsCube) "None") 3.0 12 "(R=1.000000,G=0.293504,B=0.000000,A=1.000000)" 0.0 3.0))

(fn SetUpMappingContext
  (bind _returnvalue (Pawn|GetController))
  (if (Class|GameplayStatics|ObjectIsA _returnvalue "/Script/Engine.PlayerController")
    (bind _asplayer_controller (Utilities|Casting|CastToPlayerController _returnvalue))
    (Utilities|IsValid (PlayerController|LocalPlayerSubsystems|GetEnhancedInputLocalPlayerSubsystem _asplayer_controller)
      (:Is%20Valid
        (Input|AddMappingContext (PlayerController|LocalPlayerSubsystems|GetEnhancedInputLocalPlayerSubsystem _asplayer_controller) "/Game/01_Player/RaycastSuspensionVehicle/Input/IMC_VehicleMappingContext.IMC_VehicleMappingContext" 0 "(bIgnoreAllPressedKeysUntilRelease=True,bForceImmediately=False)")))))

(fn ProcessTurning
  (params (Value :type Float%20%28double-precision%29))
  (Class|PrimitiveComponent|AddTorqueinDegrees (Variables|Default|GetBasePhysicsCube) (Math|Vector|MakeVector 0.0 0.0 (* Value (Variables|Physics|GetTurningAngleFactor))) "None" true))

(fn ProcessBreaking
  (bind _basephysicscube (Variables|Default|GetBasePhysicsCube))
  (bind _returnvalue (Physics|GetCenterOfMass _basephysicscube "None"))
  (bind (_projectedforwardvector _isvalid) (Utils|GetForwardVectorProjectedIntoSurface))
  (if _isvalid
    (Physics|AddForce _basephysicscube (* _projectedforwardvector (* (Variables|Physics|GetBreakingForce) -1.0)) "None" true)
    (Rendering|Debug|DrawDebugArrow _returnvalue (+ _returnvalue (* _projectedforwardvector -5e+02)) 5.0 "(R=1.000000,G=0.944561,B=0.000000,A=1.000000)" 0.0 5.0)))

(fn GetForwardVectorProjectedIntoSurface
  (bind _basephysicscube (Variables|Default|GetBasePhysicsCube))
  (bind _suspensionraycastinfo (Variables|Default|GetSuspensionRaycastInfo))
  (bind (_value _returnvalue) (Utilities|Map|Find _suspensionraycastinfo 1))
  (bind _returnvalue_2 (Math|Vector|GetForwardVector _basephysicscube))
  (bind (_value_2 _returnvalue_3) (Utilities|Map|Find _suspensionraycastinfo 0))
  (if (and _returnvalue_3 _returnvalue)
    (return (- _returnvalue_2 (Math|Vector|DotProduct _returnvalue_2 (Math|Vector|Normalize (+ (.surfaceimpactnormal _value) (.surfaceimpactnormal _value_2))))) true)
    (else
      (return "0, 0, 0" false))))

(fn ProcessCounterGlidingForce
  (bind _basephysicscube (Variables|Default|GetBasePhysicsCube))
  (bind _basephysicscube_2 (Variables|Default|GetBasePhysicsCube))
  (bind _returnvalue (Transformation|GetComponentVelocity _basephysicscube))
  (bind _returnvalue_2 (Math|Vector|GetRightVector _basephysicscube))
  (bind _returnvalue_3 (Math|Vector|VectorLength _returnvalue))
  (bind _angleindegrees (Utilities|GetAngleBetweenVectors _returnvalue _returnvalue_2))
  (bind _returnvalue_4 (Math|Trig|Cos(Degrees) _angleindegrees))
  (if (and (> _returnvalue_4 0.0) (< _returnvalue_4 1.0))
    (LocalVariables|SetCounterForce (* (* _returnvalue_3 -1.0) _returnvalue_2))
    (elif (and (> _returnvalue_4 -1.0) (< _returnvalue_4 0.0))
      (LocalVariables|SetCounterForce (* _returnvalue_3 _returnvalue_2))
      (else
        (LocalVariables|SetCounterForce "0, 0, 0"))))
  (if (Variables|State|GetIsDrifting)
    (Physics|AddForce _basephysicscube_2 (* (LocalVariables|GetCounterForce) (Variables|Physics|GetCounterGlidingForceDriftingFactor)) "None" true)
    (else
      (Physics|AddForce _basephysicscube_2 (* (LocalVariables|GetCounterForce) (Variables|Physics|GetCounterGlidingForceDefaultFactor)) "None" true))))

(fn ApplyDriftingImpulse
  (bind _basephysicscube (Variables|Default|GetBasePhysicsCube))
  (bind _driftingimpulseforce (Variables|Physics|GetDriftingImpulseForce))
  (bind _driftingimpulsefactor (Variables|Physics|GetDriftingImpulseFactor))
  (bind _returnvalue (Math|Vector|GetForwardVector _basephysicscube))
  (bind _returnvalue_2 (* _returnvalue _driftingimpulseforce))
  (bind _returnvalue_3 (* _returnvalue_2 _driftingimpulsefactor))
  (if (not (Variables|State|GetIsDrifting))
    (Physics|AddImpulse _basephysicscube _returnvalue_3 "None" true)
    (Development|PrintString (Utilities|String|Append "Impulse" (Utilities|String|ToString(Vector) _returnvalue_3)))))