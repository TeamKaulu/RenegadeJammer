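; BP_YellowEnergy is an energy pickup that refills the player vehicle's yellow boost (BoostAmarillo).
; On any actor overlap while CanAbsorb is set, it casts player pawn 0 to BP_Vehicle, without checking the overlapping actor, and hides its mesh.
; If boost is below maximum, it adds IncrementoBoostAmarillo, clamped, and destroys itself.
; At full boost, it remains in the world with its mesh hidden.
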(event EventBeginPlay
  (|CallParentFunction) ; This node is disabled and will not be called.\nDrag off pins to build functionality.
)

(event EventTick
  (params (DeltaSeconds :type Float%20%28single-precision%29))
  (|CallParentFunction DeltaSeconds) ; This node is disabled and will not be called.\nDrag off pins to build functionality.
)

(event Collision|EventActorBeginOverlap
  (params (OtherActor :type Actor%20Object%20Reference))
  (if (Variables|Default|GetcanAbsorb)
    (bind _asbp_vehicle (Utilities|Casting|CastToBP_Vehicle (Game|Player|GetPlayerPawn 0)))
    (Development|SetHiddeninGame (Variables|Default|GetStaticMesh) true false)
    (if (< (Variables|/Game/01_Player/BP_Vehicle.BP_Vehicle_C|GetBoostAmarillo _asbp_vehicle) (Variables|/Game/01_Player/BP_Vehicle.BP_Vehicle_C|GetBoostAmarilloMax _asbp_vehicle))
      (Variables|/Game/01_Player/BP_Vehicle.BP_Vehicle_C|SetBoostAmarillo _asbp_vehicle (Math|Float|Clamp(Float) (+ (Variables|/Game/01_Player/BP_Vehicle.BP_Vehicle_C|GetBoostAmarillo _asbp_vehicle) (Variables|Default|GetIncrementoBoostAmarillo)) 0.0 (Variables|/Game/01_Player/BP_Vehicle.BP_Vehicle_C|GetBoostAmarilloMax _asbp_vehicle)))
      (Actor|DestroyActor))))

(fn ConstructionScript
  (|CallParentFunction))