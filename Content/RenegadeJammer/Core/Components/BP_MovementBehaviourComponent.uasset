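; BP_MovementBehaviourComponent is a component that moves its owning actor from a stored start location toward a target point.
; Initialize records the owner's location and sets the play rate of a supplied Timeline to the inverse of MovementDuration.
; UpdateMovement feeds the Path value into VInterpTo as DeltaTime at unit speed, so it acts as a lerp alpha, and sets the location without sweeping.
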(event Custom|Event%20Initialize
  (params (Timeline :type Timeline%20Component%20Object%20Reference))
  (CallFunction|InitializeStartPoint)
  (CallFunction|UpdateTranslationDuration (Variables|Default|GetMovementDuration) Timeline))

(fn UpdateMovement
  (params (Path :type Float%20%28double-precision%29) (TargetPointLocation :type Vector))
  (Transformation|SetActorLocation (Components|GetOwner) (Math|Interpolation|VInterpTo (Variables|Default|GetStartPoint) TargetPointLocation Path 1.0) false false))

(fn UpdateTranslationDuration
  (params (NewMovementDuration :type Float%20%28double-precision%29) (Timeline :type Timeline%20Component%20Object%20Reference))
  (Variables|Default|SetMovementDuration NewMovementDuration)
  (Components|Timeline|SetPlayRate Timeline (/ 1.0 (Variables|Default|GetMovementDuration))))

(fn InitializeStartPoint
  (Variables|Default|SetStartPoint (Transformation|GetActorLocation (Components|GetOwner))))