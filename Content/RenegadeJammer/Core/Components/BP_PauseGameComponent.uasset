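; Component that toggles the game's paused state and manages the pause menu.
; TogglePauseGame flips pause, then on pausing lazily creates and reuses a WBP_Pause widget and shows the mouse cursor, unless told to skip the screen.
; On unpausing, it removes any existing widget and hides the cursor.
; The widget's Continue button is bound back to TogglePauseGame to resume play.
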(event Custom|OnContinueButtonClicked
  (CallFunction|TogglePauseGame false))

(event Custom|TogglePauseGame
  (params (ShouldIgnorePauseScreen :type Boolean))
  (Variables|Default|SetShouldIgnoreScreen ShouldIgnorePauseScreen)
  (Game|SetGamePaused (not (Game|IsGamePaused)))
  (if (Game|IsGamePaused)
    (if (not (Variables|Default|GetShouldIgnoreScreen))
      (Utilities|IsValid (Variables|Default|GetPauseWidget)
        (:Is%20Valid
          (UserInterface|Viewport|AddtoViewport (Variables|Default|GetPauseWidget) 0))
        (:Is%20Not%20Valid
          (bind _returnvalue (UserInterface|CreateWidget "/Game/RenegadeJammer/UserInterface/Screens/WBP_Pause.WBP_Pause_C" (Game|GetPlayerController 0)))
          (bind _output_get (Variables|Default|SetPauseWidget _returnvalue))
          (EventDispatchers|BindEventtoOnContinueButtonClicked _output_get (delegate Custom|OnContinueButtonClicked))
          (UserInterface|Viewport|AddtoViewport _returnvalue 0)))
      (Variables|/Script/Engine.PlayerController|SetbShowMouseCursor (Game|GetPlayerController 0) true)
      (Variables|Default|SetShouldIgnoreScreen false :!label _label))
    (else
      (bind _pausewidget (Variables|Default|GetPauseWidget)
        (:then
          (Widget|RemovefromParent _pausewidget)
          (Variables|/Script/Engine.PlayerController|SetbShowMouseCursor (Game|GetPlayerController 0) false)
          (goto _label))
        (:else)))))