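; BP_VignetteComponent is an actor component that manages a vignette widget for an owning BP_BasePlayerController.
; On BeginPlay it creates WBP_Vignette, adds it to the viewport and opens it, stopping if the owner is not that controller.
; CloseVignette closes the widget with an event callback, and the OnVignetteClosed event broadcasts a dispatcher for other systems.
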(event Custom|Event%20On%20Vignette%20Closed
  (Default|CallOnVignetteClosed))

(event EventBeginPlay
  (bind _asbp_base_player_controller_1 (Utilities|Casting|CastToBP_BasePlayerController (Components|GetOwner)))
  (bind _returnvalue (UserInterface|CreateWidget "/Game/RenegadeJammer/UserInterface/Common/Vignette/WBP_Vignette.WBP_Vignette_C" _asbp_base_player_controller_1))
  (bind _output_get (Variables|Default|SetCurrentVignette _returnvalue))
  (UserInterface|Viewport|AddtoViewport _output_get 2)
  (Default|Open _output_get))

(fn CloseVignette
  (bind _currentvignette (Variables|Default|GetCurrentVignette)
    (:then
      (Default|Close _currentvignette (EventDispatchers|CreateEvent :!event Custom|Event%20On%20Vignette%20Closed)))
    (:else)))