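; Camera manager component that smoothly drives its owner's camera and spring arm, including gamepad look and shake.
; Update functions set targets and speeds, and Tick interpolates FOV, arm length, lag, offset and MPC radial blur toward them.
; Gamepad input swings the arm within pitch/yaw limits and easing recenters it, while trauma-scaled Perlin shake adds timed or endless rotation.
; Looping timers pause data interpolation and recentering once values match their targets.
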(event Input|EnhancedActionEvents|EnhancedInputActionIA_MoveCamera
  (params (ActionValue :type Vector%202D%20Structure) (ElapsedSeconds :type Float%20%28double-precision%29) (TriggeredSeconds :type Float%20%28double-precision%29) (InputAction :type Input%20Action%20Object%20Reference :default "/Game/RenegadeJammer/Core/Input/IA_MoveCamera.IA_MoveCamera"))
  (:Triggered
    (Variables|CameraInput|SetDesiredCameraInput (Class|KismetMathLibrary|ClampAxes2D ActionValue -1.0 1.0)))
  (:Started
    (Variables|CameraInput|SetIsMovingCamera true)
    (Variables|Default|SetShouldStopFixingCamera true))
  (:Canceled
    (Variables|CameraInput|SetIsMovingCamera false :!label _label)
    (Variables|CameraInput|SetDesiredCameraInput "")
    (Variables|Default|SetShouldStopFixingCamera false))
  (:Completed
    (goto _label)))

(event EventTick
  (params (DeltaSeconds :type Float%20%28single-precision%29))
  (CallFunction|ProcessCamera DeltaSeconds)
  (bind _isusinggamepad (Class|BPIController|IsUsingGamepad(Message) (Game|GetPlayerController 0)))
  (CallFunction|FixCamera DeltaSeconds _isusinggamepad)
  (CallFunction|ProcessCameraShake DeltaSeconds))

(event EventBeginPlay
  (bind _returnvalue (Components|GetOwner))
  (bind _returnvalue_2 (Actor|GetComponentbyClass _returnvalue "/Script/Engine.SpringArmComponent"))
  (bind _returnvalue_3 (Actor|GetComponentbyClass _returnvalue "/Script/Engine.CameraComponent"))
  (Utilities|FlowControl|Sequence
    (:then_0
      (Utilities|IsValid _returnvalue_3
        (:Is%20Valid
          (Variables|Default|SetCamera _returnvalue_3))
        (:Is%20Not%20Valid
          (Development|PrintString "Camera Manager: Actor has no camera!")))
      (Utilities|IsValid _returnvalue_2
        (:Is%20Valid
          (Variables|Default|SetSpringArm _returnvalue_2)
          (Utilities|Time|SetTimerbyFunctionName 0 "CheckCameraDataEquality" 2.0 true true)
          (Utilities|Time|SetTimerbyFunctionName 0 "CheckCameraRotationEquality" 2.0 true true))
        (:Is%20Not%20Valid
          (Development|PrintString "Camera Manager: Actor has no spring arm!"))))
    (:then_1
      (bind _output_get (Variables|Default|SetActualCameraData (Utilities|Struct|MakeS_CameraData (select (Utilities|IsValid (Variables|Default|GetCamera)) (Variables|/Script/Engine.CameraComponent|GetFieldOfView (Variables|Default|GetCamera)) 0.0) (select (Utilities|IsValid (Variables|Default|GetSpringArm)) (Variables|/Script/Engine.SpringArmComponent|GetTargetArmLength (Variables|Default|GetSpringArm)) 0.0) (select (Utilities|IsValid (Variables|Default|GetSpringArm)) (Variables|/Script/Engine.SpringArmComponent|GetCameraLagSpeed (Variables|Default|GetSpringArm)) 0.0) (select (Utilities|IsValid (Variables|Default|GetSpringArm)) (Variables|/Script/Engine.SpringArmComponent|GetTargetOffset (Variables|Default|GetSpringArm)) "0, 0, 0"))))
      (Variables|Default|SetTargetCameraData _output_get))))

(fn ProcessCamera
  (params (DeltaSeconds :type Float%20%28double-precision%29))
  (bind _fovinterpspeed (Variables|Default|GetFOVInterpSpeed))
  (bind _actualcameradata (Variables|Default|GetActualCameraData))
  (bind _actualcameradata_2 (Variables|Default|GetActualCameraData))
  (bind _blurinterpspeed (Variables|Default|GetBlurInterpSpeed))
  (bind _targetcameradata (Variables|Default|GetTargetCameraData))
  (bind _targetcameradata_2 (Variables|Default|GetTargetCameraData))
  (bind _returnvalue (Math|Interpolation|FInterpTo (.blurstrength _actualcameradata_2) (.blurstrength _targetcameradata_2) DeltaSeconds _blurinterpspeed))
  (bind _returnvalue_2 (Math|Interpolation|FInterpTo (.fov _actualcameradata) (.fov _targetcameradata) DeltaSeconds _fovinterpspeed))
  (if (not (Variables|Default|GetShouldStopInterpCameraData))
    (Utilities|FlowControl|Sequence
      (:then_0
        (bind _camera (Variables|Default|GetCamera)
          (:then
            (Camera|SetFieldOfView _camera _returnvalue_2)
            (Utilities|Struct|SetmembersinS_CameraData (Variables|Default|GetActualCameraData) _returnvalue_2)
            (if (Variables|Debug|GetDebug)
              (Development|PrintString (Utilities|String|Append "FOV: " (Utilities|String|ToString(Float) _returnvalue_2)))))
          (:else)))
      (:then_1
        (Variables|Default|GetSpringArm
          (:then
            (Utilities|FlowControl|Sequence
              (:then_0
                (bind _output_get (Variables|/Script/Engine.SpringArmComponent|SetTargetArmLength (Variables|Default|GetSpringArm) (Math|Interpolation|FInterpTo (.length (Variables|Default|GetActualCameraData)) (.length (Variables|Default|GetTargetCameraData)) DeltaSeconds (Variables|Default|GetArmLengthInterpSpeed))))
                (Utilities|Struct|SetmembersinS_CameraData (Variables|Default|GetActualCameraData) _output_get)
                (if (Variables|Debug|GetDebug)
                  (Development|PrintString (Utilities|String|Append "Arm Length: " (Utilities|String|ToString(Float) _output_get)))))
              (:then_1
                (bind _output_get_2 (Variables|/Script/Engine.SpringArmComponent|SetCameraLagSpeed (Variables|Default|GetSpringArm) (Math|Interpolation|FInterpTo (.lagspeed (Variables|Default|GetActualCameraData)) (.lagspeed (Variables|Default|GetTargetCameraData)) DeltaSeconds (Variables|Default|GetCameraLagInterpSpeed))))
                (Utilities|Struct|SetmembersinS_CameraData (Variables|Default|GetActualCameraData) _output_get_2)
                (if (Variables|Debug|GetDebug)
                  (Development|PrintString (Utilities|String|Append "Camera lag speed: " (Utilities|String|ToString(Float) _output_get_2)))))
              (:then_2
                (bind _output_get_3 (Variables|/Script/Engine.SpringArmComponent|SetTargetOffset (Variables|Default|GetSpringArm) (Math|Interpolation|VInterpTo (.targetoffset (Variables|Default|GetActualCameraData)) (.targetoffset (Variables|Default|GetTargetCameraData)) DeltaSeconds (Variables|Default|GetOffsetInterpSpeed))))
                (Utilities|Struct|SetmembersinS_CameraData (Variables|Default|GetActualCameraData) _output_get_3)
                (if (Variables|Debug|GetDebug)
                  (Development|PrintString (Utilities|String|Append "Camera offset: " (Utilities|String|ToString(Vector) _output_get_3)))))))
          (:else)))
      (:then_2
        (Rendering|Material|SetScalarParameterValue "/Game/RenegadeJammer/MaterialLibrary/CollectionsParameters/MPC_SpeedEffect.MPC_SpeedEffect" "RadialBlur" _returnvalue :!class /Script/Engine.KismetMaterialLibrary)
        (Utilities|Struct|SetmembersinS_CameraData (Variables|Default|GetActualCameraData) _returnvalue)
        (if (Variables|Debug|GetDebug)
          (Development|PrintString (Utilities|String|Append "Camera offset: " (Utilities|String|ToString(Float) _returnvalue))))))))

(fn UpdateFOV
  (params (New%20FOV :type Float%20%28double-precision%29) (InterpSpeed :type Float%20%28double-precision%29))
  (Utilities|Struct|SetmembersinS_CameraData (Variables|Default|GetTargetCameraData) New%20FOV)
  (Variables|Default|SetFOVInterpSpeed InterpSpeed)
  (Variables|Default|SetShouldStopInterpCameraData false))

(fn UpdateCameraLag
  (params (New%20Camera%20Lag :type Float%20%28double-precision%29) (InterpSpeed :type Float%20%28double-precision%29))
  (Utilities|Struct|SetmembersinS_CameraData (Variables|Default|GetTargetCameraData) New%20Camera%20Lag)
  (Variables|Default|SetCameraLagInterpSpeed InterpSpeed)
  (Variables|Default|SetShouldStopInterpCameraData false))

(fn UpdateCameraOffset
  (params (NewOffset :type Vector) (InterpSpeed :type Float%20%28double-precision%29))
  (Utilities|Struct|SetmembersinS_CameraData (Variables|Default|GetTargetCameraData) NewOffset)
  (Variables|Default|SetOffsetInterpSpeed InterpSpeed)
  (Variables|Default|SetShouldStopInterpCameraData false))

(fn UpdateBlur
  (params (New%20Length :type Float%20%28double-precision%29) (InterpSpeed :type Float%20%28double-precision%29))
  (Utilities|Struct|SetmembersinS_CameraData (Variables|Default|GetTargetCameraData) New%20Length)
  (Variables|Default|SetBlurInterpSpeed InterpSpeed)
  (Variables|Default|SetShouldStopInterpCameraData false))

(fn UpdateLength
  (params (New%20Length :type Float%20%28double-precision%29) (InterpSpeed :type Float%20%28double-precision%29))
  (Utilities|Struct|SetmembersinS_CameraData (Variables|Default|GetTargetCameraData) New%20Length)
  (Variables|Default|SetArmLengthInterpSpeed InterpSpeed)
  (Variables|Default|SetShouldStopInterpCameraData false))

(fn CalculateIsCameraDataEqual
  (params (CameraData :type S%20Camera%20Data%20Structure%20%28by%20ref%29) (OtherCameraData :type S%20Camera%20Data%20Structure%20%28by%20ref%29))
  (bind (_fov _length _lagspeed _targetoffset _blurstrength) (Utilities|Struct|BreakS_CameraData CameraData))
  (bind (_fov_2 _length_2 _lagspeed_2 _targetoffset_2 _blurstrength_2) (Utilities|Struct|BreakS_CameraData OtherCameraData))
  (bind _tolerance (LocalVariables|GetTolerance))
  (return (Math|Boolean|ANDBoolean (CallFunction|IsFloatNearlyEqual _fov _fov_2 _tolerance) (CallFunction|IsFloatNearlyEqual _length _length_2 _tolerance) (CallFunction|IsFloatNearlyEqual _lagspeed _lagspeed_2 _tolerance) (Utilities|Operators|EqualEqual _targetoffset _targetoffset_2 _tolerance) (CallFunction|IsFloatNearlyEqual _blurstrength _blurstrength_2 _tolerance))))

(fn UpdateCameraData
  (params (NewCameraData :type S%20Camera%20Data%20Structure) (FOVInterpSpeed :type Float%20%28double-precision%29) (ArmLengthInterpSpeed :type Float%20%28double-precision%29) (CameraLagInterpSpeed :type Float%20%28double-precision%29) (OffsetInterpSpeed :type Float%20%28double-precision%29) (BlurInterpSpeed :type Float%20%28double-precision%29))
  (Variables|Default|SetTargetCameraData NewCameraData)
  (Utilities|FlowControl|Sequence
    (:then_0
      (Variables|Default|SetCameraLagInterpSpeed CameraLagInterpSpeed))
    (:then_1
      (Variables|Default|SetArmLengthInterpSpeed ArmLengthInterpSpeed))
    (:then_2
      (Variables|Default|SetFOVInterpSpeed FOVInterpSpeed))
    (:then_3
      (Variables|Default|SetOffsetInterpSpeed OffsetInterpSpeed))
    (:then_4
      (Variables|Default|SetBlurInterpSpeed BlurInterpSpeed))
    (:then_5
      (Variables|Default|SetShouldStopInterpCameraData false))))

(fn FixCamera
  (params (DeltaSeconds :type Float%20%28double-precision%29) (IsUsingController :type Boolean))
  (bind _desiredcamerainput (Variables|CameraInput|GetDesiredCameraInput))
  (bind _movingcamerainterpspeed (Variables|CameraInput|GetMovingCameraInterpSpeed))
  (bind _fixingcamerainterpspeed (Variables|CameraInput|GetFixingCameraInterpSpeed))
  (bind _springarm (Variables|Default|GetSpringArm))
  (bind _springarm_2 (Variables|Default|GetSpringArm))
  (bind (_x _y) (Math|Vector2D|BreakVector2D _desiredcamerainput))
  (bind _relativerotation (Variables|/Script/Engine.SceneComponent|GetRelativeRotation _springarm))
  (bind _relativerotation_2 (Variables|/Script/Engine.SceneComponent|GetRelativeRotation _springarm_2))
  (bind _output_get (LocalVariables|SetShouldFreeCamera (and IsUsingController (Variables|CameraInput|GetIsMovingCamera))))
  (if _output_get
    (Transformation|SetRelativeRotation (Variables|Default|GetSpringArm) (Math|Rotator|MakeRotator 0.0 (Math|Interpolation|FInterpTo (.pitch _relativerotation_2) (* _y (Variables|CameraInput|GetMaxAbsolutePitch)) DeltaSeconds _movingcamerainterpspeed) (Math|Interpolation|FInterpTo (.yaw _relativerotation_2) (* _x (Variables|CameraInput|GetMaxAbsoluteYaw)) DeltaSeconds _movingcamerainterpspeed)) false false)
    (elif (not (Variables|Default|GetShouldStopFixingCamera))
      (Transformation|SetRelativeRotation (Variables|Default|GetSpringArm) (Math|Rotator|MakeRotator 0.0 (Math|Interpolation|FInterpTo (.pitch _relativerotation) (Variables|CameraInput|GetDefaultCameraPitch) DeltaSeconds _fixingcamerainterpspeed) (Math|Interpolation|FInterpTo (.yaw _relativerotation) (Variables|CameraInput|GetDefaultCameraYaw) DeltaSeconds _fixingcamerainterpspeed)) false false))))

(fn MoveCamera
  (params (Input :type Vector%202D%20Structure) (DeltaSeconds :type Float%20%28double-precision%29))
  (if (Variables|CameraInput|GetIsMovingCamera)
    (Utilities|FlowControl|Sequence
      (:then_0
        (Transformation|SetRelativeRotation (Variables|Default|GetSpringArm) (Math|Rotator|MakeRotator 0.0 0.0 0.0) false false)))))

(fn PlayCameraShakewithDuration
  (params (Trauma :type Float%20%28double-precision%29) (Duration :type Float%20%28double-precision%29))
  (Variables|CameraShake|SetActualCameraShakeTrauma Trauma)
  (Variables|CameraShake|SetActualCameraShakeDuration Duration)
  (Variables|CameraShake|SetCameraShakeEnabled true))

(fn ProcessCameraShake
  (params (DeltaTime :type Float%20%28double-precision%29))
  (bind _springarm (Variables|Default|GetSpringArm))
  (bind _relativerotation (Variables|/Script/Engine.SceneComponent|GetRelativeRotation _springarm))
  (if (Variables|CameraShake|GetCameraShakeEnabled)
    (if (and (>= (Variables|CameraShake|GetCameraShakeTime) (Variables|CameraShake|GetActualCameraShakeDuration)) (!= (Variables|CameraShake|GetActualCameraShakeDuration) -1.0))
      (Variables|CameraShake|SetCameraShakeEnabled false)
      (Transformation|SetRelativeRotation (Variables|Default|GetSpringArm) "0, 0, 0" false false)
      (Variables|CameraShake|SetCameraShakeTime 0.0)
      (else
        (Variables|CameraShake|SetCameraShakeTime (+ (Variables|CameraShake|GetCameraShakeTime) DeltaTime))
        (Transformation|SetRelativeRotation (Variables|Default|GetSpringArm) (Math|Rotator|MakeRotator (Math|Interpolation|FInterpTo (.roll _relativerotation) (* (Class|KismetMathLibrary|PerlinNoise1D (Math|Random|RandomFloatinRange -1.0 1.0)) (Variables|CameraShake|GetActualCameraShakeTrauma) (select (== (Variables|CameraShake|GetActualCameraShakeDuration) -1.0) 1.0 (/ (- (Variables|CameraShake|GetActualCameraShakeDuration) (Variables|CameraShake|GetCameraShakeTime)) (Variables|CameraShake|GetActualCameraShakeDuration)))) DeltaTime 1e+01) (Math|Interpolation|FInterpTo (.pitch _relativerotation) (+ (* (Class|KismetMathLibrary|PerlinNoise1D (Math|Random|RandomFloatinRange -1.0 1.0)) (Variables|CameraShake|GetActualCameraShakeTrauma) (select (== (Variables|CameraShake|GetActualCameraShakeDuration) -1.0) 1.0 (/ (- (Variables|CameraShake|GetActualCameraShakeDuration) (Variables|CameraShake|GetCameraShakeTime)) (Variables|CameraShake|GetActualCameraShakeDuration)))) (Variables|CameraInput|GetDefaultCameraPitch)) DeltaTime 1e+01) (Math|Interpolation|FInterpTo (.yaw _relativerotation) (+ (* (Class|KismetMathLibrary|PerlinNoise1D (Math|Random|RandomFloatinRange -1.0 1.0)) (Variables|CameraShake|GetActualCameraShakeTrauma) (select (== (Variables|CameraShake|GetActualCameraShakeDuration) -1.0) 1.0 (/ (- (Variables|CameraShake|GetActualCameraShakeDuration) (Variables|CameraShake|GetCameraShakeTime)) (Variables|CameraShake|GetActualCameraShakeDuration)))) (Variables|CameraInput|GetDefaultCameraYaw)) DeltaTime 1e+01)) false false)))))

(fn PlayCameraShake
  (params (Trauma :type Float%20%28double-precision%29))
  (CallFunction|PlayCameraShakewithDuration Trauma -1.0))

(fn StopCameraShake
  (Variables|CameraShake|SetCameraShakeEnabled false)
  (Variables|CameraShake|SetCameraShakeTime 0.0))

(fn CheckCameraDataEquality
  (bind _returnvalue (CallFunction|CalculateIsCameraDataEqual (Variables|Default|GetActualCameraData) (Variables|Default|GetTargetCameraData)))
  (Variables|Default|SetShouldStopInterpCameraData _returnvalue))

(fn CheckCameraRotationEquality
  (bind _springarm (Variables|Default|GetSpringArm))
  (bind _relativerotation (Variables|/Script/Engine.SceneComponent|GetRelativeRotation _springarm))
  (if (not (Variables|CameraInput|GetIsMovingCamera))
    (Variables|Default|SetShouldStopFixingCamera (and (CallFunction|IsFloatNearlyEqual (.pitch _relativerotation) (Variables|CameraInput|GetDefaultCameraPitch) 0.01) (CallFunction|IsFloatNearlyEqual (Variables|CameraInput|GetDefaultCameraYaw) (.yaw _relativerotation) 0.01)))))