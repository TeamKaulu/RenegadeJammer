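; Blue "hard" destructible object, a child Blueprint that extends a parent destructible with boost-gated destruction.
; CanBeDestroyed allows destruction only under Blue or Green boost while the object is active, and rejects No Boost and Yellow Boost.
; Destroy runs the parent logic, then sends a testing-info message identifying which of two deactivation zones the destroyed object belonged to.
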(event EventDestroy
  (bind _deactivationzone (Variables|Default|GetDeactivationZone))
  (|CallParentFunction)
  (if (Utilities|Enum|Equal(Enum) _deactivationzone "NewEnumerator1")
    (Default|CallCommunicateTestingInfo "Destroyed blue hard object - Zone 1")
    (elif (Utilities|Enum|Equal(Enum) _deactivationzone "NewEnumerator2")
      (Default|CallCommunicateTestingInfo "Destroyed blue hard object - Zone 2"))))

(fn ConstructionScript
  (|CallParentFunction))

(fn CanbeDestroyed
  (params (BoostState :type E_BoostStateEnum%20Enum :default "NewEnumerator0"))
  (switch Utilities|FlowControl|Switch|SwitchonE_BoostStateEnum BoostState
    (:NewEnumerator0
      (return false))
    (:NewEnumerator1
      (return false))
    (:NewEnumerator2
      _)
    (:NewEnumerator3
      _))
  (if (Variables|Default|GetIsActive)
    (return true)))