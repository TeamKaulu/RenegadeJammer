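; BP_ThirdZoneTargetBlueObject is a blue target object, destructible only while active and under Blue Boost.
; On BeginPlay it binds to the game mode's difficulty event and maps the four levels to movement durations passed to UpdateTranslationDuration.
; On destruction it notifies the game mode, then runs parent destroy logic.
; Despite its Third Zone name, both game mode hooks are the First Zone ones.
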(event Custom|UpdateDifficulty
  (params (NewDifficulty :type E_FirstZoneDifficulty%20Enum :default "NewEnumerator0"))
  (switch Utilities|FlowControl|Switch|SwitchonE_FirstZoneDifficulty NewDifficulty
    (:NewEnumerator0
      (CallFunction|UpdateTranslationDuration (Variables|Default|GetLevel1MovementDuration)))
    (:NewEnumerator1
      (CallFunction|UpdateTranslationDuration (Variables|Default|GetLevel2MovementDuration)))
    (:NewEnumerator2
      (CallFunction|UpdateTranslationDuration (Variables|Default|GetLevel3MovementDuration)))
    (:NewEnumerator3
      (CallFunction|UpdateTranslationDuration (Variables|Default|GetLevel4MovementDuration)))))

(event EventDestroy
  (Class|BPIDefaultGameMode|OnFirstZoneTargetObjectDestroyed(Message) (Variables|Default|GetGameModeReference))
  (|CallParentFunction))

(event EventBeginPlay
  (|CallParentFunction)
  (bind _asbp_default_game_mode (Utilities|Casting|CastToBP_DefaultGameMode (Game|GetGameMode)))
  (bind _output_get (Variables|Default|SetGameModeReference _asbp_default_game_mode))
  (EventDispatchers|BindEventtoOnFirstZoneDifficultyUpdated _output_get (delegate Custom|UpdateDifficulty)))

(fn ConstructionScript
  (|CallParentFunction))

(fn CanbeDestroyed
  (params (BoostState :type E_BoostStateEnum%20Enum :default "NewEnumerator0"))
  (switch Utilities|FlowControl|Switch|SwitchonE_BoostStateEnum BoostState
    (:NewEnumerator0
      (return false))
    (:NewEnumerator1
      (return false))
    (:NewEnumerator2
      (if (Variables|Default|GetIsActive)
        (return true)))
    (:NewEnumerator3
      (return false))))