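; BP_FirstZoneTargetBlueObject is a blue destructible target in the first zone, with a looping robot animation.
; It binds to the game mode's difficulty event and passes a per-level duration to its movement component's timeline.
; When destroyed, it notifies the game mode, runs parent destruction, switches off the tunnel line through the zone's Material Parameter Collection, and reports testing info.
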(event Custom|UpdateDifficulty
  (params (NewDifficulty :type E_FirstZoneDifficulty%20Enum :default "NewEnumerator0"))
  (Default|UpdateTranslationDuration (Variables|Default|GetMovementBehaviourComponent) (Utilities|Select :Index NewDifficulty :NewEnumerator0 (Variables|Default|GetLevel1MovementDuration) :NewEnumerator1 (Variables|Default|GetLevel2MovementDuration) :NewEnumerator2 (Variables|Default|GetLevel3MovementDuration) :NewEnumerator3 (Variables|Default|GetLevel4MovementDuration)) (Variables|Default|GetMovementTimeline)))

(event EventDestroy
  (Class|BPIDefaultGameMode|OnFirstZoneTargetObjectDestroyed(Message) (Variables|Default|GetGameModeReference))
  (|CallParentFunction)
  ;[1 1 1] Deactivate line tunnel material when player destroy the object
  (CallFunction|UpdateTunnelMaterial (Variables|Default|GetTunnelLine) (Variables|Default|GetTunnelLineValue))
  (Default|CallCommunicateTestingInfo "Destroyed blue easy object - Zone 1"))

(event EventBeginPlay
  (|CallParentFunction)
  (bind _asbp_default_game_mode (Utilities|Casting|CastToBP_DefaultGameMode (Game|GetGameMode)))
  (bind _output_get (Variables|Default|SetGameModeReference _asbp_default_game_mode))
  (EventDispatchers|BindEventtoOnFirstZoneDifficultyUpdated _output_get (delegate Custom|UpdateDifficulty))
  ;[1 1 1] Play Animation
  (Components|Animation|PlayAnimation (Variables|Default|GetSkeletalMesh) "/Game/RenegadeJammer/Art/DestructibleObjects/Flotant/EliceRobot/SM_EliceRobot_Anim_Montage.SM_EliceRobot_Anim_Montage" true))

(fn ConstructionScript
  (|CallParentFunction))

(fn UpdateTunnelMaterial
  (params (ParameterName :type Name) (ParameterValue :type Float%20%28double-precision%29))
  (Rendering|Material|SetScalarParameterValue "/Game/RenegadeJammer/MaterialLibrary/ComicEffect/MPC_Zone01.MPC_Zone01" ParameterName ParameterValue :!class /Script/Engine.KismetMaterialLibrary))