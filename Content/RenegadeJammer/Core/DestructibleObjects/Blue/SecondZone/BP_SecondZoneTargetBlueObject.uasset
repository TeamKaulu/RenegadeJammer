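; BP_SecondZoneTargetBlueObject is a blue destructible target object for the second zone.
; It overrides CanBeDestroyed so that only Blue Boost can destroy it, and only while it is active.
; It caches BP_DefaultGameMode on BeginPlay and, on Destroy, notifies it that a Zone 2 target fell, then runs the parent logic and reports testing info.
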(event EventDestroy
  (Class|BPIDefaultGameMode|OnSecondZoneTargetObjectDestroyed(Message) (Variables|Default|GetGameModeReference))
  (|CallParentFunction)
  (Default|CallCommunicateTestingInfo "Destroyed blue easy object - Zone 2"))

(event EventBeginPlay
  (|CallParentFunction)
  (bind _asbp_default_game_mode (Utilities|Casting|CastToBP_DefaultGameMode (Game|GetGameMode)))
  (Variables|Default|SetGameModeReference _asbp_default_game_mode))

(fn ConstructionScript
  (|CallParentFunction))

(fn CanbeDestroyed
  (params (BoostState :type E_BoostStateEnum%20Enum :default "NewEnumerator0"))
  (switch Utilities|FlowControl|Switch|SwitchonE_BoostStateEnum BoostState
    (:NewEnumerator0
      (return false))
    (:NewEnumerator1
      (return false))
    (:NewEnumerator2
      (if (Variables|Default|GetIsActive)
        (return true)))
    (:NewEnumerator3
      (return false))))