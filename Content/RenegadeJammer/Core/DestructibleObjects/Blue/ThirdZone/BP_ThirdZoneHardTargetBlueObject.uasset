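; Blue hard-target destructible for the third zone that travels along a spline and can only be destroyed by Blue Boost while active.
; On BeginPlay it caches the game mode and runs a timeline, rate-scaled to the completion time and optionally reversed, that maps progress to world locations along the spline.
; On destruction it notifies the game mode, runs the parent logic and logs a testing message.
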(event Custom|PlaySpline
  (bind _spline (Variables|Default|GetSpline))
  (bind _spline_2 (Variables|/Game/RenegadeJammer/Core/Obstacles/BP_SplinePath.BP_SplinePath_C|GetSpline _spline))
  (Variables|Default|GetSpline
    (:then
      ;[1 1 1] Adjust spline play rate
      (Components|Timeline|SetPlayRate (Variables|Default|GetSplineTimeline) (/ 1.0 (Variables|Default|GetTime%20to%20Complete%20Spline)))
      (Utilities|FlowControl|Sequence
        (:then_0
          (if (Variables|Default|GetReverse)
            (bind _path (Timeline|SplineTimeline ReverseFromEnd)
              (:Update
                (Transformation|SetActorLocation (Spline|GetLocationatDistanceAlongSpline _spline_2 (Math|Float|Lerp 0.0 (Spline|GetSplineLength _spline_2) _path) "World") false false)))
            (else
              (Timeline|SplineTimeline PlayFromStart))))
        (:then_1
          (Timeline|SplineTimeline SetNewTime))))
    (:else)))

(event EventDestroy
  (Class|BPIDefaultGameMode|OnThirdZoneHardTargetObjectDestroyed(Message) (Variables|Default|GetGameModeReference))
  (|CallParentFunction)
  (Default|CallCommunicateTestingInfo "Destroyed blue hard object - Zone 3"))

(event EventBeginPlay
  (|CallParentFunction)
  (bind _asbp_default_game_mode (Utilities|Casting|CastToBP_DefaultGameMode (Game|GetGameMode)))
  (Variables|Default|SetGameModeReference _asbp_default_game_mode)
  (CallFunction|PlaySpline))

(fn ConstructionScript
  (|CallParentFunction))

(fn CanbeDestroyed
  (params (BoostState :type E_BoostStateEnum%20Enum :default "NewEnumerator0"))
  (switch Utilities|FlowControl|Switch|SwitchonE_BoostStateEnum BoostState
    (:NewEnumerator0
      (return false))
    (:NewEnumerator1
      (return false))
    (:NewEnumerator2
      (if (Variables|Default|GetIsActive)
        (return true)))
    (:NewEnumerator3
      (return false))))