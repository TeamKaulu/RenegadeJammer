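; BP_ThirdZoneTargetBlueObject is a destructible blue target in Zone 3 that can be destroyed only with Blue Boost while active.
; It extends a parent destructible, overriding the boost check and the destroy event.
; On destruction it notifies BP_DefaultGameMode, sets a scalar in the MPC_Zone03 material parameter collection to switch off emission, and stops its linked fan's rotation.
; It also sends a testing-info message.
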(event EventDestroy
  (Default|OnThirdZoneTargetObjectDestroyed (Variables|Default|GetGameModeReference))
  (|CallParentFunction)
  ;[1 1 1] Deactivate emission when player destroy the object
  (CallFunction|UpdateMaterial (Variables|Default|GetTargetMaterial) (Variables|Default|GetTargetMaterialValue))
  ;[1 1 1] Deactivate blue ventilator rotation
  (CallFunction|DeactivateFanRotation)
  (Default|CallCommunicateTestingInfo "Destroyed blue easy object - Zone 3"))

(event EventBeginPlay
  (|CallParentFunction)
  (bind _asbp_default_game_mode (Utilities|Casting|CastToBP_DefaultGameMode (Game|GetGameMode)))
  (Variables|Default|SetGameModeReference _asbp_default_game_mode))

(fn ConstructionScript
  (|CallParentFunction))

(fn CanbeDestroyed
  (params (BoostState :type E_BoostStateEnum%20Enum :default "NewEnumerator0"))
  (switch Utilities|FlowControl|Switch|SwitchonE_BoostStateEnum BoostState
    (:NewEnumerator0
      (return false))
    (:NewEnumerator1
      (return false))
    (:NewEnumerator2
      (if (Variables|Default|GetIsActive)
        (return true)))
    (:NewEnumerator3
      (return false))))

(fn UpdateMaterial
  (params (ParameterName :type Name) (ParameterValue :type Float%20%28double-precision%29))
  (Rendering|Material|SetScalarParameterValue "/Game/RenegadeJammer/MaterialLibrary/ComicEffect/MPC_Zone03.MPC_Zone03" ParameterName ParameterValue :!class /Script/Engine.KismetMaterialLibrary))

(fn DeactivateFanRotation
  (bind _relatedfan (Variables|Default|GetRelatedFan)
    (:then
      (Components|Activation|Deactivate (Actor|GetComponentbyClass _relatedfan "/Script/Engine.RotatingMovementComponent"))
      (bind _asbp_fan (Utilities|Casting|CastToBP_Fan _relatedfan))
      (Default|DeactivateFan _asbp_fan))
    (:else)))