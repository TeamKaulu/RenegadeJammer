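; Base destructible object that rewards the player with boost when destroyed on overlap.
; Sphere collision caches the player through BPI_Player, then TryDestroyingObject checks the active flag and CanBeDestroyed, which receives boost state and returns true here.
; Destruction triggers vibration, spawns an emitter and hides Sphere and Hoop before the reward is granted.
; The object then either reappears after a respawn timer or is removed.
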(event OnComponentBeginOverlap(SphereCollision)
  (params (OverlappedComponent :type Primitive%20Component%20Object%20Reference) (OtherActor :type Actor%20Object%20Reference) (OtherComp :type Primitive%20Component%20Object%20Reference) (OtherBodyIndex :type Integer) (bFromSweep :type Boolean) (SweepResult :type Hit%20Result%20Structure%20%28by%20ref%29))
  ;[1 1 1] Is the other actor the player?
  (if (Utilities|DoesObjectImplementInterface OtherActor "/Game/RenegadeJammer/Core/Characters/Common/BPI_Player.BPI_Player_C")
    ;[1 1 1] We need to save the player reference to interact with it. To prevent the cast every time the player start overriding, we check if the player reference is already loaded
    (Utilities|IsValid (Utilities|ToObject(Interface) (Variables|Default|GetPlayerReference))
      (:Is%20Valid
        ;[1 1 1] Try once destroying the object. This function makes sure that all conditions are met to destroy the object. It returns the result
        (CallFunction|TryDestroyingObject (Variables|Default|GetPlayerReference)))
      (:Is%20Not%20Valid
        (bind _asbpi_player (Utilities|Casting|CastToBPI_Player OtherActor))
        (bind _output_get (Variables|Default|SetPlayerReference _asbpi_player))
        (CallFunction|TryDestroyingObject _output_get)))))

(event Custom|OnRespawnTimerEnded
  (Development|SetHiddeninGame (Variables|Default|GetSphere) false false)
  (Variables|Default|SetIsActive true))

(event EventOnPreDestroy
  (Default|PlayonDestroyObjectVibration (Variables|Default|GetPlayerReference)))

(event EventDestroy
  (Effects|SpawnEmitteratLocation 0 (Transformation|GetWorldLocation (Variables|Default|GetSphere)))
  (Development|PrintText (Utilities|Text|FormatText "{className} destroyed" (Utilities|GetClassDisplayName (Utilities|GetClass self))))
  (Development|SetHiddeninGame (Variables|Default|GetSphere) true false)
  (Variables|Default|SetIsActive false)
  (if (Variables|Respawn|GetShouldRespawn)
    (Utilities|Time|SetTimerbyEvent (delegate Custom|OnRespawnTimerEnded) (Variables|Respawn|GetRespawnTime))
    (else
      (Actor|DestroyActor))))

(fn ConstructionScript)

(fn TryDestroyingObject
  (params (PlayerReference :type BPI%20Player%20Interface))
  (bind _booststate (Class|BPIPlayer|GetBoostState(Message) PlayerReference))
  (bind _canbedestroyed (CallFunction|CanbeDestroyed _booststate))
  (if (and _canbedestroyed (Variables|Default|GetIsActive))
    (Utilities|FlowControl|Sequence
      (:then_0
        (CallFunction|OnPreDestroy)
        (CallFunction|Destroy))
      (:then_1
        (Class|BPIPlayer|AddBoostReward(Message) PlayerReference (Variables|Default|GetReward)))
      (:then_2
        (return true)))
    (else
      (return false))))

(fn CanbeDestroyed
  (params (BoostState :type E_BoostStateEnum%20Enum :default "NewEnumerator0"))
  (return true))

(fn GetReward
  (return (Variables|Default|GetReward)))