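; Base Blueprint for a movable destructible object that shuttles back and forth between its starting location and a TargetPoint, when one is valid.
; The Movement timeline's Path value drives VInterpTo as a lerp-style alpha, setting the location without sweep.
; On finish, a FlipFlop alternates reverse and forward playback to loop the motion.
; MovementDuration scales the play rate at BeginPlay and can be changed through UpdateTranslationDuration.
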(event Custom|Replay
  (Utilities|FlowControl|FlipFlop
    (:A
      (bind _path (Timeline|Movement Reverse) ; Movement timeline
        (:Update
          (Transformation|SetActorLocation (Math|Interpolation|VInterpTo (Variables|Default|GetStartPoint) (Transformation|GetActorLocation (Variables|Default|GetTargetPoint)) _path 1.0) false false))
        (:Finished
          (CallFunction|Replay))))
    (:B
      (Timeline|Movement Play))))

(event Custom|UpdateTranslationDuration
  (params (NewDuration :type Float%20%28double-precision%29))
  (Variables|Default|SetMovementDuration NewDuration)
  (Components|Timeline|SetPlayRate (Variables|Default|GetMovement) (/ 1.0 (Variables|Default|GetMovementDuration))))

(event EventBeginPlay
  (bind _movement (Variables|Default|GetMovement))
  (|CallParentFunction)
  (Utilities|IsValid (Variables|Default|GetTargetPoint)
    (:Is%20Valid
      (Variables|Default|SetStartPoint (Transformation|GetActorLocation))
      (Components|Timeline|SetPlayRate _movement (/ (Components|Animation|GetPlayRate _movement) (Variables|Default|GetMovementDuration)))
      (bind _path (Timeline|Movement Play) ; Movement timeline
        (:Update
          (Transformation|SetActorLocation (Math|Interpolation|VInterpTo (Variables|Default|GetStartPoint) (Transformation|GetActorLocation (Variables|Default|GetTargetPoint)) _path 1.0) false false))
        (:Finished
          (CallFunction|Replay))))))

(fn ConstructionScript
  (|CallParentFunction))