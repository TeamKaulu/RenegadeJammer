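; BP_MovableObjects is an actor, filed under destructible objects, that slides back and forth or along a path from its placed position.
; On BeginPlay it stores its start location, then picks an axis from the actor tag: ObMovX moves it on X, ObMovY on Y.
; Each axis has its own timeline whose scaled curve value is added to the start position every update.
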(event EventBeginPlay
  (Variables|Default|SetIniPosition (Transformation|GetActorLocation))
  (if (Actor|ActorHasTag "ObMovX")
    (bind _movx (Timeline|Timeline Play)
      (:Update
        (Transformation|SetActorLocation (Math|Vector|MakeVector (+ (* _movx 3.0) (.x (Variables|Default|GetIniPosition))) (.y (Variables|Default|GetIniPosition)) (.z (Variables|Default|GetIniPosition))) false false)))
    (elif (Actor|ActorHasTag "ObMovY")
      (bind _movy (Timeline|Timeline_0 Play)
        (:Update
          (Transformation|SetActorLocation (Math|Vector|MakeVector (.x (Variables|Default|GetIniPosition)) (+ (* _movy 3.0) (.y (Variables|Default|GetIniPosition))) (.z (Variables|Default|GetIniPosition))) false false))))))

(event EventTick
  (params (DeltaSeconds :type Float%20%28single-precision%29))
  (|CallParentFunction DeltaSeconds) ; This node is disabled and will not be called.\nDrag off pins to build functionality.
)

(event Collision|EventActorBeginOverlap
  (params (OtherActor :type Actor%20Object%20Reference)))

(fn ConstructionScript
  (|CallParentFunction))