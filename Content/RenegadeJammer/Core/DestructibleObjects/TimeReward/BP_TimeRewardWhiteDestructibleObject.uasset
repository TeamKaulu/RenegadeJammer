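; White time-reward destructible object that can travel along a referenced spline and reports "Time reward achieved" as testing info when destroyed.
; Depending on its play mode, movement starts on BeginPlay or when a BPI_Player actor overlaps the trigger, which then disables its collision.
; A timeline scaled to the completion time moves the actor by distance along the spline.
; The floating bob timeline is configured at construction but never played.
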(event OnComponentBeginOverlap(SplineCollision)
  (params (OverlappedComponent :type Primitive%20Component%20Object%20Reference) (OtherActor :type Actor%20Object%20Reference) (OtherComp :type Primitive%20Component%20Object%20Reference) (OtherBodyIndex :type Integer) (bFromSweep :type Boolean) (SweepResult :type Hit%20Result%20Structure%20%28by%20ref%29))
  (if (and (Utilities|Enum|Equal(Enum) (Variables|Spline|GetPlaySpineMode) "NewEnumerator1") (Utilities|DoesObjectImplementInterface OtherActor "/Game/RenegadeJammer/Core/Characters/Common/BPI_Player.BPI_Player_C"))
    (CallFunction|PlaySpline)
    (CallFunction|DeactivateSplineCollision)))

(event Custom|PlaySpline
  (bind _spline (Variables|Spline|GetSpline))
  (bind _spline_2 (Variables|/Game/RenegadeJammer/Core/Obstacles/BP_SplinePath.BP_SplinePath_C|GetSpline _spline))
  (Variables|Spline|GetSpline
    (:then
      ;[1 1 1] Adjust spline play rate
      (Components|Timeline|SetPlayRate (Variables|Default|GetSplineTimeline) (/ 1.0 (Variables|Spline|GetTimeToCompleteSpline)))
      (bind _path (Timeline|SplineTimeline PlayFromStart)
        (:Update
          (Transformation|SetActorLocation (Spline|GetLocationatDistanceAlongSpline _spline_2 (Math|Float|Lerp 0.0 (Spline|GetSplineLength _spline_2) _path) "World") false false))))
    (:else)))

(event EventBeginPlay
  (|CallParentFunction)
  (CallFunction|InitializeSplinePath))

(event EventDestroy
  (|CallParentFunction)
  (Default|CallCommunicateTestingInfo "Time reward achieved"))

(fn ConstructionScript
  (bind _floatingmovement (Variables|Default|GetFloatingMovement))
  (|CallParentFunction)
  (Components|Timeline|SetPlayRate _floatingmovement (/ (Components|Animation|GetPlayRate _floatingmovement) (Variables|Default|GetFloatingMovementDuration))))

(fn InitializeSplinePath
  (bind _splinecollision (Variables|Default|GetSplineCollision))
  (switch Utilities|FlowControl|Switch|SwitchonE_PlaySplineMode (Variables|Spline|GetPlaySpineMode)
    (:NewEnumerator0
      ;[1 1 1] Play spline mode immediately if mode is OnBeginPlay
      (CallFunction|PlaySpline))
    (:NewEnumerator1
      ;[1 1 1] By default, spline collision is disabled. Activate the collision if mode is OnOverlapTriggerBox
      (Collision|SetCollisionEnabled _splinecollision "QueryOnly")
      (Variables|/Script/Engine.PrimitiveComponent|SetbGenerateOverlapEvents _splinecollision true)
      (Rendering|SetVisibility _splinecollision true false))))

(fn DeactivateSplineCollision
  (bind _splinecollision (Variables|Default|GetSplineCollision))
  (Collision|SetCollisionEnabled _splinecollision "NoCollision")
  (Variables|/Script/Engine.PrimitiveComponent|SetbGenerateOverlapEvents _splinecollision true)
  (Rendering|SetVisibility _splinecollision true false))