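; BP_FirstZoneTargetYellowObject is a moving yellow destructible target in Zone 1 that can be destroyed only while active and under Yellow Boost.
; It binds to the game mode's first-zone difficulty event and sets its translation duration for each of four levels.
; On destruction it notifies the game mode, runs parent logic, switches off a tunnel line's emission through the MPC_Zone01 parameter collection, and reports testing info.
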(event Custom|UpdateDifficulty
  (params (NewDifficulty :type E_FirstZoneDifficulty%20Enum :default "NewEnumerator0"))
  (switch Utilities|FlowControl|Switch|SwitchonE_FirstZoneDifficulty NewDifficulty
    (:NewEnumerator0
      (CallFunction|UpdateTranslationDuration (Variables|Default|GetLevel1MovementDuration)))
    (:NewEnumerator1
      (CallFunction|UpdateTranslationDuration (Variables|Default|GetLevel2MovementDuration)))
    (:NewEnumerator2
      (CallFunction|UpdateTranslationDuration (Variables|Default|GetLevel3MovementDuration)))
    (:NewEnumerator3
      (CallFunction|UpdateTranslationDuration (Variables|Default|GetLevel4MovementDuration)))))

(event EventBeginPlay
  (|CallParentFunction)
  (bind _asbp_default_game_mode (Utilities|Casting|CastToBP_DefaultGameMode (Game|GetGameMode)))
  (bind _output_get (Variables|Default|SetGameModeReference _asbp_default_game_mode))
  (EventDispatchers|BindEventtoOnFirstZoneDifficultyUpdated _output_get (delegate Custom|UpdateDifficulty)))

(event EventDestroy
  (Class|BPIDefaultGameMode|OnFirstZoneTargetObjectDestroyed(Message) (Game|GetGameMode))
  (|CallParentFunction)
  ;[1 1 1] Deactivate line tunnel emission when player destroy the object
  (CallFunction|UpdateTunnelMaterial (Variables|Default|GetTunnelLine) (Variables|Default|GetTunnelLineValue))
  (Default|CallCommunicateTestingInfo "Destroyed yellow easy object - Zone1"))

(fn ConstructionScript
  (|CallParentFunction))

(fn CanbeDestroyed
  (params (BoostState :type E_BoostStateEnum%20Enum :default "NewEnumerator0"))
  (switch Utilities|FlowControl|Switch|SwitchonE_BoostStateEnum BoostState
    (:NewEnumerator0
      (return false))
    (:NewEnumerator1
      (if (Variables|Default|GetIsActive)
        (return true)))
    (:NewEnumerator2
      (return false))
    (:NewEnumerator3
      (return false))))

(fn UpdateTunnelMaterial
  (params (ParameterName :type Name) (ParameterValue :type Float%20%28double-precision%29))
  (Rendering|Material|SetScalarParameterValue "/Game/RenegadeJammer/MaterialLibrary/ComicEffect/MPC_Zone01.MPC_Zone01" ParameterName ParameterValue :!class /Script/Engine.KismetMaterialLibrary))