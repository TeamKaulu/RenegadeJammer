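; Second-zone yellow destructible target that disables an obstacle when destroyed, extending a parent destructible object.
; It can only be destroyed under Yellow Boost while active.
; It binds to the game mode's first-zone difficulty event, shortening its translation duration as the level rises.
; On destruction it notifies the game mode, disables the first BP_BigWaveEmitter02 found in the level and logs testing info.
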(event Custom|UpdateDifficulty
  (params (NewDifficulty :type E_FirstZoneDifficulty%20Enum :default "NewEnumerator0"))
  (switch Utilities|FlowControl|Switch|SwitchonE_FirstZoneDifficulty NewDifficulty
    (:NewEnumerator0
      (CallFunction|UpdateTranslationDuration 3.0))
    (:NewEnumerator1
      (CallFunction|UpdateTranslationDuration 2.5))
    (:NewEnumerator2
      (CallFunction|UpdateTranslationDuration 2.0))
    (:NewEnumerator3
      (CallFunction|UpdateTranslationDuration 1.5))))

(event EventBeginPlay
  (|CallParentFunction)
  (bind _asbp_default_game_mode (Utilities|Casting|CastToBP_DefaultGameMode (Game|GetGameMode)))
  (bind _output_get (Variables|Default|SetGameModeReference _asbp_default_game_mode))
  (EventDispatchers|BindEventtoOnFirstZoneDifficultyUpdated _output_get (delegate Custom|UpdateDifficulty)))

(event EventDestroy
  (Class|BPIDefaultGameMode|OnSecondZoneTargetObjectDestroyed(Message) (Game|GetGameMode))
  (|CallParentFunction)
  (CallFunction|DeactivatePlatform)
  (Default|CallCommunicateTestingInfo "Destroyed yellow easy object - Zone 2"))

(fn ConstructionScript
  (|CallParentFunction))

(fn CanbeDestroyed
  (params (BoostState :type E_BoostStateEnum%20Enum :default "NewEnumerator0"))
  (switch Utilities|FlowControl|Switch|SwitchonE_BoostStateEnum BoostState
    (:NewEnumerator0
      (return false))
    (:NewEnumerator1
      (if (Variables|Default|GetIsActive)
        (return true)))
    (:NewEnumerator2
      (return false))
    (:NewEnumerator3
      (return false))))

(fn DeactivatePlatform
  (bind _outactors (Actor|GetAllActorsOfClass "/Game/RenegadeJammer/Core/Obstacles/BP_BigWaveEmitter02.BP_BigWaveEmitter02_C"))
  (Default|DisableObstacle (Utilities|Array|Get(acopy) _outactors)))