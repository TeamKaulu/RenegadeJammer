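; Zone 3 yellow target destructible, breakable only while active and under Yellow Boost.
; On destruction it notifies the game mode, runs the parent destroy logic and sends a testing-info message.
; It also sets a scalar in the Zone 3 material parameter collection to switch off emission, then stops the linked fan by deactivating its rotating movement and calling DeactivateFan.
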(event EventBeginPlay
  (|CallParentFunction)
  (bind _asbp_default_game_mode (Utilities|Casting|CastToBP_DefaultGameMode (Game|GetGameMode)))
  (Variables|Default|SetGameModeReference _asbp_default_game_mode))

(event EventDestroy
  (Class|BPIDefaultGameMode|OnThirdZoneTargetObjectDestroyed(Message) (Game|GetGameMode))
  (|CallParentFunction)
  ;[1 1 1] Deactivate emission when player destroy objetc
  (CallFunction|UpdateMaterial (Variables|Default|GetTargetMaterial) (Variables|Default|GetTargetMaterialValue))
  ;[1 1 1] Deactivate yellow fan rotation
  (CallFunction|DeactivateFanRotation)
  (Default|CallCommunicateTestingInfo "Destroyed yellow easy object - Zone 3"))

(fn ConstructionScript
  (|CallParentFunction))

(fn CanbeDestroyed
  (params (BoostState :type E_BoostStateEnum%20Enum :default "NewEnumerator0"))
  (switch Utilities|FlowControl|Switch|SwitchonE_BoostStateEnum BoostState
    (:NewEnumerator0
      (return false))
    (:NewEnumerator1
      (if (Variables|Default|GetIsActive)
        (return true)))
    (:NewEnumerator2
      (return false))
    (:NewEnumerator3
      (return false))))

(fn UpdateMaterial
  (params (ParameterName :type Name) (ParameterValue :type Float%20%28double-precision%29))
  (Rendering|Material|SetScalarParameterValue "/Game/RenegadeJammer/MaterialLibrary/ComicEffect/MPC_Zone03.MPC_Zone03" ParameterName ParameterValue :!class /Script/Engine.KismetMaterialLibrary))

(fn DeactivateFanRotation
  (bind _relatedfan (Variables|Default|GetRelatedFan)
    (:then
      (Components|Activation|Deactivate (Actor|GetComponentbyClass _relatedfan "/Script/Engine.RotatingMovementComponent"))
      (bind _asbp_fan (Utilities|Casting|CastToBP_Fan _relatedfan))
      (Default|DeactivateFan _asbp_fan))
    (:else)))