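; Yellow destructible target object for Zone 2 that switches off a wave emitter obstacle when destroyed.
; It overrides CanBeDestroyed so only the Yellow Boost can destroy it, and only while it is active.
; On Destroy it notifies the game mode, runs the parent logic, disables the first BP_BigWaveEmitter02 found in the level and reports a testing message.
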(event EventBeginPlay
  (|CallParentFunction)
  (bind _asbp_default_game_mode (Utilities|Casting|CastToBP_DefaultGameMode (Game|GetGameMode)))
  (Variables|Default|SetGameModeReference _asbp_default_game_mode))

(event EventDestroy
  (Class|BPIDefaultGameMode|OnSecondZoneTargetObjectDestroyed(Message) (Game|GetGameMode))
  (|CallParentFunction)
  (CallFunction|DeactivatePlatform)
  (Default|CallCommunicateTestingInfo "Destroyed yellow easy object - Zone 2"))

(fn ConstructionScript
  (|CallParentFunction))

(fn CanbeDestroyed
  (params (BoostState :type E_BoostStateEnum%20Enum :default "NewEnumerator0"))
  (switch Utilities|FlowControl|Switch|SwitchonE_BoostStateEnum BoostState
    (:NewEnumerator0
      (return false))
    (:NewEnumerator1
      (if (Variables|Default|GetIsActive)
        (return true)))
    (:NewEnumerator2
      (return false))
    (:NewEnumerator3
      (return false))))

(fn DeactivatePlatform
  (bind _outactors (Actor|GetAllActorsOfClass "/Game/RenegadeJammer/Core/Obstacles/BP_BigWaveEmitter02.BP_BigWaveEmitter02_C"))
  (Default|DisableObstacle (Utilities|Array|Get(acopy) _outactors)))