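; BP_TriggerDialogue is a box trigger that opens a dialogue widget with a portrait and sound when a tagged actor overlaps it.
; It can be activated or deactivated, and an optional DoOnce limits it to one firing until reset.
; The widget shows one Dialoge entry, advances once after a delay, and is removed only if the index passes the array length.
; The construction script applies box size and development label text.
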(event OnComponentBeginOverlap(Box)
  (params (OverlappedComponent :type Primitive%20Component%20Object%20Reference) (OtherActor :type Actor%20Object%20Reference) (OtherComp :type Primitive%20Component%20Object%20Reference) (OtherBodyIndex :type Integer) (bFromSweep :type Boolean) (SweepResult :type Hit%20Result%20Structure%20%28by%20ref%29))
  (if (Variables|Components|GetActivado?)
    (if (Actor|ActorHasTag OtherActor (Variables|Default|GetTagTrigger))
      (if (Variables|Default|GetDoOnce)
        (Utilities|FlowControl|DoOnce false
          (:Completed
            _)))
      (CallFunction|ActivateDialogue))))

(event Custom|ResetDoOnce
  ;[1 1 1] Reset DoOnce
  (Utilities|FlowControl|DoOnce false) ; enters at Reset
)

(event Custom|ActivateTrigger
  ;[1 1 1] Activate/Deactivate Trigger
  (CallFunction|ResetDoOnce)
  (Variables|Components|SetActivado? true))

(event Custom|DeactivateTrigger
  ;[1 1 1] Activate/Deactivate Trigger
  (Variables|Components|SetActivado? false))

(event Custom|RemoveWidget
  ;[1 1 1] Dialoge
  (Utilities|IsValid (Variables|Default|GetDialogeWidget)
    (:Is%20Valid
      (Widget|RemovefromParent (Variables|Default|GetDialogeWidget))
      (Variables|Default|SetDialogeWidget 0)
      (Variables|Default|SetDialogeIndex 0)
      (Variables|Default|SetDialogeOpened false)
      (Input|SetInputModeGameOnly (Game|GetPlayerController 0) false))))

(event Custom|ActivateDialogue
  ;[1 1 1] Dialoge
  (Audio|PlaySound2D 0 1.0 1.0 0.0 0 0)
  (if (not (Variables|Default|GetWidget%20Active))
    (if (not (Variables|Default|GetDialogeOpened))
      (bind _returnvalue (UserInterface|CreateWidget "/Game/RenegadeJammer/Core/Dialogue/WBP_Dialoge.WBP_Dialoge_C"))
      (bind _output_get (Variables|Default|SetDialogeWidget _returnvalue))
      (Appearance|SetBrushfromTexture (Variables|/Game/RenegadeJammer/Core/Dialogue/WBP_Dialoge.WBP_Dialoge_C|GetPortrait (Variables|Default|GetDialogeWidget)) (Variables|Default|GetPortraitBrush) false)
      (UserInterface|Viewport|AddtoViewport _output_get 0)
      (Variables|Default|SetDialogeOpened true)
      (Rendering|Components|TextRender|SetText (Variables|/Game/RenegadeJammer/Core/Dialogue/WBP_Dialoge.WBP_Dialoge_C|GetDialogeText (Variables|Default|GetDialogeWidget)) (Utilities|Array|Get(acopy) (Variables|Default|GetDialoge) (Variables|Default|GetDialogeIndex)))
      (Math|Integer|IncrementInt (Variables|Default|GetDialogeIndex)
        (:%20%20
          (Input|SetInputModeGameandUI (Game|GetPlayerController 0) (Variables|Default|GetDialogeWidget) "DoNotLock" true false)
          (Utilities|FlowControl|Delay 5.0)
          (Rendering|Components|TextRender|SetText (Variables|/Game/RenegadeJammer/Core/Dialogue/WBP_Dialoge.WBP_Dialoge_C|GetDialogeText (Variables|Default|GetDialogeWidget)) (Utilities|Array|Get(acopy) (Variables|Default|GetDialoge) (Variables|Default|GetDialogeIndex)))
          (Math|Integer|IncrementInt (Variables|Default|GetDialogeIndex)
            (:%20%20
              (if (> (Variables|Default|GetDialogeIndex) (Utilities|Array|Length (Variables|Default|GetDialoge)))
                (CallFunction|RemoveWidget)))))))))

(fn ConstructionScript
  (Components|Box|SetBoxExtent (Variables|Default|GetBox) (Variables|Default|GetSize) true)
  (Rendering|Components|TextRender|SetText (Variables|Default|GetTextRender) (Variables|Default|GetDevelopmentText)))