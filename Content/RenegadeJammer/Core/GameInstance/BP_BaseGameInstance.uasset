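; Base Game Instance for RenegadeJammer that holds a player ID and the main level name, each exposed through a getter.
; On Init it assigns a random five-digit number as the player ID string, and NewPlayerId rerolls it the same way.
; A ReplayTesting event triggers CallReplay.
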(event EventInit
  (Variables|Default|Setplayer_id (Utilities|String|ToString(Integer) (Math|Random|RandomIntegerinRange 10000 99999))))

(event EventNewPlayerId
  (Variables|Default|Setplayer_id (Utilities|String|ToString(Integer) (Math|Random|RandomIntegerinRange 10000 99999))))

(event EventReplayTesting
  (Default|CallReplay))

(fn GetMainLevelName
  (return (Variables|Default|GetMainLevelName)))

(fn GetPlayerId
  (return (Variables|Default|Getplayer_id)))