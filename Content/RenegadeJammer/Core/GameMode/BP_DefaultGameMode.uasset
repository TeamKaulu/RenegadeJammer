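; Default game mode for RenegadeJammer that runs a timed three-zone match, from optional paused instructions screen to win or loss.
; A looping timer drives the countdown and a speedrun clock; added time extends the former and reduces the latter.
; Per-zone events count destroyed targets to unlock level-Blueprint paths, raise difficulty in zones one and three, and broadcast completion while switching off material-collection light lines.
; It also relays timer, boost and drift updates to the HUD.
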(event Custom|OnTimeRanOut
  (Utilities|FlowControl|Delay (Variables|Timer|GetCourtesyTime))
  (if (not (Variables|State|GetIsGameWon))
    (Class|BPIPlayer|OnLostGame(Message) (Game|Player|GetPlayerPawn 0))
    (Default|LoseGame (Variables|UI|GetUserInterfaceWidget))))

(event Custom|OnInstructionScreenClosed
  (Default|TogglePauseGame (Variables|Default|GetPauseGameComponent) true)
  (CallFunction|StartGame))

(event EventBeginPlay
  (Input|SetInputModeGameandUI (Game|GetPlayerController 0) 0 "DoNotLock" true false)
  (UI|LoadUserInterface (delegate Custom|OnInstructionScreenClosed))
  (if (not (Variables|State|GetShouldShowInstructionsScreen))
    (CallFunction|StartGame)))

(event EventOnThirdZoneTargetObjectDestroyed
  (bind _result (Math|Integer|IncrementInt (Variables|ThirdZone|GetThirdObjectsDestroyed))
    (:%20%20
      (if (== _result (Variables|ThirdZone|GetThird%20Target%20Objects))
        (Default|UnlockFirstZoneEasyPath (Variables|Default|GetThirdZoneLevelBlueprintReference))
        (else
          (Variables|ThirdZone|SetThird%20Zone%20Difficulty (Utilities|Enum|ByteToEnumE_FirstZoneDifficulty (+ (Variables|ThirdZone|GetThird%20Zone%20Difficulty) 1))))))))

(event EventWinGame
  (Variables|State|SetIsGameWon true)
  ;[1 1 1] First of all, we stop the timer
  (Utilities|Time|ClearandInvalidateTimerbyHandle (Variables|Timer|GetTimerTimeHandle))
  (bind _text (Timer|TimetoHumanFriendlyText (Variables|Timer|GetSpeedrunTimer)))
  (Default|SetSpeedrunText (Variables|UI|GetUserInterfaceWidget) _text)
  ;[1 1 1] Tell user interface we won the game!
  (Default|WinGame (Variables|UI|GetUserInterfaceWidget))
  (Pawn|UnPossess (Game|GetPlayerController 0)))

(event EventProcessTimerIteration
  (Variables|Timer|SetSpeedrunTimer (+ (Variables|Timer|GetSpeedrunTimer) (Variables|Timer|GetTimerDelay)))
  (bind _output_get (Variables|Timer|SetCountdownTimer (- (Variables|Timer|GetCountdownTimer) (Variables|Timer|GetTimerDelay))))
  (bind _text (Timer|TimetoHumanFriendlyText _output_get))
  (Default|UpdateTimerText (Variables|UI|GetUserInterfaceWidget) _text)
  (if (<= _output_get 0.0)
    (Variables|Timer|SetCountdownTimer 0.0)
    (CallFunction|OnTimeRanOut)
    (Utilities|Time|ClearandInvalidateTimerbyHandle (Variables|Timer|GetTimerTimeHandle))))

(event EventAddTime
  (params (Seconds :type Float%20%28double-precision%29))
  (Variables|Timer|SetCountdownTimer (+ (Variables|Timer|GetCountdownTimer) Seconds))
  (Default|TimeAddedEvent (Variables|UI|GetUserInterfaceWidget) Seconds)
  (Variables|Timer|SetSpeedrunTimer (- (Variables|Timer|GetSpeedrunTimer) Seconds)))

(event EventLoadFirstLevelReference
  (params (LevelReference :type BPI%20Demo%20Level%20Interface))
  (Variables|Default|SetFirstZoneLevelBlueprintReference LevelReference))

(event EventOnFirstZoneGreenObjectDestroyed
  (Default|CallOnFirstZoneCompleted)
  (Default|UpdateGreenBoostCounter (Variables|UI|GetUserInterfaceWidget))
  ;[1 1 1] Update "0 - Zone" light line
  (Rendering|Material|SetScalarParameterValue "/Game/RenegadeJammer/MaterialLibrary/Lines/MPC_Lines.MPC_Lines" "LineZone01Int" 0.0 :!class /Script/Engine.KismetMaterialLibrary)
  (Variables|FirstZone|SetIsFirstZoneCompleted true))

(event EventOnFirstZoneTargetObjectDestroyed
  (bind _result (Math|Integer|IncrementInt (Variables|FirstZone|GetObjectsDestroyed))
    (:%20%20
      (if (== _result (Variables|FirstZone|GetTargetObjectsNumber))
        (Default|UnlockFirstZoneEasyPath (Variables|Default|GetFirstZoneLevelBlueprintReference))
        (else
          (bind _output_get (Variables|FirstZone|SetFirstZoneDifficulty (Utilities|Enum|ByteToEnumE_FirstZoneDifficulty (+ (Variables|FirstZone|GetFirstZoneDifficulty) 1))))
          (Default|CallOnFirstZoneDifficultyUpdated _output_get))))))

(event EventLoadSecondLevelReference
  (params (LevelReference :type BPI%20Demo%20Level%20Interface))
  (Variables|Default|SetSecondZoneLevelBlueprintReference LevelReference))

(event EventOnSecondZoneTargetObjectDestroyed
  (bind _result (Math|Integer|IncrementInt (Variables|SecondZone|GetSecondObjectsDestroyed))
    (:%20%20
      (if (== _result (Variables|SecondZone|GetSecondTargetObjects))
        (Default|UnlockFirstZoneEasyPath (Variables|Default|GetSecondZoneLevelBlueprintReference))))))

(event EventOnSecondZoneGreenObjectDestroyed
  (Default|CallOnSecondZoneCompleted)
  (Default|UpdateGreenBoostCounter (Variables|UI|GetUserInterfaceWidget))
  ;[1 1 1] Update "0 - Zone" light line
  (Rendering|Material|SetScalarParameterValue "/Game/RenegadeJammer/MaterialLibrary/Lines/MPC_Lines.MPC_Lines" "LineZone02Int" 0.0 :!class /Script/Engine.KismetMaterialLibrary)
  (Variables|SecondZone|SetIsSecondZoneCompleted true))

(event EventLoadThirdLevelReference
  (params (LevelReference :type BPI%20Demo%20Level%20Interface))
  (Variables|Default|SetThirdZoneLevelBlueprintReference LevelReference))

(event EventOnThirdZoneGreenObjectDestroyed
  (Default|CallOnThirdZoneCompleted)
  (Default|UpdateGreenBoostCounter (Variables|UI|GetUserInterfaceWidget))
  ;[1 1 1] Update "0 - Zone" light line
  (Rendering|Material|SetScalarParameterValue "/Game/RenegadeJammer/MaterialLibrary/Lines/MPC_Lines.MPC_Lines" "LineZone03Int" 0.0 :!class /Script/Engine.KismetMaterialLibrary)
  (Variables|ThirdZone|SetIsThirdZoneCompleted true))

(event EventToggleGreenBoostIndicator
  (params (IsActivated :type Boolean) (IsDecrementing :type Boolean))
  (Default|UpdateGreenBoostIndicator (Variables|UI|GetUserInterfaceWidget) IsActivated IsDecrementing))

(event EventUpdateDriftingProgressBarwithCompletedColor
  (params (Percentage :type Float%20%28double-precision%29))
  (bind _userinterfacewidget (Variables|UI|GetUserInterfaceWidget))
  (Default|SetDriftingProgressBarPercentage _userinterfacewidget Percentage)
  (Default|SetDriftingProgressBarColor _userinterfacewidget (Variables|UI|GetCompletedDriftingImpulseProgressBarColor)))

(event EventUpdateBoostAmount
  (params (YellowBoostPercentage :type Float%20%28double-precision%29) (BlueBoostPercentage :type Float%20%28double-precision%29))
  (bind _userinterfacewidget (Variables|UI|GetUserInterfaceWidget))
  (Default|SetYellowBoostProgressBarPercentage _userinterfacewidget YellowBoostPercentage)
  (Default|SetBlueBoostProgressBarPercentage _userinterfacewidget BlueBoostPercentage))

(event EventUpdateDriftingProgressBarwithDefaultColor
  (params (Percentage :type Float%20%28double-precision%29))
  (bind _userinterfacewidget (Variables|UI|GetUserInterfaceWidget))
  (Default|SetDriftingProgressBarPercentage _userinterfacewidget Percentage)
  (Default|SetDriftingProgressBarColor _userinterfacewidget (Variables|UI|GetDefaultDriftingImpulseProgressBarColor)))

(fn ConstructionScript)

(fn StartTimer
  (Variables|Timer|SetCountdownTimer (Variables|Timer|GetLevelTime))
  (bind _returnvalue (Utilities|Time|SetTimerbyFunctionName 0 "ProcessTimerIteration" (Variables|Timer|GetTimerDelay) true))
  (Variables|Timer|SetTimerTimeHandle _returnvalue))

(fn TimetoHumanFriendlyText
  (params (TotalSeconds :type Float%20%28double-precision%29))
  (bind _newparam (Timer|GetIntegerwithTwoDigits (/ TotalSeconds 60)))
  (bind _newparam_2 (Timer|GetIntegerwithTwoDigits (Math|Integer|%(Integer) (Math|Float|Truncate TotalSeconds) 60)))
  (bind _newparam_3 (Timer|GetIntegerwithTwoDigits (Math|Float|Truncate (* (- TotalSeconds (Math|Float|Truncate TotalSeconds)) 1e+02))))
  (return (Utilities|String|Append _newparam ":" _newparam_2 "," _newparam_3)))

(fn GetIntegerwithTwoDigits
  (params (Number :type Integer))
  (bind _returnvalue (Utilities|String|ToString(Integer) Number))
  (if (< Number 10)
    (return (Utilities|String|Append "0" _returnvalue))
    (else
      (return _returnvalue))))

(fn LoadUserInterface
  (params (OnInstructionScreenClosed :type Delegate%20%28by%20ref%29))
  (bind _returnvalue (UserInterface|CreateWidget "/Game/RenegadeJammer/UserInterface/Debug/WBP_UserInterface.WBP_UserInterface_C" (Game|GetPlayerController 0)))
  (bind _output_get (Variables|UI|SetUserInterfaceWidget _returnvalue))
  (UserInterface|Viewport|AddtoViewport _output_get 0)
  (if (Variables|State|GetShouldShowInstructionsScreen)
    (Default|TogglePauseGame (Variables|Default|GetPauseGameComponent) true)
    (bind _returnvalue_2 (UserInterface|CreateWidget "/Game/RenegadeJammer/UserInterface/Debug/WBP_Instruccion.WBP_Instruccion_C" (Game|GetPlayerController 0)))
    (EventDispatchers|BindEventtoOnInstructionScreenClosed _returnvalue_2 OnInstructionScreenClosed)
    (UserInterface|Viewport|AddtoViewport _returnvalue_2 0)))

(fn StartGame
  (Timer|StartTimer)
  (Variables|State|SetHasGameAlreadyStarted true))

(fn GetZonesCompletionState
  (return (Variables|FirstZone|GetIsFirstZoneCompleted) (Variables|SecondZone|GetIsSecondZoneCompleted) (Variables|ThirdZone|GetIsThirdZoneCompleted)))

(fn HasGameStarted
  (return (Variables|State|GetHasGameAlreadyStarted)))