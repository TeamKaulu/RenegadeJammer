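; Game mode for the lobby that provides its guide UI and the name of its exit level.
; LoadUserInterface creates a WBP_Guide widget, adds it to the viewport and passes it the current guide text as the mission.
; GetExitLevelName asks the game instance for the string of a fixed level enum entry and returns it as a Name.
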(fn ConstructionScript
  (|CallParentFunction))

(fn LoadUserInterface
  (bind _returnvalue (UserInterface|CreateWidget "/Game/RenegadeJammer/UserInterface/Tutorial/WBP_Guide.WBP_Guide_C"))
  (UserInterface|Viewport|AddtoViewport _returnvalue 0)
  (Default|ChangeMission _returnvalue (Variables|Default|GetCurrentGuideText)))

(fn GetExitLevelName
  (bind _levelname (Class|BPIGameInstance|GetLevelasString(Message) (Game|GetGameInstance) "NewEnumerator0"))
  (return (Utilities|String|StringToName _levelname)))