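; BP_OnlineGameMode is a game mode that registers the current member with an online league through its ACOnlineManager.
; On BeginPlay it binds a league access server response handler, then calls CreateMember with the manager's current member and league name.
; The handler only writes the success flag and raw response to a text file at a hard-coded developer path.
; LoadUserInterface is an empty stub.
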(event Custom|ManageServerResponse
  (params (Response :type String) (Successful :type Boolean) (OutHeader :type Http%20Header%20Structure) (Status :type serverResponseStatus%20Enum :default "NewEnumerator0") (League :type Array%20of%20S%20Member%20Structures))
  (Class|FileSDKBPLibrary|WriteStringtoFile "C:\\Users\\gaela\\Documents\\GitHub\\RenegadeJammer\\serverResponse.txt" (Utilities|String|Append "Server Response: " (Utilities|String|ToString(Boolean) Successful) " 
" Response) false "AutoDetect"))

(event EventBeginPlay
  (bind _ac_onlinemanager (Variables|Default|GetAC_OnlineManager))
  (|CallParentFunction)
  (EventDispatchers|BindEventtoOnLeagueAccessServerResponse _ac_onlinemanager (delegate Custom|ManageServerResponse))
  (Default|CreateMember _ac_onlinemanager (Variables|/Game/RenegadeJammer/Online/AC_OnlineManager.AC_OnlineManager_C|GetCurrentMember _ac_onlinemanager) (Variables|/Game/RenegadeJammer/Online/AC_OnlineManager.AC_OnlineManager_C|GetLeagueName _ac_onlinemanager)))

(fn ConstructionScript
  (|CallParentFunction))

(fn LoadUserInterface)