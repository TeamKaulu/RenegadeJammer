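; BP_SelectorGameMode is the game mode for the selector screen, providing its UI setup and exit level name.
; LoadUserInterface creates the WBP_SelectorPrincipal widget for the first player, adds it to the viewport, sets Game and UI input focused on that widget, and shows the cursor.
; GetExitLevelName returns "None", and the event graph holds no active logic, so nothing in this Blueprint calls either function.
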(event EventBeginPlay
  (|CallParentFunction) ; This node is disabled and will not be called.\nDrag off pins to build functionality.
)

(event EventTick
  (params (DeltaSeconds :type Float%20%28single-precision%29)))

(fn ConstructionScript
  (|CallParentFunction))

(fn LoadUserInterface
  (bind _returnvalue (Game|GetPlayerController 0))
  (bind _returnvalue_2 (UserInterface|CreateWidget "/Game/RenegadeJammer/UserInterface/Screens/WBP_SelectorPrincipal.WBP_SelectorPrincipal_C" _returnvalue))
  (UserInterface|Viewport|AddtoViewport _returnvalue_2 0)
  (Input|SetInputModeGameandUI _returnvalue (Default|GetDesiredFocusInput _returnvalue_2) "DoNotLock" true false)
  (Variables|/Script/Engine.PlayerController|SetbShowMouseCursor _returnvalue true))

(fn GetExitLevelName
  (return "None"))