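; Tutorial game mode that guides the player through phased missions via a guide widget, with HUD and optional paused instruction screen.
; SwitchPhase sets or completes string-table missions.
; Zone events count destroyed targets to unlock paths or raise difficulty, while green-object kills drive material-collection effects and deactivate zones, though all three flag only the first zone completed.
; A looping countdown timer exists; winning and timeout loss require the completed final-zone phase.
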(event Custom|OnTimeRanOut
  (Utilities|FlowControl|Delay (Variables|Timer|GetCourtesyTime))
  (if (not (Variables|State|GetIsGameWon))
    (Class|BPIPlayer|OnLostGame(Message) (Game|Player|GetPlayerPawn 0))
    (Class|BPIController|OnGameLost(Message) (Game|GetPlayerController 0))
    (Default|CallFinishTesting)))

(event Custom|OnInstructionScreenClosed
  (Game|SetGamePaused false)
  (CallFunction|StartGame))

(event Custom|FinishLevel
  (params (Name :type Name))
  (bind _widgetblueprintguide (Variables|Default|GetWidgetBlueprintGuide))
  (Default|CompleteMission _widgetblueprintguide)
  (Utilities|FlowControl|Delay 5.0)
  (Default|ChangeMission _widgetblueprintguide (Class|KismetStringTableLibrary|GetTableEntrySourceString Name "Back")))

(event EventBeginPlay
  (Utilities|LoadAssetBlocking "/Game/RenegadeJammer/Core/Tutorial/STab_Mission.STab_Mission")
  (UI|LoadUserInterface (delegate Custom|OnInstructionScreenClosed))
  (if (not (Variables|State|GetShouldShowInstructionsScreen))
    (CallFunction|StartGame)))

(event EventWinGame
  (bind _countdowntimer (Variables|Timer|GetCountdownTimer))
  (bind _greenobjectscompleted (Variables|Default|GetGreenObjectsCompleted))
  (bind _text (Timer|TimetoHumanFriendlyText _countdowntimer))
  (if (Utilities|Enum|Equal(Enum) (Variables|Default|GetTutorialPhase) "NewEnumerator13")
    (Variables|State|SetIsGameWon true)
    ;[1 1 1] First of all, we stop the timer
    (Utilities|Time|ClearandInvalidateTimerbyHandle (Variables|Timer|GetTimerTimeHandle))
    ;[1 1 1] Tell game controller we won the game!
    (Class|BPIController|OnGameWon(Message) (Game|GetPlayerController 0) _text _greenobjectscompleted)
    ;[1 1 1] Tell user interface we won the game!
    (Default|OnGameWon (Variables|UI|GetUserInterfaceWidget) _text _greenobjectscompleted)
    (Default|CallFinishTesting)))

(event EventProcessTimerIteration
  (Variables|Timer|SetSpeedrunTimer (+ (Variables|Timer|GetSpeedrunTimer) (Variables|Timer|GetTimerDelay)))
  (bind _output_get (Variables|Timer|SetCountdownTimer (- (Variables|Timer|GetCountdownTimer) (Variables|Timer|GetTimerDelay))))
  (Default|UpdateTimerText (Variables|UI|GetUserInterfaceWidget) (Timer|TimetoHumanFriendlyText _output_get))
  (if (<= _output_get 0.0)
    (if (Utilities|Enum|Equal(Enum) (Variables|Default|GetTutorialPhase) "NewEnumerator13")
      (Variables|Timer|SetCountdownTimer 0.0)
      (CallFunction|OnTimeRanOut)
      (Utilities|Time|ClearandInvalidateTimerbyHandle (Variables|Timer|GetTimerTimeHandle))
      (else
        (Utilities|Time|ClearandInvalidateTimerbyHandle (Variables|Timer|GetTimerTimeHandle))
        (Variables|Timer|SetCountdownTimer 0.0)))))

(event EventAddTime
  (params (Seconds :type Float%20%28double-precision%29))
  (Variables|Timer|SetCountdownTimer (+ (Variables|Timer|GetCountdownTimer) Seconds))
  (Default|OnTimeAdded (Variables|UI|GetUserInterfaceWidget) Seconds)
  (Variables|Timer|SetSpeedrunTimer (- (Variables|Timer|GetSpeedrunTimer) Seconds)))

(event EventLoadFirstLevelReference
  (params (LevelReference :type BPI%20Demo%20Level%20Interface))
  (Variables|Default|SetFirstZoneLevelBlueprintReference LevelReference))

(event EventOnFirstZoneGreenObjectDestroyed
  (Default|CallOnFirstZoneCompleted)
  (Default|UpdateGreenObjectsCounter (Variables|UI|GetUserInterfaceWidget))
  ;[1 1 1] Update "0 - Zone" light line
  (Rendering|Material|SetScalarParameterValue "/Game/RenegadeJammer/MaterialLibrary/Lines/MPC_Lines.MPC_Lines" "LineZone01Int" 0.0 :!class /Script/Engine.KismetMaterialLibrary)
  (Utilities|FlowControl|Sequence
    (:then_0
      ;[1 1 1] Destroy Effect
      ;;[1 1 1] Cupsule Effect
      (bind _flickering (Timeline|Timeline Play)
        (:Update
          (Rendering|Material|SetScalarParameterValue "/Game/RenegadeJammer/MaterialLibrary/Cupule/MPC_Cupule.MPC_Cupule" "EmissiveZone1_Int" _flickering :!class /Script/Engine.KismetMaterialLibrary))))
    (:then_1
      ;;[1 1 1] PostProcessEffect
      (Class|BPIPlayer|DestroyGreenObjectCamEffect(Message) (Game|Player|GetPlayerPawn 0)))
    (:then_2
      (Default|DeactivateZone (Variables|Default|GetFirstZoneLevelBlueprintReference)))
    (:then_3
      (Variables|FirstZone|SetIsFirstZoneCompleted true)
      (Math|Integer|IncrementInt (Variables|Default|GetGreenObjectsCompleted)))))

(event EventOnFirstZoneTargetObjectDestroyed
  (bind _result (Math|Integer|IncrementInt (Variables|FirstZone|GetObjectsDestroyed))
    (:%20%20
      (if (== _result (Variables|FirstZone|GetTargetObjectsNumber))
        (Default|UnlockEasyPath (Variables|Default|GetFirstZoneLevelBlueprintReference))
        (else
          (bind _output_get (Variables|FirstZone|SetFirstZoneDifficulty (Utilities|Enum|ByteToEnumE_FirstZoneDifficulty (+ (Variables|FirstZone|GetFirstZoneDifficulty) 1))))
          (Default|CallOnFirstZoneDifficultyUpdated _output_get))))))

(event EventLoadSecondLevelReference
  (params (LevelReference :type BPI%20Demo%20Level%20Interface))
  (Variables|Default|SetSecondZoneLevelBlueprintReference LevelReference))

(event EventOnSecondZoneTargetObjectDestroyed
  (bind _result (Math|Integer|IncrementInt (Variables|SecondZone|GetSecondObjectsDestroyed))
    (:%20%20
      (if (== _result (Variables|SecondZone|GetSecondTargetObjects))
        (Default|UnlockEasyPath (Variables|Default|GetSecondZoneLevelBlueprintReference))))))

(event EventOnSecondZoneGreenObjectDestroyed
  (Default|CallOnSecondZoneCompleted)
  (Default|UpdateGreenObjectsCounter (Variables|UI|GetUserInterfaceWidget))
  ;[1 1 1] Update "0 - Zone" light line
  (Rendering|Material|SetScalarParameterValue "/Game/RenegadeJammer/MaterialLibrary/Lines/MPC_Lines.MPC_Lines" "LineZone02Int" 0.0 :!class /Script/Engine.KismetMaterialLibrary)
  (Utilities|FlowControl|Sequence
    (:then_0
      ;[1 1 1] Destroy Effect
      ;;[1 1 1] Cupsule Effect
      (bind _flickering (Timeline|Timeline_0 Play)
        (:Update
          (Rendering|Material|SetScalarParameterValue "/Game/RenegadeJammer/MaterialLibrary/Cupule/MPC_Cupule.MPC_Cupule" "EmissiveZone2_Int" _flickering :!class /Script/Engine.KismetMaterialLibrary))))
    (:then_1
      ;;[1 1 1] PostProcessEffect
      (Class|BPIPlayer|DestroyGreenObjectCamEffect(Message) (Game|Player|GetPlayerPawn 0)))
    (:then_2
      (Default|DeactivateZone (Variables|Default|GetSecondZoneLevelBlueprintReference)))
    (:then_3
      (Variables|FirstZone|SetIsFirstZoneCompleted true)
      (Math|Integer|IncrementInt (Variables|Default|GetGreenObjectsCompleted)))))

(event EventOnThirdZoneTargetObjectDestroyed
  (bind _output_get (Variables|ThirdZone|SetThirdEasyPathZoneDifficulty (+ (Variables|ThirdZone|GetThirdEasyPathZoneDifficulty) 1)))
  (Default|CallOnThirdZoneDifficultyUpdated (Utilities|Array|Get(acopy) (Variables|ThirdZone|GetThirdZoneRotationRates) (Math|Conversions|ToInteger(Byte) _output_get)))
  (bind _result (Math|Integer|IncrementInt (Variables|ThirdZone|GetThirdEasyPathObjectsDestroyed))
    (:%20%20
      (if (== _result (Variables|ThirdZone|GetThirdEasyPathTargetObjects))
        (Default|UnlockEasyPath (Variables|Default|GetThirdZoneLevelBlueprintReference))))))

(event EventOnThirdZoneHardTargetObjectDestroyed
  (bind _result (Math|Integer|IncrementInt (Variables|ThirdZone|GetThirdHardPathObjectsDestroyed))
    (:%20%20
      (if (== _result (Variables|ThirdZone|GetThirdHardPathTargetObjects))
        (Default|UnlockHardPath (Variables|Default|GetThirdZoneLevelBlueprintReference))))))

(event EventLoadThirdLevelReference
  (params (LevelReference :type BPI%20Demo%20Level%20Interface))
  (Variables|Default|SetThirdZoneLevelBlueprintReference LevelReference))

(event EventOnThirdZoneGreenObjectDestroyed
  (Default|CallOnThirdZoneCompleted)
  (Default|UpdateGreenObjectsCounter (Variables|UI|GetUserInterfaceWidget))
  ;[1 1 1] Update "0 - Zone" light line
  (Rendering|Material|SetScalarParameterValue "/Game/RenegadeJammer/MaterialLibrary/Lines/MPC_Lines.MPC_Lines" "LineZone03Int" 0.0 :!class /Script/Engine.KismetMaterialLibrary)
  (Utilities|FlowControl|Sequence
    (:then_0
      ;[1 1 1] Destroy Effect
      ;;[1 1 1] Cupsule Effect
      (bind _flickering (Timeline|Timeline_1 Play)
        (:Update
          (Rendering|Material|SetScalarParameterValue "/Game/RenegadeJammer/MaterialLibrary/Cupule/MPC_Cupule.MPC_Cupule" "EmissiveZone3_Int" _flickering :!class /Script/Engine.KismetMaterialLibrary))))
    (:then_1
      ;;[1 1 1] PostProcessEffect
      (Class|BPIPlayer|DestroyGreenObjectCamEffect(Message) (Game|Player|GetPlayerPawn 0)))
    (:then_2
      (Default|DeactivateZone (Variables|Default|GetThirdZoneLevelBlueprintReference)))
    (:then_3
      (Variables|FirstZone|SetIsFirstZoneCompleted true)
      (Math|Integer|IncrementInt (Variables|Default|GetGreenObjectsCompleted)))))

(event EventToggleGreenBoostIndicator
  (params (IsActivated :type Boolean) (IsDecrementing :type Boolean))
  (Default|UpdateGreenBoostIndicator (Variables|UI|GetUserInterfaceWidget) IsActivated IsDecrementing))

(event EventUpdateBoostAmount
  (params (YellowBoostPercentage :type Float%20%28double-precision%29) (BlueBoostPercentage :type Float%20%28double-precision%29))
  (bind _userinterfacewidget (Variables|UI|GetUserInterfaceWidget))
  (Default|SetYellowBoostProgressBarPercentage _userinterfacewidget YellowBoostPercentage)
  (Default|SetBlueBoostProgressBarPercentage _userinterfacewidget BlueBoostPercentage))

(fn ConstructionScript)

(fn StartTimer
  (Variables|Timer|SetCountdownTimer (Variables|Timer|GetLevelTime))
  (bind _returnvalue (Utilities|Time|SetTimerbyFunctionName 0 "ProcessTimerIteration" (Variables|Timer|GetTimerDelay) true))
  (Variables|Timer|SetTimerTimeHandle _returnvalue))

(fn TimetoHumanFriendlyText
  (params (TotalSeconds :type Float%20%28double-precision%29))
  (bind _newparam (Timer|GetIntegerwithTwoDigits (/ TotalSeconds 60)))
  (bind _newparam_2 (Timer|GetIntegerwithTwoDigits (Math|Integer|%(Integer) (Math|Float|Truncate TotalSeconds) 60)))
  (bind _newparam_3 (Timer|GetIntegerwithTwoDigits (Math|Float|Truncate (* (- TotalSeconds (Math|Float|Truncate TotalSeconds)) 1e+02))))
  (return (Utilities|String|Append _newparam ":" _newparam_2 "," _newparam_3)))

(fn GetIntegerwithTwoDigits
  (params (Number :type Integer))
  (bind _returnvalue (Utilities|String|ToString(Integer) Number))
  (if (< Number 10)
    (return (Utilities|String|Append "0" _returnvalue))
    (else
      (return _returnvalue))))

(fn LoadUserInterface
  (params (OnInstructionScreenClosed :type Delegate%20%28by%20ref%29))
  (bind _returnvalue (UserInterface|CreateWidget "/Game/RenegadeJammer/UserInterface/Tutorial/WBP_Guide.WBP_Guide_C"))
  (bind _output_get (Variables|Default|SetWidgetBlueprintGuide _returnvalue))
  (bind _returnvalue_2 (UserInterface|CreateWidget "/Game/RenegadeJammer/UserInterface/Screens/WBP_UserInterface.WBP_UserInterface_C" (Game|GetPlayerController 0)))
  (Variables|UI|SetUserInterfaceWidget _returnvalue_2)
  (UserInterface|Viewport|AddtoViewport _returnvalue_2 0)
  (CallFunction|SwitchPhase "NewEnumerator0")
  (if (Variables|State|GetShouldShowInstructionsScreen)
    (Game|SetGamePaused true)
    (bind _returnvalue_3 (UserInterface|CreateWidget "/Game/RenegadeJammer/UserInterface/Screens/WBP_Instruccion.WBP_Instruccion_C" (Game|GetPlayerController 0)))
    (EventDispatchers|BindEventtoOnInstructionScreenClosed _returnvalue_3 OnInstructionScreenClosed)
    (UserInterface|Viewport|AddtoViewport _returnvalue_3 0)))

(fn StartGame)

(fn SwitchPhase
  (params (Phase :type E_Phases%20Enum :default "NewEnumerator0"))
  (bind _widgetblueprintguide (Variables|Default|GetWidgetBlueprintGuide))
  (bind _widgetblueprintguide_2 (Variables|Default|GetWidgetBlueprintGuide))
  (bind _missionsstringtable (LocalVariables|GetMissionsStringTable))
  (bind _output_get (Variables|Default|SetTutorialPhase Phase))
  (switch Utilities|FlowControl|Switch|SwitchonE_Phases _output_get
    (:NewEnumerator0
      (Default|ChangeMission _widgetblueprintguide_2 (Class|KismetStringTableLibrary|GetTableEntrySourceString (LocalVariables|GetMissionsStringTable) "ColorBoost")))
    (:NewEnumerator1
      (Default|CompleteMission _widgetblueprintguide_2 :!label _label))
    (:NewEnumerator2
      (Default|ChangeMission _widgetblueprintguide_2 (Class|KismetStringTableLibrary|GetTableEntrySourceString (LocalVariables|GetMissionsStringTable) "BeatFirstZone")))
    (:NewEnumerator3
      (goto _label))
    (:NewEnumerator4
      (Default|ChangeMission _widgetblueprintguide_2 (Class|KismetStringTableLibrary|GetTableEntrySourceString (LocalVariables|GetMissionsStringTable) "RampsZone")))
    (:NewEnumerator5
      (goto _label))
    (:NewEnumerator6
      (Default|ChangeMission _widgetblueprintguide (Class|KismetStringTableLibrary|GetTableEntrySourceString (LocalVariables|GetMissionsStringTable) "DriftZone")))
    (:NewEnumerator7
      (goto _label))
    (:NewEnumerator8
      (Default|ChangeMission _widgetblueprintguide (Class|KismetStringTableLibrary|GetTableEntrySourceString (LocalVariables|GetMissionsStringTable) "ObjectsZone")))
    (:NewEnumerator9
      (goto _label))
    (:NewEnumerator10
      (Default|ChangeMission _widgetblueprintguide (Class|KismetStringTableLibrary|GetTableEntrySourceString (LocalVariables|GetMissionsStringTable) "BoostSensibleZone")))
    (:NewEnumerator11
      (goto _label))
    (:NewEnumerator12
      (Default|ChangeMission _widgetblueprintguide (Class|KismetStringTableLibrary|GetTableEntrySourceString _missionsstringtable "FinalZone")))
    (:NewEnumerator13
      (CallFunction|FinishLevel _missionsstringtable))))

(fn GetZonesCompletionState
  (return (Variables|FirstZone|GetIsFirstZoneCompleted) (Variables|SecondZone|GetIsSecondZoneCompleted) (Variables|ThirdZone|GetIsThirdZoneCompleted)))

(fn HasGameStarted
  (return (Variables|State|GetHasGameAlreadyStarted)))

(fn HasPlayerWon
  (return (Variables|State|GetIsGameWon)))