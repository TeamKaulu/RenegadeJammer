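; Expo game mode for Renegade Jammer that runs a timed challenge to destroy a target number of green objects.
; Overrides of the parent's first and second zone destruction events feed one shared counter.
; An elapsed timer counts up to the UI, and AddTime subtracts seconds from it, clamped at zero.
; Reaching the target stops the timer, disables pawn movement, shows the win screen with final time and reveals the cursor.
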(event Custom|AnyGreenObjectDestroyed
  (bind _result (Math|Integer|IncrementInt (Variables|Default|GetGreenObjectsDestroyed))
    (:%20%20
      (if (>= _result (Variables|Default|GetGreenObjectsTarget))
        (Utilities|Time|ClearandInvalidateTimerbyHandle (Variables|Default|GetTimerTimeHandle))
        (CallFunction|OnGameEnded)))))

(event Custom|OnGameEnded
  (Class|BPIPlayer|DisableMovementInput(Message) (Game|Player|GetPlayerPawn 0))
  (Default|OnGameWon (Variables|Default|GetUserInterfaceWidget) (CallFunction|TimetoHumanFriendlyText (Variables|Default|GetCountdownTimer)))
  (Variables|/Script/Engine.PlayerController|SetbShowMouseCursor (Game|GetPlayerController 0) true))

(event EventAddTime
  (params (Seconds :type Float%20%28double-precision%29))
  (if (< (- (Variables|Default|GetCountdownTimer) Seconds) 0.0)
    (Variables|Default|SetCountdownTimer 0.0)
    (else
      (Variables|Default|SetCountdownTimer (- (Variables|Default|GetCountdownTimer) Seconds)))))

(event EventProcessTimerIteration
  (bind _output_get (Variables|Default|SetCountdownTimer (+ (Variables|Default|GetCountdownTimer) (Variables|Default|GetTimerDelay))))
  (Default|UpdateTimerText (Variables|Default|GetUserInterfaceWidget) (CallFunction|TimetoHumanFriendlyText _output_get)))

(event EventOnFirstZoneGreenObjectDestroyed
  (|CallParentFunction)
  (CallFunction|AnyGreenObjectDestroyed))

(event EventOnSecondZoneGreenObjectDestroyed
  (|CallParentFunction)
  (CallFunction|AnyGreenObjectDestroyed))

(fn ConstructionScript
  (|CallParentFunction))