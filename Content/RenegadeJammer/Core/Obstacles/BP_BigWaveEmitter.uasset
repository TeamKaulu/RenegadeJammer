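; BP_BigWaveEmitter is an obstacle emitter that periodically spawns an actor, presumably a big wave, at its own transform.
; It spawns one on BeginPlay, then a looping one-second timer decrements a counter seeded from the Time variable.
; Each tick of that timer writes the count to the VisibleCounter text, and reaching zero resets the counter and spawns the next wave.
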(event Custom|NewWave
  (Game|SpawnActorfromClass "/Game/RenegadeJammer/Core/Obstacles/BP_BigWave.BP_BigWave_C" (Transformation|GetActorTransform) "Undefined" "MultiplyWithRoot" 0 0))

(event Custom|Count
  (bind _result (Math|Integer|DecrementInt (Variables|Default|GetTimeCounter))
    (:%20%20
      (Rendering|Components|TextRender|SetText (Variables|Default|GetVisibleCounter) (Utilities|Text|ToText(Integer) _result))
      (if (== _result 0)
        (Variables|Default|SetTimeCounter (Variables|Default|GetTime))
        (CallFunction|NewWave)))))

(event EventBeginPlay
  (Variables|Default|SetTimeCounter (Variables|Default|GetTime))
  (Utilities|FlowControl|Sequence
    (:then_0
      (CallFunction|NewWave))
    (:then_1
      (Utilities|Time|SetTimerbyEvent (delegate Custom|Count) 1.0 true))))

(event Collision|EventActorBeginOverlap
  (params (OtherActor :type Actor%20Object%20Reference)))

(event EventTick
  (params (DeltaSeconds :type Float%20%28single-precision%29)))

(fn ConstructionScript)