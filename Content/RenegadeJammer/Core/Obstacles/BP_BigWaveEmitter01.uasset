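; BP_BigWaveEmitter01 is an obstacle that periodically spawns a BP_BigWave at its transform with a flamethrower sound.
; It fires on BeginPlay, then a looping one-second timer updates a visible countdown and fires again at zero.
; A timeline, restarted with each timed wave, drives the ProgressBarBlue parameter in MPC_Zone02.
; DisableObstacle clears Activated, so later ticks stop counting and zero that parameter.
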(event Custom|NewWave
  ;[1 1 1] Create new wave
  (Game|SpawnActorfromClass "/Game/RenegadeJammer/Core/Obstacles/BP_BigWave.BP_BigWave_C" (Transformation|GetActorTransform) "Undefined" "MultiplyWithRoot" 0 0)
  (Class|AkGameObject|PostAssociatedAkEvent (Variables|Default|GetPlay_SHOT_Flamethrower1)))

(event Custom|Count
  ;[1 1 1] Check if is activated
  (if (Variables|Activated|GetActivated)
    ;[1 1 1] Substract one second
    (bind _result (Math|Integer|DecrementInt (Variables|Default|GetTimeCounter))
      (:%20%20
        (Rendering|Components|TextRender|SetText (Variables|Default|GetVisibleCounter) (Utilities|Text|ToText(Integer) _result))
        ;[1 1 1] If time end reset timer
        (if (== _result 0)
          (Variables|Default|SetTimeCounter (Variables|Default|GetTime))
          (CallFunction|NewWave)
          ;[1 1 1] Progress Bar animation
          (bind _newtrack_0 (Timeline|Timeline PlayFromStart)
            (:Update
              (Rendering|Material|SetScalarParameterValue "/Game/RenegadeJammer/MaterialLibrary/ComicEffect/MPC_Zone02.MPC_Zone02" "ProgressBarBlue" _newtrack_0 :!class /Script/Engine.KismetMaterialLibrary))))))
    (else
      ;[1 1 1] Deactivate ProgressBar
      (Rendering|Material|SetScalarParameterValue "/Game/RenegadeJammer/MaterialLibrary/ComicEffect/MPC_Zone02.MPC_Zone02" "ProgressBarBlue" 0.0 :!class /Script/Engine.KismetMaterialLibrary))))

(event EventBeginPlay
  ;[1 1 1] Set timer
  (Variables|Default|SetTimeCounter (Variables|Default|GetTime))
  (Utilities|FlowControl|Sequence
    (:then_0
      ;[1 1 1] Create new wave
      (CallFunction|NewWave))
    (:then_1
      (Utilities|Time|SetTimerbyEvent (delegate Custom|Count) 1.0 true))
    (:then_2
      ;[1 1 1] Progress Bar animation
      (bind _newtrack_0 (Timeline|Timeline Play)
        (:Update
          (Rendering|Material|SetScalarParameterValue "/Game/RenegadeJammer/MaterialLibrary/ComicEffect/MPC_Zone02.MPC_Zone02" "ProgressBarBlue" _newtrack_0 :!class /Script/Engine.KismetMaterialLibrary))))))

(event EventDisableObstacle
  ;[1 1 1] Deactivate platform
  (Variables|Activated|SetActivated false))

(fn ConstructionScript)