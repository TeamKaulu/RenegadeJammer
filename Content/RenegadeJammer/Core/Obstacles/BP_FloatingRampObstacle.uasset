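; BP_FloatingRampObstacle is an obstacle whose StaticMesh1, referred to as a sphere in its variables, oscillates sideways along its relative Y axis.
; BeginPlay caches the mesh's starting relative location and starts MoveSphere.
; A Timeline maps its Height track to an offset range either side of that start, keeping X and Z fixed.
; A FlipFlop re-triggered on Finished alternates Play and Reverse for continuous ping-pong motion.
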(event Custom|MoveSphere
  (bind _spherelocation (Variables|Default|GetSphereLocation))
  (bind _sphereyoffset (Variables|Default|GetSphereYOffset))
  (bind _spherelocation_2 (Variables|Default|GetSphereLocation))
  (Utilities|FlowControl|FlipFlop :!label _label
    (:A
      (bind _height (Timeline|Timeline Play)
        (:Update
          (Transformation|SetRelativeLocation (Variables|Default|GetStaticMesh1) (Math|Vector|MakeVector (.x _spherelocation_2) (Math|Float|MapRangeClamped _height 0.0 1.0 (- (.y _spherelocation) _sphereyoffset) (+ (.y _spherelocation) _sphereyoffset)) (.z _spherelocation_2)) false false))
        (:Finished
          (goto _label))))
    (:B
      (Timeline|Timeline Reverse))))

(event EventBeginPlay
  (Variables|Default|SetSphereLocation (Variables|/Script/Engine.SceneComponent|GetRelativeLocation (Variables|Default|GetStaticMesh1)))
  (CallFunction|MoveSphere))

(event EventTick
  (params (DeltaSeconds :type Float%20%28single-precision%29)))

(event Collision|EventActorBeginOverlap
  (params (OtherActor :type Actor%20Object%20Reference)))

(fn ConstructionScript)