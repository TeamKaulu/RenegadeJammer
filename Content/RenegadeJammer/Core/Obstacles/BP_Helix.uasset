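; BP_Helix is a helix obstacle that carries one of four payloads: blue energy, yellow energy, one clock or four clocks.
; Its construction script applies EnergySphereRadius to the collision spheres of the yellow and blue destructible child actors.
; It then switches on HelixType and destroys the unused child actor components, leaving only the chosen energy object or white time-reward destructibles.
; All logic runs at construction, as the event graph is empty.
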(event EventBeginPlay)

(event Collision|EventActorBeginOverlap
  (params (OtherActor :type Actor%20Object%20Reference)))

(event EventTick
  (params (DeltaSeconds :type Float%20%28single-precision%29)))

(fn ConstructionScript
  (bind _asbp_yellow_destructible_object_p (Utilities|Casting|CastToBP_YellowDestructibleObject_P (Variables|/Script/Engine.ChildActorComponent|GetChildActor (Variables|Default|GetBP_YellowDestructibleObject_P))))
  (Components|Sphere|SetSphereRadius (Variables|/Game/RenegadeJammer/Core/DestructibleObjects/Common/BP_BaseDestructibleObject.BP_BaseDestructibleObject_C|GetSphereCollision _asbp_yellow_destructible_object_p) (Variables|Default|GetEnergySphereRadius) true)
  (bind _asbp_blue_destructible_object_p (Utilities|Casting|CastToBP_BlueDestructibleObject_P (Variables|/Script/Engine.ChildActorComponent|GetChildActor (Variables|Default|GetBP_BlueDestructibleObject_P))))
  (Components|Sphere|SetSphereRadius (Variables|/Game/RenegadeJammer/Core/DestructibleObjects/Common/BP_BaseDestructibleObject.BP_BaseDestructibleObject_C|GetSphereCollision _asbp_blue_destructible_object_p) (Variables|Default|GetEnergySphereRadius) true)
  (switch Utilities|FlowControl|Switch|SwitchonE_HelixType (Variables|Default|GetHelixType)
    (:NewEnumerator0
      (Components|DestroyComponent (Variables|Default|GetBP_TimeRewardWhiteDestructibleObject_P1)))
    (:NewEnumerator1
      (Components|DestroyComponent (Variables|Default|GetBP_TimeRewardWhiteDestructibleObject_P2)))
    (:NewEnumerator2
      (Components|DestroyComponent (Variables|Default|GetBP_BlueDestructibleObject_P)))
    (:NewEnumerator4
      (Components|DestroyComponent (Variables|Default|GetBP_YellowDestructibleObject_P)))))