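; Light platform obstacle with five tiles, where a randomly chosen safe tile changes each cycle and the others punish the player.
; A looping timer advances a counter that blinks the unsafe tiles blue, then turns them red and enables their collision boxes.
; Players (BPI_Player) overlapping an active box teleport to the BP_LightPlatformReset actor found at BeginPlay.
; The cycle's last step clears materials and collision, then rerolls the safe index.
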(event OnComponentBeginOverlap(Box1)
  (params (OverlappedComponent :type Primitive%20Component%20Object%20Reference) (OtherActor :type Actor%20Object%20Reference) (OtherComp :type Primitive%20Component%20Object%20Reference) (OtherBodyIndex :type Integer) (bFromSweep :type Boolean) (SweepResult :type Hit%20Result%20Structure%20%28by%20ref%29))
  (bind _returnvalue (Utilities|DoesObjectImplementInterface OtherActor "/Game/RenegadeJammer/Core/Characters/Common/BPI_Player.BPI_Player_C"))
  (Development|PrintString (Utilities|String|ToString(Boolean) _returnvalue))
  (if _returnvalue
    (Transformation|SetActorLocation OtherActor (Transformation|GetActorLocation (Variables|Default|GetResetPlatform)) false true)
    (Development|PrintString "Last Check")))

(event OnComponentBeginOverlap(Box)
  (params (OverlappedComponent :type Primitive%20Component%20Object%20Reference) (OtherActor :type Actor%20Object%20Reference) (OtherComp :type Primitive%20Component%20Object%20Reference) (OtherBodyIndex :type Integer) (bFromSweep :type Boolean) (SweepResult :type Hit%20Result%20Structure%20%28by%20ref%29))
  (bind _returnvalue (Utilities|DoesObjectImplementInterface OtherActor "/Game/RenegadeJammer/Core/Characters/Common/BPI_Player.BPI_Player_C"))
  (Development|PrintString (Utilities|String|ToString(Boolean) _returnvalue))
  (if _returnvalue
    (Transformation|SetActorLocation OtherActor (Transformation|GetActorLocation (Variables|Default|GetResetPlatform)) false true)
    (Development|PrintString "Last Check")))

(event OnComponentBeginOverlap(Box4)
  (params (OverlappedComponent :type Primitive%20Component%20Object%20Reference) (OtherActor :type Actor%20Object%20Reference) (OtherComp :type Primitive%20Component%20Object%20Reference) (OtherBodyIndex :type Integer) (bFromSweep :type Boolean) (SweepResult :type Hit%20Result%20Structure%20%28by%20ref%29))
  (bind _returnvalue (Utilities|DoesObjectImplementInterface OtherActor "/Game/RenegadeJammer/Core/Characters/Common/BPI_Player.BPI_Player_C"))
  (Development|PrintString (Utilities|String|ToString(Boolean) _returnvalue))
  (if _returnvalue
    (Transformation|SetActorLocation OtherActor (Transformation|GetActorLocation (Variables|Default|GetResetPlatform)) false true)
    (Development|PrintString "Last Check")))

(event OnComponentBeginOverlap(Box2)
  (params (OverlappedComponent :type Primitive%20Component%20Object%20Reference) (OtherActor :type Actor%20Object%20Reference) (OtherComp :type Primitive%20Component%20Object%20Reference) (OtherBodyIndex :type Integer) (bFromSweep :type Boolean) (SweepResult :type Hit%20Result%20Structure%20%28by%20ref%29))
  (Development|PrintString (Utilities|GetObjectName OtherActor))
  (if (Utilities|DoesObjectImplementInterface OtherActor "/Game/RenegadeJammer/Core/Characters/Common/BPI_Player.BPI_Player_C")
    (Transformation|SetActorLocation OtherActor (Transformation|GetActorLocation (Variables|Default|GetResetPlatform)) false true)
    (Development|PrintString "Last Check")))

(event OnComponentBeginOverlap(Box3)
  (params (OverlappedComponent :type Primitive%20Component%20Object%20Reference) (OtherActor :type Actor%20Object%20Reference) (OtherComp :type Primitive%20Component%20Object%20Reference) (OtherBodyIndex :type Integer) (bFromSweep :type Boolean) (SweepResult :type Hit%20Result%20Structure%20%28by%20ref%29))
  (bind _returnvalue (Utilities|DoesObjectImplementInterface OtherActor "/Game/RenegadeJammer/Core/Characters/Common/BPI_Player.BPI_Player_C"))
  (Development|PrintString (Utilities|String|ToString(Boolean) _returnvalue))
  (if _returnvalue
    (Transformation|SetActorLocation OtherActor (Transformation|GetActorLocation (Variables|Default|GetResetPlatform)) false true)
    (Development|PrintString "Last Check")))

(event Custom|NewState
  (bind _totalloops (Variables|Default|GetTotalLoops))
  (Development|PrintString (Utilities|String|ToString(Integer) (Variables|Default|GetCounter)))
  (bind _result (Math|Integer|IncrementInt (Variables|Default|GetCounter))
    (:%20%20
      (if (== _result _totalloops)
        (CallFunction|ChangeState)
        (CallFunction|DisableCollisions)
        (Variables|Default|SetCounter 0)
        (Variables|Default|SetChosenIndex (Math|Random|RandomIntegerinRange 0 4))
        (elif (== _result (- _totalloops 1))
          (CallFunction|ChangeState 2)
          (CallFunction|BeatPlayer)
          (elif (== (Math|Integer|%(Integer) _result 2) 1)
            (CallFunction|ChangeState 1)
            (else
              (CallFunction|ChangeState))))))))

(event EventBeginPlay
  ;[1 1 1] Esta fórmula es un horror, sólo es de prueba
  (bind _returnvalue (Actor|GetActorOfClass "/Game/RenegadeJammer/Core/Obstacles/BP_LightPlatformReset.BP_LightPlatformReset_C"))
  (Variables|Default|SetResetPlatform _returnvalue)
  (Variables|Default|SetMeshesArray (Utilities|Array|MakeArray (Variables|Default|GetPlane) (Variables|Default|GetPlane1) (Variables|Default|GetPlane2) (Variables|Default|GetPlane3) (Variables|Default|GetPlane4)))
  (Variables|Default|SetCollisionArray (Utilities|Array|MakeArray (Variables|Default|GetBox) (Variables|Default|GetBox1) (Variables|Default|GetBox2) (Variables|Default|GetBox3) (Variables|Default|GetBox4)))
  (Variables|Default|SetChosenIndex (Math|Random|RandomIntegerinRange 0 4))
  (Utilities|Time|SetTimerbyEvent (delegate Custom|NewState) (Variables|Default|GetTime) true))

(event Collision|EventActorBeginOverlap
  (params (OtherActor :type Actor%20Object%20Reference)))

(event EventTick
  (params (DeltaSeconds :type Float%20%28single-precision%29)))

(fn ConstructionScript)

(fn ChangeState
  (params (state :type Integer))
  (for (_array_element _array_index) (Variables|Default|GetMeshesArray)
    (if (not (== _array_index (Variables|Default|GetChosenIndex)))
      (switch int state
        (:0
          (Rendering|Material|SetMaterial _array_element 0 "/Engine/BasicShapes/BasicShapeMaterial.BasicShapeMaterial"))
        (:1
          (Rendering|Material|SetMaterial _array_element 0 "/AnimationSharing/AnimSharingBlue.AnimSharingBlue"))
        (:2
          (Rendering|Material|SetMaterial _array_element 0 "/AnimationSharing/AnimSharingRed.AnimSharingRed"))))))

(fn BeatPlayer
  (for (_array_element _array_index) (Variables|Default|GetCollisionArray)
    (if (not (== _array_index (Variables|Default|GetChosenIndex)))
      (Collision|SetCollisionEnabled _array_element "QueryAndPhysics"))))

(fn DisableCollisions
  (for _array_element (Variables|Default|GetCollisionArray)
    (Collision|SetCollisionEnabled _array_element "NoCollision")))