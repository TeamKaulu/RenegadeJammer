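; Obstacle emitter that slides sideways along Y and fires BP_LittleWave actors, with a Wwise flamethrower shot sound.
; It fires once on BeginPlay, then a looping timer runs Move every ShootTime.
; Move picks a random Y within MovRange of the start location, and a Timeline slides the emitter there before spawning the next wave.
; The chosen Y is still printed as debug output.
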(event Custom|Move
  (bind _movrange (Variables|Default|GetMovRange))
  (bind _movrange_2 (Variables|Default|GetMovRange))
  (bind _shoottime (Variables|Default|GetShootTime))
  (bind _initiallocation (Variables|Default|GetInitialLocation))
  (bind _returnvalue (* _movrange -1.0))
  (bind _returnvalue_2 (/ _shoottime 2.0))
  (bind _returnvalue_3 (+ (.y _initiallocation) _movrange_2))
  (bind _returnvalue_4 (+ (.y _initiallocation) _returnvalue))
  (bind _returnvalue_5 (Math|Random|RandomFloatinRange _returnvalue_4 _returnvalue_3))
  (Variables|Default|SetStoredLocation (.location (Transformation|GetActorTransform)))
  (bind _output_get (Variables|Default|SetDesiredY _returnvalue_5))
  (Development|PrintString (Utilities|String|ToString(Float) _output_get) true true "(R=0.000000,G=0.660000,B=1.000000,A=1.000000)" _returnvalue_5)
  (bind _movpoint (Timeline|Timeline PlayFromStart)
    (:Update
      (Transformation|SetActorRelativeLocation (Math|Vector|MakeVector (.x (Variables|Default|GetStoredLocation)) (Math|Float|MapRangeClamped _movpoint 0.0 _returnvalue_2 (.y (Variables|Default|GetStoredLocation)) (Variables|Default|GetDesiredY)) (.z (Variables|Default|GetStoredLocation)))))
    (:Finished
      (Game|SpawnActorfromClass "/Game/RenegadeJammer/Core/Obstacles/BP_LittleWave.BP_LittleWave_C" (Transformation|GetActorTransform) "Undefined" "MultiplyWithRoot" 0 0)
      (Class|AkGameObject|PostAssociatedAkEvent (Variables|Default|GetPlay_SHOT_Flamethrower2)))))

(event EventBeginPlay
  (Utilities|FlowControl|Sequence
    (:then_0
      (Game|SpawnActorfromClass "/Game/RenegadeJammer/Core/Obstacles/BP_LittleWave.BP_LittleWave_C" (Transformation|GetActorTransform) "Undefined" "MultiplyWithRoot" 0 0)
      (Class|AkGameObject|PostAssociatedAkEvent (Variables|Default|GetPlay_SHOT_Flamethrower2)))
    (:then_1
      (Variables|Default|SetInitialLocation (Transformation|GetActorLocation)))
    (:then_2
      (Utilities|Time|SetTimerbyEvent (delegate Custom|Move) (Variables|Default|GetShootTime) true))))

(event Collision|EventActorBeginOverlap
  (params (OtherActor :type Actor%20Object%20Reference)))

(event EventTick
  (params (DeltaSeconds :type Float%20%28single-precision%29)))

(fn ConstructionScript)