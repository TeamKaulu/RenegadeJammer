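; BP_MobilePilars is an obstacle of two pillar sets that slide back and forth in opposite directions along local X.
; The construction script sizes and places two boundary boxes and spreads pillar instances along Y, alternating between two hierarchical instanced mesh components starting at opposite boxes.
; Tick offsets each component by a per-frame speed, unscaled by delta time.
; Only Box1's overlap with an instanced mesh reverses the shared speed.
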(event OnComponentBeginOverlap(Box1)
  (params (OverlappedComponent :type Primitive%20Component%20Object%20Reference) (OtherActor :type Actor%20Object%20Reference) (OtherComp :type Primitive%20Component%20Object%20Reference) (OtherBodyIndex :type Integer) (bFromSweep :type Boolean) (SweepResult :type Hit%20Result%20Structure%20%28by%20ref%29))
  (if (== (Utilities|GetClass OtherComp) "/Script/Engine.HierarchicalInstancedStaticMeshComponent")
    (Variables|Default|SetSpeed (* (Variables|Default|GetSpeed) -1.0))))

(event EventBeginPlay)

(event Collision|EventActorBeginOverlap
  (params (OtherActor :type Actor%20Object%20Reference)))

(event EventTick
  (params (DeltaSeconds :type Float%20%28single-precision%29))
  (Transformation|AddLocalOffset (Variables|Default|GetHierarchicalPillarsA) (Math|Vector|MakeVector (Variables|Default|GetSpeed) 0.0 0.0) false false)
  (Transformation|AddLocalOffset (Variables|Default|GetHierarchicalPillarsB) (Math|Vector|MakeVector (* (Variables|Default|GetSpeed) -1.0) 0.0 0.0) false false))

(fn ConstructionScript
  (bind _box1 (Variables|Default|GetBox1))
  (bind _distancex (Variables|Default|GetDistanceX))
  (Components|Box|SetBoxExtent _box1 (Math|Vector|MakeVector 32.0 (Variables|Default|GetExtentY) 1.5e+02) true)
  (Transformation|SetRelativeLocation _box1 (Math|Vector|MakeVector (* _distancex -1.0) 0.0 9e+01) false false)
  (Transformation|SetRelativeLocation (Variables|Default|GetBox) (Math|Vector|MakeVector _distancex 0.0 9e+01) false false)
  (Variables|Default|SetDistanceY (/ (Variables|Default|GetExtentY) (Variables|Default|GetNumberOfPillars)))
  (for _index (range 1 (Variables|Default|GetNumberOfPillars))
    (Utilities|FlowControl|FlipFlop
      (:A
        (Components|InstancedStaticMesh|AddInstance (Variables|Default|GetHierarchicalPillarsA) (Math|Transform|MakeTransform (Math|Vector|MakeVector (.x (Variables|/Script/Engine.SceneComponent|GetRelativeLocation (Variables|Default|GetBox1))) (* (+ (/ (Variables|Default|GetExtentY) -2.0) (+ (/ (Variables|Default|GetDistanceY) 2.0) (* (- _index 1) (Variables|Default|GetDistanceY)))) 2.0) 0.0) "0, 0, 0" (Variables|Default|GetInstanceScale)) false))
      (:B
        (Components|InstancedStaticMesh|AddInstance (Variables|Default|GetHierarchicalPillarsB) (Math|Transform|MakeTransform (Math|Vector|MakeVector (.x (Variables|/Script/Engine.SceneComponent|GetRelativeLocation (Variables|Default|GetBox))) (* (+ (/ (Variables|Default|GetExtentY) -2.0) (+ (/ (Variables|Default|GetDistanceY) 2.0) (* (- _index 1) (Variables|Default|GetDistanceY)))) 2.0) 0.0) "0, 0, 0" (Variables|Default|GetInstanceScale)) false)))))