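; BP_Punch is an obstacle with a boxing glove that punches along its local X axis and disturbs the movement of players it hits.
; A timeline, with play rate set by Speed, starts on BeginPlay and scales its curve by Displacement to move the glove.
; Timeline event tracks toggle the punch collision, whose overlap sends a disturbance message to actors implementing BPI_Player.
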(event OnComponentBeginOverlap(PunchingCollision)
  (params (OverlappedComponent :type Primitive%20Component%20Object%20Reference) (OtherActor :type Actor%20Object%20Reference) (OtherComp :type Primitive%20Component%20Object%20Reference) (OtherBodyIndex :type Integer) (bFromSweep :type Boolean) (SweepResult :type Hit%20Result%20Structure%20%28by%20ref%29))
  (if (Utilities|DoesObjectImplementInterface OtherActor "/Game/RenegadeJammer/Core/Characters/Common/BPI_Player.BPI_Player_C")
    (Class|BPIPlayer|DisturbMovement(Message) OtherActor "NewEnumerator0" self)))

(event EventBeginPlay
  (bind _punchingcollision (Variables|Default|GetPunchingCollision))
  (Components|Timeline|SetPlayRate (Variables|Default|GetDisplacementTimeline) (Variables|Default|GetSpeed))
  (bind _displacement (Timeline|DisplacementTimeline Play)
    (:Update
      (Transformation|SetRelativeLocation (Variables|Default|GetSM_BoxingGlove) (Math|Vector|MakeVector (* _displacement (Variables|Default|GetDisplacement)) 0.0 0.0) false false))
    (:StartPunching
      (Collision|SetCollisionEnabled _punchingcollision "QueryOnly"))
    (:StopPunching
      (Collision|SetCollisionEnabled _punchingcollision "NoCollision"))))

(fn ConstructionScript)