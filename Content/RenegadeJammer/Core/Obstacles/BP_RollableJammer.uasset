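; BP_RollableJammer is an obstacle that starts simulating physics when a player comes near, then removes itself.
; An overlap on its Sphere by an actor implementing BPI_Player triggers it once, enabling physics on the static mesh.
; A Timeline then multiplies the mesh's initial world scale by its Scale track and destroys the actor when finished.
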(event OnComponentBeginOverlap(Sphere)
  (params (OverlappedComponent :type Primitive%20Component%20Object%20Reference) (OtherActor :type Actor%20Object%20Reference) (OtherComp :type Primitive%20Component%20Object%20Reference) (OtherBodyIndex :type Integer) (bFromSweep :type Boolean) (SweepResult :type Hit%20Result%20Structure%20%28by%20ref%29))
  (if (and (Utilities|DoesObjectImplementInterface OtherActor "/Game/RenegadeJammer/Core/Characters/Common/BPI_Player.BPI_Player_C") (not (Variables|Default|GetIsAlreadyPlaying)))
    (Variables|Default|SetIsAlreadyPlaying true)
    (Physics|SetSimulatePhysics (Variables|Default|GetStaticMesh) true)
    (bind _scale (Timeline|Timeline PlayFromStart)
      (:Update
        (Transformation|SetWorldScale3D (Variables|Default|GetStaticMesh) (* (Variables|Default|GetInitialScale) _scale)))
      (:Finished
        (Actor|DestroyActor)))))

(event EventBeginPlay
  (Variables|Default|SetInitialScale (Transformation|GetWorldScale (Variables|Default|GetStaticMesh))))

(fn ConstructionScript)