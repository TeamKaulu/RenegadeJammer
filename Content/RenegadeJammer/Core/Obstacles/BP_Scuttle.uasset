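; BP_Scuttle is an obstacle that opens and closes by switching the collision of three box components off and on.
; OpenScuttle and CloseScuttle act only when the state changes, flipping IsOpen and setting all three boxes to no collision or to query and physics.
; The construction script sizes the boxes from one shared BoxExtent and applies collision to match the initial IsOpen value.
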(event Custom|CloseScuttle
  (if (Variables|Default|GetIsOpen)
    (Variables|Default|SetIsOpen (not (Variables|Default|GetIsOpen)))
    (Collision|SetCollisionEnabled (Variables|Default|GetBox) "QueryAndPhysics")
    (Collision|SetCollisionEnabled (Variables|Default|GetBox2) "QueryAndPhysics")
    (Collision|SetCollisionEnabled (Variables|Default|GetBox1) "QueryAndPhysics")))

(event Custom|OpenScuttle
  (if (not (Variables|Default|GetIsOpen))
    (Variables|Default|SetIsOpen (not (Variables|Default|GetIsOpen)))
    (Collision|SetCollisionEnabled (Variables|Default|GetBox) "NoCollision")
    (Collision|SetCollisionEnabled (Variables|Default|GetBox2) "NoCollision")
    (Collision|SetCollisionEnabled (Variables|Default|GetBox1) "NoCollision")))

(fn ConstructionScript
  (bind _boxextent (Variables|Default|GetBoxExtent))
  (Components|Box|SetBoxExtent (Variables|Default|GetBox) _boxextent true)
  (Components|Box|SetBoxExtent (Variables|Default|GetBox2) _boxextent true)
  (Components|Box|SetBoxExtent (Variables|Default|GetBox1) _boxextent true)
  (if (Variables|Default|GetIsOpen)
    (Collision|SetCollisionEnabled (Variables|Default|GetBox) "NoCollision")
    (Collision|SetCollisionEnabled (Variables|Default|GetBox2) "NoCollision")
    (Collision|SetCollisionEnabled (Variables|Default|GetBox1) "NoCollision")
    (else
      (Collision|SetCollisionEnabled (Variables|Default|GetBox) "QueryAndPhysics")
      (Collision|SetCollisionEnabled (Variables|Default|GetBox2) "QueryAndPhysics")
      (Collision|SetCollisionEnabled (Variables|Default|GetBox1) "QueryAndPhysics"))))