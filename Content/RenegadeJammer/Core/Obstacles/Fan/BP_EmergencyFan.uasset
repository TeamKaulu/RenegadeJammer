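; Emergency fan obstacle, a child Blueprint that uses capsules as its impulse trigger volumes.
; Capsule begin and end overlaps register and unregister components through AddObject and RemoveObject.
; UpdateImpulseTriggerBoxes resizes the capsule children of Scene to a half height of half ImpulseHeight.
; It then offsets each on Z by half height minus radius, keeping the lower cap one radius below the Scene origin.
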(event OnComponentBeginOverlap(Capsule)
  (params (OverlappedComponent :type Primitive%20Component%20Object%20Reference) (OtherActor :type Actor%20Object%20Reference) (OtherComp :type Primitive%20Component%20Object%20Reference) (OtherBodyIndex :type Integer) (bFromSweep :type Boolean) (SweepResult :type Hit%20Result%20Structure%20%28by%20ref%29))
  (CallFunction|AddObject OtherComp))

(event OnComponentEndOverlap(Capsule)
  (params (OverlappedComponent :type Primitive%20Component%20Object%20Reference) (OtherActor :type Actor%20Object%20Reference) (OtherComp :type Primitive%20Component%20Object%20Reference) (OtherBodyIndex :type Integer))
  (CallFunction|RemoveObject OtherComp))

(fn ConstructionScript
  (|CallParentFunction))

(fn UpdateImpulseTriggerBoxes
  (for _array_element (Components|GetChildrenComponents (Variables|Default|GetScene) false)
    (bind _ascapsule_collision (Utilities|Casting|CastToCapsuleComponent _array_element))
    (Components|Capsule|SetCapsuleHalfHeight _ascapsule_collision (/ (Variables|Default|GetImpulseHeight) 2.0) true)
    (Transformation|SetRelativeLocation _ascapsule_collision (Math|Vector|MakeVector (.x (Variables|/Script/Engine.SceneComponent|GetRelativeLocation _ascapsule_collision)) (.y (Variables|/Script/Engine.SceneComponent|GetRelativeLocation _ascapsule_collision)) (- (Variables|/Script/Engine.CapsuleComponent|GetCapsuleHalfHeight _ascapsule_collision) (Variables|/Script/Engine.CapsuleComponent|GetCapsuleRadius _ascapsule_collision))) false false)))