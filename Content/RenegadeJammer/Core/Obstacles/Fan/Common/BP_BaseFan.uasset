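; Base Blueprint for a rotating fan obstacle that pushes physics objects along its up vector, leaving impulse trigger box setup to children.
; Tick applies force to a capped list of registered components, scaled by a sigmoid speed-limit curve.
; Wwise events play on wind impulse and as blade yaw crosses set angles.
; Construction sets material, spin and activation; optional game mode difficulty updates change spin speed, and DeactivateFan disables force.
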(event Custom|Event%20On%20Update%20Difficulty
  (params (FanSpeed :type Float%20%28double-precision%29))
  (CallFunction|SetFanSpeed FanSpeed)
  (Development|PrintString (Utilities|String|Append "[" (Utilities|GetDisplayName self) "] updated fan speed at " (Utilities|String|ToString(Float) FanSpeed))))

(event Custom|ResetWindImpulse
  (Utilities|FlowControl|DoOnce false) ; enters at Reset
)

(event EventTick
  (params (DeltaSeconds :type Float%20%28single-precision%29))
  (bind _self self)
  (bind _audioevent (Variables|Default|GetAudioEvent))
  (bind _fan (Variables|Default|GetFan))
  (bind _returnvalue (Transformation|GetWorldLocation _fan))
  (bind _fan_2 (Variables|Default|GetFan _self))
  (bind _returnvalue_2 (Transformation|GetWorldRotation _fan_2))
  (Utilities|FlowControl|Sequence
    (:then_0
      (if (Variables|Default|GetActivateFanForce)
        (bind (_array_element _array_index) (Utilities|Array|ForEachLoopwithBreak (Variables|Default|GetObjectsInside) :!label _label)
          (:LoopBody
            (if (>= _array_index (Variables|Default|GetMaxObjectsToApplyForce))
              (goto _label Break)
              (else
                (bind _returnvalue_3 (Physics|GetPhysicsLinearVelocity _array_element "None"))
                (Physics|AddForce _array_element (* (* (Transformation|GetActorUpVector) (Variables|Default|GetFanForceStrength)) (CallFunction|GetSpeedLimitFactor (Variables|Default|GetSpeed%20Limit) 0.01 1.0 (CallFunction|CmstoKmH (Math|Vector|VectorLength (Math|Vector|ProjectVectorontoVector _returnvalue_3 (Transformation|GetActorUpVector)))))) "None" true)
                (Utilities|FlowControl|DoOnce false
                  (:Completed
                    (Development|PrintString (Utilities|String|Append "Force: " (Utilities|String|ToString(Float) (.Z (Math|Vector|BreakVector (* (* (Transformation|GetActorUpVector) (Variables|Default|GetFanForceStrength)) (CallFunction|GetSpeedLimitFactor (Variables|Default|GetSpeed%20Limit) 0.01 1.0 (CallFunction|CmstoKmH (Math|Vector|VectorLength (Math|Vector|ProjectVectorontoVector _returnvalue_3 (Transformation|GetActorUpVector)))))))))))
                    (Development|PrintString "WIND IMPULSE")
                    (Class|AkGameplayStatics|PostEvent "/Game/WwiseAudio/Events/Default_Work_Unit/ObjectsEvents/Map1Zone3/Play_wind_impulse.Play_wind_impulse")
                    (Utilities|Time|SetTimerbyEvent (delegate Custom|ResetWindImpulse) 2.0)))))))))
    (:then_1
      (if (and (> (.yaw _returnvalue_2) 7e+01) (< (.yaw _returnvalue_2) 8e+01))
        (Utilities|FlowControl|DoOnce false :!label _label_2
          (:Completed
            (Class|AkGameplayStatics|PostEventatLocation _audioevent _returnvalue "0, 0, 0")
            (Utilities|FlowControl|Sequence
              (:then_0
                (goto _label_3 Reset))
              (:then_1
                (goto _label_4 Reset))
              (:then_2
                (goto _label_5 Reset)))))
        (elif (and (> (.yaw _returnvalue_2) 1.6e+02) (< 1.7e+02 (.yaw _returnvalue_2)))
          (Utilities|FlowControl|DoOnce false :!label _label_3
            (:Completed
              (Class|AkGameplayStatics|PostEventatLocation _audioevent _returnvalue "0, 0, 0")
              (Utilities|FlowControl|Sequence
                (:then_0
                  (goto _label_2 Reset))
                (:then_1
                  (goto _label_4 Reset))
                (:then_2
                  (goto _label_5 Reset)))))
          (elif (and (> (.yaw _returnvalue_2) -1.1e+02) (< (.yaw _returnvalue_2) -1e+02))
            (Utilities|FlowControl|DoOnce false :!label _label_4
              (:Completed
                (Class|AkGameplayStatics|PostEventatLocation _audioevent _returnvalue "0, 0, 0")))
            (elif (and (> (.yaw _returnvalue_2) -2e+01) (< (.yaw _returnvalue_2) -1e+01))
              (Utilities|FlowControl|DoOnce false :!label _label_5
                (:Completed
                  (Class|AkGameplayStatics|PostEventatLocation _audioevent _returnvalue "0, 0, 0")
                  (Utilities|FlowControl|Sequence
                    (:then_0
                      (goto _label_4 Reset))
                    (:then_1
                      (goto _label_3 Reset))
                    (:then_2
                      (goto _label_2 Reset))))))))))))

(event EventBeginPlay
  (if (Variables|Default|GetShouldUpdateDifficulty)
    (bind _asbp_default_game_mode (Utilities|Casting|CastToBP_DefaultGameMode (Game|GetGameMode)))
    (EventDispatchers|BindEventtoOnThirdZoneDifficultyUpdated _asbp_default_game_mode (delegate Custom|Event%20On%20Update%20Difficulty))))

(fn ConstructionScript
  (Rendering|Material|SetMaterial (Variables|Default|GetFan) 0 (Variables|Default|GetFanMaterial))
  (CallFunction|SetFanSpeed (Variables|Default|GetFanSpeed))
  (CallFunction|UpdateImpulseTriggerBoxes)
  (CallFunction|UpdateFanActivation)
  (if (Variables|Default|GetIsBigFan)
    (Variables|Default|SetAudioEvent "/Game/WwiseAudio/Events/Default_Work_Unit/ObjectsEvents/Map1Zone3/Play_FanBladesBig.Play_FanBladesBig")
    (else
      (Variables|Default|SetAudioEvent "/Game/WwiseAudio/Events/Default_Work_Unit/ObjectsEvents/Map1Zone3/Play_FanBladesSmall.Play_FanBladesSmall"))))

(fn SetFanMaterial
  (params (Material :type Material%20Instance%20Object%20Reference))
  (bind _fan (Variables|Default|GetFan))
  (Rendering|Material|SetMaterial _fan 1 Material)
  (Rendering|Material|SetMaterial _fan 2 Material))

(fn SetFanSpeed
  (params (Speed :type Float%20%28double-precision%29))
  (bind _rotatingmovement (Variables|Default|GetRotatingMovement))
  (Variables|/Script/Engine.RotatingMovementComponent|SetRotationRate _rotatingmovement (Math|Rotator|MakeRotator (.roll (Variables|/Script/Engine.RotatingMovementComponent|GetRotationRate _rotatingmovement)) (.pitch (Variables|/Script/Engine.RotatingMovementComponent|GetRotationRate _rotatingmovement)) (Utilities|Select :Index (Variables|Default|GetFanDirection) :NewEnumerator0 Speed :NewEnumerator1 (* Speed -1.0)))))

(fn UpdateImpulseTriggerBoxes
  (Development|PrintString (Utilities|String|Append "[" (Utilities|GetDisplayName self) "] this logic should be implemented in children")))

(fn RegisterComponent
  (params (Component :type Primitive%20Component%20Object%20Reference)))

(fn UpdateFanActivation
  (Actor|Tick|SetActorTickEnabled (select (Variables|Default|GetActivateFanForce) true false))
  (for _array_element (Components|GetChildrenComponents (Variables|Default|GetScene) false)
    (bind _asstatic_mesh_component (Utilities|Casting|CastToStaticMeshComponent _array_element))
    (Collision|SetCollisionEnabled _asstatic_mesh_component (select (Variables|Default|GetActivateFanForce) "QueryOnly" "NoCollision"))))

(fn AddObject
  (params (Component :type Primitive%20Component%20Object%20Reference%20%28by%20ref%29))
  (if (Utilities|Array|ContainsItem (Variables|Default|GetObjectsInside) Component)
    (Development|PrintString "already inside" true true "(R=1.000000,G=0.002430,B=0.000000,A=1.000000)")
    (else
      (Utilities|Array|Add (Variables|Default|GetObjectsInside) Component))))

(fn UpdateRotationSpeed
  (params (NewSpeed :type Float%20%28double-precision%29))
  (Variables|/Script/Engine.RotatingMovementComponent|SetRotationRate (Variables|Default|GetRotatingMovement) (Math|Rotator|MakeRotator 0.0 0.0 NewSpeed))
  (Variables|Default|SetFanSpeed NewSpeed))

(fn GetRotationComponent
  (return (Variables|Default|GetRotatingMovement)))

(fn RemoveObject
  (params (Item :type Primitive%20Component%20Object%20Reference%20%28by%20ref%29))
  (if (Utilities|Array|ContainsItem (Variables|Default|GetObjectsInside) Item)
    (Utilities|Array|RemoveItem (Variables|Default|GetObjectsInside) Item)
    (else
      (Development|PrintString "not inside" true true "(R=0.006647,G=1.000000,B=0.000000,A=1.000000)"))))

(fn GetSpeedLimitFactor
  (params (SpeedLimit :type Float%20%28double-precision%29) (CurveFactor :type Float%20%28double-precision%29) (InputValue :type Float%20%28double-precision%29) (Speed :type Float%20%28double-precision%29))
  (if (< 0.0 SpeedLimit)
    (return (* (+ -1.0 (/ 2.0 (+ 1.0 (Class|KismetMathLibrary|Exp (* CurveFactor (- Speed SpeedLimit)))))) InputValue))
    (else
      (return 0.0))))

(fn SetImpulseHeigh
  (params (ImpulseHeight :type Float%20%28double-precision%29))
  (Variables|Default|SetImpulseHeight ImpulseHeight)
  (CallFunction|UpdateImpulseTriggerBoxes))

(fn DeactivateFan
  (Variables|Default|SetActivateFanForce false)
  (CallFunction|UpdateFanActivation)
  (Utilities|IsValid (Variables|Default|GetAkAmbientSound)
    (:Is%20Valid
      (Actor|DestroyActor (Variables|Default|GetAkAmbientSound)))))