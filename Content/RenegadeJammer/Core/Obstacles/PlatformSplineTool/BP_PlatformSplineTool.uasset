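; Construction-script spline tool that builds obstacle platforms and ramps from spline mesh segments along a spline.
; Segments are either mesh-length sections or one per spline point pair, chosen by UseSectionLength.
; PopulateData resizes the per-segment PlatformsData array to match, letting each entry set type, visibility and start/end scale.
; BuildPlatform adds each visible segment with its type's mesh, material and collision, making ForwardRamp spline points linear.
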(fn ConstructionScript
  (bind _mesh (CallFunction|GetMeshfromType "NewEnumerator0"))
  (bind _returnvalue (StaticMesh|GetBoundingBox _mesh))
  (if (> (Spline|GetNumberOfSplinePoints (Variables|Default|GetSpline)) 1)
    (Variables|Default|SetSection%20Length (.x (+ (Math|Vector|VectorGetAbs (.min _returnvalue)) (Math|Vector|VectorGetAbs (.max _returnvalue)))))
    (Variables|Default|SetPlatformsNumber (select (Variables|Default|GetUseSectionLength) (Math|Float|Truncate (/ (Spline|GetSplineLength (Variables|Default|GetSpline)) (Variables|Default|GetSection%20Length))) (- (Spline|GetNumberOfSplinePoints (Variables|Default|GetSpline)) 1)))
    (CallFunction|PopulateData)
    (for _index (range 0 (- (Variables|Default|GetPlatformsNumber) 1))
      (CallFunction|BuildPlatform _index))
    (else
      (Development|PrintString "Not enough spline points"))))

(fn GetMeshfromType
  (params (PlatformType :type E_SplineToolPlatformType%20Enum :default "NewEnumerator0"))
  (return (Utilities|Select :Index PlatformType :NewEnumerator0 "/Game/RenegadeJammer/Core/Obstacles/PlatformSplineTool/SM_LargeBasePlatform.SM_LargeBasePlatform" :NewEnumerator1 "/Game/RenegadeJammer/Core/Obstacles/PlatformSplineTool/SM_ForwardBaseRamp.SM_ForwardBaseRamp" :NewEnumerator2 "/Game/RenegadeJammer/Core/Obstacles/PlatformSplineTool/SM_BaseLeftBowl.SM_BaseLeftBowl" :NewEnumerator3 "/Game/RenegadeJammer/Core/Obstacles/PlatformSplineTool/SM_BaseRightBowl.SM_BaseRightBowl" :NewEnumerator4 "/Game/RenegadeJammer/Core/Obstacles/PlatformSplineTool/SM_BackwardBaseRamp.SM_BackwardBaseRamp")))

(fn BuildPlatform
  (params (Index :type Integer))
  (bind _platformsdata (Variables|Default|GetPlatformsData))
  (bind (_startpoint _starttangent _endpoint _endtangent) (CallFunction|GetSplinePointData Index))
  (bind _output (Utilities|Array|Get(acopy) _platformsdata Index))
  (bind (_type _startwidth _startheight _endwidth _endheigth _hideplatform) (Utilities|Struct|BreakS_SplineToolPlatformData _output))
  (if (not _hideplatform)
    (Utilities|FlowControl|Sequence
      (:then_0
        (LocalVariables|SetStartPosition _startpoint)
        (LocalVariables|SetStartTangent _starttangent)
        (LocalVariables|SetEndPosition _endpoint)
        (LocalVariables|SetEndTangent _endtangent))
      (:then_1
        (bind _returnvalue (AddComponent|AddSplineMeshComponent false))
        (LocalVariables|SetSplineMeshComponent _returnvalue))
      (:then_2
        (Components|StaticMesh|SetStaticMesh (LocalVariables|GetSplineMeshComponent) (CallFunction|GetMeshfromType _type)))
      (:then_3
        (Rendering|Material|SetMaterial (LocalVariables|GetSplineMeshComponent) 0 (CallFunction|GetMaterialfromType _type)))
      (:then_4
        (SplineMesh|SetForwardAxis (LocalVariables|GetSplineMeshComponent) "X" true))
      (:then_5
        (Collision|SetCollisionProfileName (LocalVariables|GetSplineMeshComponent) (Variables|Default|GetIn%20Collision%20Profile%20Name) true :!class /Script/Engine.PrimitiveComponent))
      (:then_6
        (Collision|SetCollisionEnabled (LocalVariables|GetSplineMeshComponent) (Variables|Default|GetCollisionSettings)))
      (:then_7
        (SplineMesh|SetStartScale (LocalVariables|GetSplineMeshComponent) (Math|Vector2D|MakeVector2D _startwidth _startheight) true :!class /Script/Engine.SplineMeshComponent)
        (SplineMesh|SetEndScale (LocalVariables|GetSplineMeshComponent) (Math|Vector2D|MakeVector2D _endwidth _endheigth) true :!class /Script/Engine.SplineMeshComponent))
      (:then_8
        (Spline|SetSplinePointType (Variables|Default|GetSpline) Index (select (Utilities|Enum|Equal(Enum) _type "NewEnumerator1") "Linear" "CurveCustomTangent") true))
      (:then_9
        (SplineMesh|SetStartandEnd (LocalVariables|GetSplineMeshComponent) (LocalVariables|GetStartPosition) (LocalVariables|GetStartTangent) (LocalVariables|GetEndPosition) (LocalVariables|GetEndTangent) true :!class /Script/Engine.SplineMeshComponent)))))

(fn GetMaterialfromType
  (params (Type :type E_SplineToolPlatformType%20Enum :default "NewEnumerator0"))
  (return (Utilities|Select :Index Type :NewEnumerator0 "/Game/RenegadeJammer/Art/Industrial/Zone01/Ramps/FloatingRamp/MI_FloatingRamp.MI_FloatingRamp" :NewEnumerator1 "/Game/RenegadeJammer/Art/Industrial/Zone01/Ramps/FloatingRamp/MI_FloatingRamp.MI_FloatingRamp" :NewEnumerator2 "/Game/RenegadeJammer/Art/Industrial/Zone01/Ramps/FloatingRamp/MI_FloatingRamp.MI_FloatingRamp" :NewEnumerator3 "/Game/RenegadeJammer/Art/Industrial/Zone01/Ramps/FloatingRamp/MI_FloatingRamp.MI_FloatingRamp" :NewEnumerator4 "/Game/RenegadeJammer/Art/Industrial/Zone01/Ramps/FloatingRamp/MI_FloatingRamp.MI_FloatingRamp")))

(fn PopulateData
  (bind _platformsdata (Variables|Default|GetPlatformsData))
  (Math|Integer|CompareInt (Utilities|Array|Length (Variables|Default|GetPlatformsData)) (Variables|Default|GetPlatformsNumber) :!label _label
    (:>
      (Utilities|Array|RemoveIndex _platformsdata (Utilities|Array|LastIndex _platformsdata))
      (goto _label))
    (:==
      (Development|PrintString "Platforms data succesfully updated!" true true "(R=0.000000,G=1.000000,B=0.051450,A=1.000000)"))
    (:<
      (Utilities|Array|Add :TargetArray (Variables|Default|GetPlatformsData))
      (goto _label))))

(fn GetSplinePointData
  (params (Index :type Integer))
  (bind _usesectionlength (Variables|Default|GetUseSectionLength))
  (bind _spline (Variables|Default|GetSpline))
  (bind _section_length (Variables|Default|GetSection%20Length))
  (bind _section_length_2 (Variables|Default|GetSection%20Length))
  (bind _spline_2 (Variables|Default|GetSpline))
  (bind _returnvalue (* Index _section_length))
  (bind (_location _tangent) (Spline|GetLocationandTangentatSplinePoint _spline_2 Index "Local"))
  (bind _returnvalue_2 (+ Index 1))
  (bind _returnvalue_3 (* _returnvalue_2 _section_length_2))
  (bind (_location_2 _tangent_2) (Spline|GetLocationandTangentatSplinePoint _spline _returnvalue_2 "Local"))
  (return (select _usesectionlength (Spline|GetLocationatDistanceAlongSpline _spline _returnvalue "Local") _location) (select _usesectionlength (Math|Vector|ClampVectorSize (Spline|GetTangentatDistanceAlongSpline _spline _returnvalue "Local") 0.0 (Variables|Default|GetSection%20Length)) _tangent) (select _usesectionlength (Spline|GetLocationatDistanceAlongSpline _spline _returnvalue_3 "Local") _location_2) (select _usesectionlength (Math|Vector|ClampVectorSize (Spline|GetTangentatDistanceAlongSpline _spline _returnvalue_3 "Local") 0.0 (Variables|Default|GetSection%20Length)) _tangent_2)))