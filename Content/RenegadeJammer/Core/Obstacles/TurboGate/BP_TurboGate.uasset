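; Turbo gate obstacle that applies a movement disturbance to players entering its box trigger, gated by their boost state.
; On overlap it queries the actor through BPI_Player; Yellow and Blue gates require a matching boost, while NoBoost and Green gates always fire.
; The construction script scales the mesh's Y and Z by Radius over InitialRadius and sets its material by Boost, with materials assigned only for Yellow and Blue.
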(event OnComponentBeginOverlap(Box)
  (params (OverlappedComponent :type Primitive%20Component%20Object%20Reference) (OtherActor :type Actor%20Object%20Reference) (OtherComp :type Primitive%20Component%20Object%20Reference) (OtherBodyIndex :type Integer) (bFromSweep :type Boolean) (SweepResult :type Hit%20Result%20Structure%20%28by%20ref%29))
  (if (Utilities|DoesObjectImplementInterface OtherActor "/Game/RenegadeJammer/Core/Characters/Common/BPI_Player.BPI_Player_C")
    (bind _booststate (Class|BPIPlayer|GetBoostState(Message) OtherActor))
    (if (Utilities|Select :Index (Variables|Default|GetBoost) :NewEnumerator0 true :NewEnumerator1 (Utilities|Enum|Equal(Enum) (Variables|Default|GetBoost) _booststate) :NewEnumerator2 (Utilities|Enum|Equal(Enum) (Variables|Default|GetBoost) _booststate) :NewEnumerator3 true)
      (Class|BPIPlayer|DisturbMovement(Message) OtherActor "NewEnumerator6" self))))

(fn ConstructionScript
  (bind _radius (Variables|Default|GetRadius))
  (bind _initialradius (LocalVariables|GetInitialRadius))
  (bind _returnvalue (/ _radius _initialradius))
  (Transformation|SetRelativeScale3D (Variables|Default|GetStaticMesh) (Math|Vector|MakeVector 1.0 _returnvalue _returnvalue))
  (Rendering|Material|SetMaterial (Variables|Default|GetStaticMesh) 0 (Utilities|Select :Index (Variables|Default|GetBoost) :NewEnumerator0 0 :NewEnumerator1 "/Game/RenegadeJammer/MaterialLibrary/Debug/M_YellowBoostMaterial.M_YellowBoostMaterial" :NewEnumerator2 "/Game/RenegadeJammer/MaterialLibrary/Debug/M_BlueBoostMaterial.M_BlueBoostMaterial" :NewEnumerator3 0)))