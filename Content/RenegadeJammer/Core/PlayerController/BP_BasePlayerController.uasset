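; Base player controller that tracks whether the player uses a gamepad and relays UI accept and cancel input.
; Any key press or gamepad left-stick X input updates the input type, broadcasting InputMethodChanged only when it changes, with a focus flag set for gamepad or keyboard keys.
; Enhanced Input UI actions fire accept and cancel dispatchers, and IsUsingGamepad exposes the current state.
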(event Input|EnhancedActionEvents|EnhancedInputActionIA_Cancel_UI
  (params (ActionValue :type Boolean) (ElapsedSeconds :type Float%20%28double-precision%29) (TriggeredSeconds :type Float%20%28double-precision%29) (InputAction :type Input%20Action%20Object%20Reference :default "/Game/RenegadeJammer/Core/Input/IA_Cancel_UI.IA_Cancel_UI"))
  ;[1 1 1] Update when player is using gamepad
  (:Started
    (Default|CallOnUICancelInputPressed)))

(event Input|EnhancedActionEvents|EnhancedInputActionIA_Accept_UI
  (params (ActionValue :type Boolean) (ElapsedSeconds :type Float%20%28double-precision%29) (TriggeredSeconds :type Float%20%28double-precision%29) (InputAction :type Input%20Action%20Object%20Reference :default "/Game/RenegadeJammer/Core/Input/IA_Accept_UI.IA_Accept_UI"))
  ;[1 1 1] Update when player is using gamepad
  (:Started
    (Default|CallOnUIAcceptInput)))

(event EventUpdateInputType
  (params (KeyPressed :type Key%20Structure :default "None"))
  (bind _returnvalue (Class|KismetInputLibrary|KeyIsGamepadKey KeyPressed))
  ;[1 1 1] Update when player is using gamepad
  (Variables|Default|SetPreviousInputType (Variables|Default|GetInputType))
  (Variables|Default|SetInputType (select _returnvalue "NewEnumerator1" "NewEnumerator0"))
  (if (Utilities|Enum|NotEqual(Enum) (Variables|Default|GetInputType) (Variables|Default|GetPreviousInputType))
    (Variables|Default|SetShoudUseFocus (or _returnvalue (Class|KismetInputLibrary|KeyIsKeyboardKey KeyPressed)))
    (Default|CallInputMethodChanged (Variables|Default|GetShoudUseFocus) (Variables|Default|GetInputType))))

(event Input|GamepadEvents|GamepadLeftX
  (params (Key :type Key%20Structure :default "None"))
  ;[1 1 1] Update when player is using gamepad
  (:Pressed
    (CallFunction|UpdateInputType Key)))

(event Input|KeyboardEvents|AnyKey
  (params (Key :type Key%20Structure :default "None"))
  ;[1 1 1] Update when player is using gamepad
  (:Pressed
    (CallFunction|UpdateInputType Key)))

(fn ConstructionScript)

(fn IsUsingGamepad
  (return (Utilities|Enum|Equal(Enum) (Variables|Default|GetInputType) "NewEnumerator1")))