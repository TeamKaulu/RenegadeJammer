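; BP_MainMenuPlayerController is the player controller that sets up the main menu.
; On BeginPlay it creates WBP_MainMenu, adds it to the viewport, shows the mouse cursor and sets Game and UI input mode.
; It focuses the menu's desired widget only if an IsUsingGamepad message to player controller 0 returns true.
; Its own IsUsingGamepad function always returns false.
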(event EventBeginPlay
  (bind _returnvalue (Game|GetPlayerController 0))
  (bind _returnvalue_2 (UserInterface|CreateWidget "/Game/RenegadeJammer/UserInterface/Screens/WBP_MainMenu.WBP_MainMenu_C" (Game|GetPlayerController 0)))
  (UserInterface|Viewport|AddtoViewport _returnvalue_2 0)
  (Variables|/Script/Engine.PlayerController|SetbShowMouseCursor _returnvalue true)
  (bind _isusinggamepad (Class|BPIController|IsUsingGamepad(Message) _returnvalue))
  (Input|SetInputModeGameandUI self (select _isusinggamepad (Default|GetDesiredFocusInput _returnvalue_2) 0) "DoNotLock" true true))

(fn ConstructionScript)

(fn IsUsingGamepad
  (return false))