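; Player controller for the Renegade Jammer vehicle game, handling input setup, pause menu, end-of-game cleanup and gamepad vibration.
; On BeginPlay it binds win/lose events from the default or tutorial game mode, adds the vehicle mapping context and async-loads force feedback effects.
; Pause opens WBP_Pause only mid-game, switching input mode and restoring it on close.
; Vibration events play drift, green boost and object-destroyed effects; a noted first-play hitch persists despite async loading.
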(event Custom|On%20Game%20Lost
  (Pawn|UnPossess)
  (CallFunction|StopDriftingVibration)
  (CallFunction|StopGreenBoostVibration)
  (Variables|Default|SetbShowMouseCursor true)
  (bind _returnvalue (Actor|GetActorOfClass "/Game/RenegadeJammer/Core/Characters/Jammer/BP_Jammer.BP_Jammer_C"))
  (Default|ConfigureAudio (Variables|/Game/RenegadeJammer/Core/Characters/Jammer/BP_Jammer.BP_Jammer_C|GetAudioComponent _returnvalue) "NewEnumerator1"))

(event Custom|On%20Game%20Won
  (params (FinalTime :type String) (ObjectsDestroyed :type Integer))
  (bind _returnvalue (Game|Player|GetPlayerPawn 0))
  (Utilities|IsValid _returnvalue
    (:Is%20Valid
      (Actor|DestroyActor _returnvalue))
    (:Is%20Not%20Valid
      _))
  (CallFunction|StopDriftingVibration)
  (CallFunction|StopGreenBoostVibration)
  (Variables|Default|SetbShowMouseCursor true))

(event EventBeginPlay
  (bind _self self)
  (bind _returnvalue (PlayerController|LocalPlayerSubsystems|GetEnhancedInputLocalPlayerSubsystem _self))
  (|CallParentFunction)
  (Utilities|FlowControl|Sequence
    (:then_0
      (bind _asbp_default_game_mode (Utilities|Casting|CastToBP_DefaultGameMode (Game|GetGameMode))
        (:then
          (EventDispatchers|BindEventtoOnGameWon _asbp_default_game_mode (delegate Custom|On%20Game%20Won))
          (EventDispatchers|BindEventtoOnGameLost _asbp_default_game_mode (delegate Custom|On%20Game%20Lost)))
        (:CastFailed
          (bind _asbp_tutorial_game_mode (Utilities|Casting|CastToBP_TutorialGameMode (Game|GetGameMode)))
          (EventDispatchers|BindEventtoOnTutorialWon _asbp_tutorial_game_mode (delegate Custom|On%20Game%20Won))
          (EventDispatchers|AssignOnTutorialLost _asbp_tutorial_game_mode (delegate Custom|On%20Game%20Lost)))))
    (:then_1
      (Input|SetInputModeGameOnly self true)
      (Variables|Default|SetbShowMouseCursor false))
    (:then_2
      (Utilities|IsValid _returnvalue
        (:Is%20Valid
          (Input|AddMappingContext _returnvalue "/Game/RenegadeJammer/Core/Input/IMC_VehicleMappingContext.IMC_VehicleMappingContext" 0 "(bIgnoreAllPressedKeysUntilRelease=True,bForceImmediately=False,bNotifyUserSettings=False)"))))
    (:then_3
      (Utilities|AsyncLoadForceFeedback))))

(event Custom|On%20Pause%20Closed
  (if (not (Variables|/Game/RenegadeJammer/UserInterface/Common/WBP_BaseUserWidget.WBP_BaseUserWidget_C|GetShouldBlockInput (Variables|Default|GetPauseWidget)))
    (Game|SetGamePaused false)
    (CallFunction|SetGameMode)
    (Input|EnableInput (Game|Player|GetPlayerPawn 0) self)
    (Variables|Default|GetPauseWidget
      (:then
        (Variables|Default|SetPauseWidget 0))
      (:else))))

(event Input|EnhancedActionEvents|EnhancedInputActionIA_Pause
  (params (ActionValue :type Boolean) (ElapsedSeconds :type Float%20%28double-precision%29) (TriggeredSeconds :type Float%20%28double-precision%29) (InputAction :type Input%20Action%20Object%20Reference :default "/Game/RenegadeJammer/Core/Input/IA_Pause.IA_Pause"))
  (:Completed
    (CallFunction|ProcessPause (delegate Custom|On%20Pause%20Closed))))

(event EventStopGreenBoostVibration
  ;[1 0.5654 0.09486] There is a problem when playing the force feedback for the first time. Even async loading the asset, game freezes until it completes the loading. After that, the game never freezes again.
  (bind _greenboostforcefeedback (Variables|Default|GetGreenBoostForceFeedback)
    (:then
      (Game|Feedback|ClientStopForceFeedback _greenboostforcefeedback "None"))
    (:else)))

(event EventStartDriftingVibration
  ;[1 0.5654 0.09486] There is a problem when playing the force feedback for the first time. Even async loading the asset, game freezes until it completes the loading. After that, the game never freezes again.
  (bind _driftforcefeedback (Variables|Default|GetDriftForceFeedback)
    (:then
      (Game|Feedback|ClientPlayForceFeedback _driftforcefeedback "None" false false false))
    (:else)))

(event EventStopDriftingVibration
  ;[1 0.5654 0.09486] There is a problem when playing the force feedback for the first time. Even async loading the asset, game freezes until it completes the loading. After that, the game never freezes again.
  (bind _driftforcefeedback (Variables|Default|GetDriftForceFeedback)
    (:then
      (Game|Feedback|ClientStopForceFeedback _driftforcefeedback "None"))
    (:else)))

(event EventPlayonDestroyObjectVibration
  ;[1 0.5654 0.09486] There is a problem when playing the force feedback for the first time. Even async loading the asset, game freezes until it completes the loading. After that, the game never freezes again.
  (bind _onobjectdestroyedforcefeedback (Variables|Default|GetOnObjectDestroyedForceFeedback)
    (:then
      (Game|Feedback|ClientPlayForceFeedback _onobjectdestroyedforcefeedback "None" false false false))
    (:else)))

(event EventStartGreenBoostVibration
  ;[1 0.5654 0.09486] There is a problem when playing the force feedback for the first time. Even async loading the asset, game freezes until it completes the loading. After that, the game never freezes again.
  (bind _greenboostforcefeedback (Variables|Default|GetGreenBoostForceFeedback)
    (:then
      (Game|Feedback|ClientPlayForceFeedback _greenboostforcefeedback "None" true false false))
    (:else)))

(fn ConstructionScript)

(fn AsyncLoadVibrationAsset)

(fn SetGameMode
  (Input|SetInputModeGameOnly self true)
  (Variables|Default|SetbShowMouseCursor false))

(fn SetUIMode
  (params (InWidgetToFocus :type Widget%20Object%20Reference))
  (Input|SetInputModeUIOnly self InWidgetToFocus "DoNotLock" false)
  (Variables|Default|SetbShowMouseCursor true))

(fn ShowPause
  (params (Delegate :type Delegate%20%28by%20ref%29))
  (bind _returnvalue (UserInterface|CreateWidget "/Game/RenegadeJammer/UserInterface/Screens/WBP_Pause.WBP_Pause_C" self))
  (bind _output_get (Variables|Default|SetPauseWidget _returnvalue))
  (UserInterface|Viewport|AddtoViewport _output_get 0)
  (Game|SetGamePaused true)
  (Input|SetInputModeGameandUI self (Default|GetDesiredFocusInput _output_get) "DoNotLock" true false)
  (Input|DisableInput (Game|Player|GetPlayerPawn 0) self)
  (EventDispatchers|BindEventtoOnCustomRemovedfromParent _output_get Delegate))

(fn ProcessPause
  (params (Delegate :type Delegate%20%28by%20ref%29))
  (bind _returnvalue (Game|GetGameMode))
  (bind _isgamewon (Class|BPIDefaultGameMode|HasPlayerWon(Message) _returnvalue))
  (bind _hasgamestarted (Class|BPIDefaultGameMode|HasGameStarted(Message) _returnvalue))
  (if (and _hasgamestarted (not _isgamewon))
    (bind _pausewidget (Variables|Default|GetPauseWidget)
      (:then
        (if (not (Variables|/Game/RenegadeJammer/UserInterface/Common/WBP_BaseUserWidget.WBP_BaseUserWidget_C|GetShouldBlockInput (Variables|Default|GetPauseWidget)))
          (Default|RemovefromParentandRemoveMappingContext _pausewidget)))
      (:else
        (CallFunction|ShowPause Delegate)))))