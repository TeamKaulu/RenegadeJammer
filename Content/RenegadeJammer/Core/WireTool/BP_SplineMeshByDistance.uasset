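; Wire tool actor that builds a wire or cable along an editable spline in its construction script, with no runtime logic.
; Each pair of neighboring points gets a spline mesh with configurable mesh, forward axis and thickness in centimeters.
; Tangents keep the spline's direction but scale with straight-line point distance and a multiplier.
; A dynamic material per segment scales YTiling by that same distance to account for segment length.
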(event EventBeginPlay)

(event Collision|EventActorBeginOverlap
  (params (OtherActor :type Actor%20Object%20Reference)))

(event EventTick
  (params (DeltaSeconds :type Float%20%28single-precision%29)))

(fn ConstructionScript
  (bind _spline (Variables|Default|GetSpline))
  (bind _wiresizecm (Variables|Default|GetWireSizeCM))
  (bind _tangentlengthmult (Variables|Default|GetTangentLengthMult))
  (bind _returnvalue (/ _wiresizecm 1e+02))
  (bind _returnvalue_2 (Math|Vector2D|MakeVector2D _returnvalue _returnvalue))
  (for _index (range 0 (- (Spline|GetNumberOfSplinePoints (Variables|Default|GetSpline)) 2))
    (bind _returnvalue_3 (AddComponent|AddSplineMeshComponent false))
    (SplineMesh|SetStartandEnd _returnvalue_3 (.Location (Spline|GetLocationandTangentatSplinePoint _spline _index "Local")) (* (Math|Vector|Normalize (.Tangent (Spline|GetLocationandTangentatSplinePoint _spline _index "Local"))) (Math|Vector|VectorLength (- (.Location (Spline|GetLocationandTangentatSplinePoint _spline _index "Local")) (.Location (Spline|GetLocationandTangentatSplinePoint _spline (+ _index 1) "Local")))) _tangentlengthmult) (.Location (Spline|GetLocationandTangentatSplinePoint _spline (+ _index 1) "Local")) (* (Math|Vector|Normalize (.Tangent (Spline|GetLocationandTangentatSplinePoint _spline (+ _index 1) "Local"))) (Math|Vector|VectorLength (- (.Location (Spline|GetLocationandTangentatSplinePoint _spline _index "Local")) (.Location (Spline|GetLocationandTangentatSplinePoint _spline (+ _index 1) "Local")))) _tangentlengthmult) true :!class /Script/Engine.SplineMeshComponent)
    (SplineMesh|SetForwardAxis _returnvalue_3 (Variables|Default|GetForward%20Axis) true)
    (SplineMesh|SetStartScale _returnvalue_3 _returnvalue_2 true :!class /Script/Engine.SplineMeshComponent)
    (SplineMesh|SetEndScale _returnvalue_3 _returnvalue_2 true :!class /Script/Engine.SplineMeshComponent)
    (Components|StaticMesh|SetStaticMesh _returnvalue_3 (Variables|Default|GetMesh))
    (bind _returnvalue_4 (Rendering|Material|CreateDynamicMaterialInstance _returnvalue_3 0 (Variables|Default|GetWireMaterial) "None" :!class /Script/Engine.PrimitiveComponent))
    (Rendering|Material|SetScalarParameterValue _returnvalue_4 "YTiling" (* (Variables|Default|GetYTilingMultiplier) (Math|Vector|VectorLength (- (.Location (Spline|GetLocationandTangentatSplinePoint _spline _index "Local")) (.Location (Spline|GetLocationandTangentatSplinePoint _spline (+ _index 1) "Local"))))) :!class /Script/Engine.MaterialInstanceDynamic)))