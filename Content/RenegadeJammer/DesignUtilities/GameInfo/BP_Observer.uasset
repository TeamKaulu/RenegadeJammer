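; BP_Observer is a design-utility trigger that reports which direction a player passes through it.
; Two boxes each flip their own boolean whenever an actor implementing BPI_Player ends overlap with them.
; When both booleans match after a flip, it broadcasts a communicate event: BackEvent if Box0 was exited last, ForwardEvent if Box1 was.
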(event OnComponentEndOverlap(Box1)
  (params (OverlappedComponent :type Primitive%20Component%20Object%20Reference) (OtherActor :type Actor%20Object%20Reference) (OtherComp :type Primitive%20Component%20Object%20Reference) (OtherBodyIndex :type Integer))
  (if (Utilities|DoesObjectImplementInterface OtherActor "/Game/RenegadeJammer/Core/Characters/Common/BPI_Player.BPI_Player_C")
    (Variables|Default|SetSwitch1 (not (Variables|Default|GetSwitch1)))
    (if (== (Variables|Default|GetSwitch0) (Variables|Default|GetSwitch1))
      (Default|CallCommunicateEvent (Variables|Default|GetForwardEvent)))))

(event OnComponentEndOverlap(Box0)
  (params (OverlappedComponent :type Primitive%20Component%20Object%20Reference) (OtherActor :type Actor%20Object%20Reference) (OtherComp :type Primitive%20Component%20Object%20Reference) (OtherBodyIndex :type Integer))
  (if (Utilities|DoesObjectImplementInterface OtherActor "/Game/RenegadeJammer/Core/Characters/Common/BPI_Player.BPI_Player_C")
    (Variables|Default|SetSwitch0 (not (Variables|Default|GetSwitch0)))
    (if (== (Variables|Default|GetSwitch0) (Variables|Default|GetSwitch1))
      (Default|CallCommunicateEvent (Variables|Default|GetBackEvent)))))

(event EventBeginPlay)

(event Collision|EventActorBeginOverlap
  (params (OtherActor :type Actor%20Object%20Reference)))

(event EventTick
  (params (DeltaSeconds :type Float%20%28single-precision%29)))

(fn ConstructionScript)