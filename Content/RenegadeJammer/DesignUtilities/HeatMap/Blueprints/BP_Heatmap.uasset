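; BP_Heatmap is a design utility actor that records where the player's BP_Jammer goes as a heatmap texture.
; A looping timer traces down from the player, and hits on this actor become plane-local positions scaled by Resolution.
; Each hit draws a splat material into a runtime render target, then a bake material into a final one.
; ExportResult saves the final target as a JPG under the project directory.
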(event Custom|DrawToRenderTarget
  (params (Location :type Vector) (Strength :type Float%20%28double-precision%29) (Size :type Float%20%28double-precision%29))
  (bind _mid_heatsplat (Variables|Default|GetMID_Heatsplat))
  (Rendering|Material|SetScalarParameterValue _mid_heatsplat "Size" Size :!class /Script/Engine.MaterialInstanceDynamic)
  (Rendering|Material|SetScalarParameterValue _mid_heatsplat "Strength" Strength :!class /Script/Engine.MaterialInstanceDynamic)
  (Rendering|Material|SetVectorParameterValue _mid_heatsplat "Position" (Math|Conversions|ToLinearColor(Vector) (/ (Math|Transform|TransformLocation (Math|Transform|InvertTransform (Transformation|GetWorldTransform (Variables|Default|GetPositionGatheringPlane))) Location) (Variables|Default|GetResolution))) :!class /Script/Engine.MaterialInstanceDynamic)
  (Rendering|DrawMaterialtoRenderTarget (Variables|Default|GetRenderTargetRuntime) _mid_heatsplat)
  (Rendering|DrawMaterialtoRenderTarget (Variables|Default|GetRenderTargetFinal) (Variables|Default|GetMID_Heat)))

(event Custom|Draw
  (bind _playerref (Variables|Default|GetPlayerRef))
  (bind _returnvalue (Transformation|GetActorLocation _playerref))
  (bind (_x _y) (Math|Vector|BreakVector _returnvalue))
  (Utilities|IsValid _playerref
    (:Is%20Valid
      (bind _outhits (Class|KismetSystemLibrary|LineTraceMultiforObjects _returnvalue (Math|Vector|MakeVector _x _y (- (.z (Transformation|GetWorldLocation (Variables|Default|GetPositionGatheringPlane))) 2e+02)) (Utilities|Array|MakeArray "ObjectTypeQuery1" "ObjectTypeQuery2") false 0 "ForDuration" false "(R=1.000000,G=0.000000,B=0.000000,A=1.000000)" "(R=0.000000,G=1.000000,B=0.000000,A=1.000000)" 1.0))
      (for _array_element _outhits
        (if (== (.HitActor (Collision|BreakHitResult _array_element)) self)
          (CallFunction|DrawtoRenderTarget (.Location (Collision|BreakHitResult _array_element)) 2.0 0.012))))))

(event EventBeginPlay
  (Utilities|FlowControl|Delay 0.2)
  (bind _returnvalue (Actor|GetActorOfClass "/Game/RenegadeJammer/Core/Characters/Jammer/BP_Jammer.BP_Jammer_C"))
  (Variables|Default|SetPlayerRef _returnvalue)
  (Rendering|ClearRenderTarget2D "/Game/RenegadeJammer/DesignUtilities/HeatMap/Renders/RT_HeatmapRuntime.RT_HeatmapRuntime")
  (Utilities|Time|SetTimerbyEvent (delegate Custom|Draw) 0.2 true true))

(event Collision|EventActorBeginOverlap
  (params (OtherActor :type Actor%20Object%20Reference)))

(fn ConstructionScript
  (bind _returnvalue (Rendering|Material|CreateDynamicMaterialInstance "/Game/RenegadeJammer/DesignUtilities/HeatMap/Materials/M_HeatSplat.M_HeatSplat" "None" "None" :!class /Script/Engine.KismetMaterialLibrary))
  (Variables|Default|SetMID_Heatsplat _returnvalue)
  (bind _returnvalue_2 (Rendering|Material|CreateDynamicMaterialInstance "/Game/RenegadeJammer/DesignUtilities/HeatMap/Materials/M_HeatmapBake.M_HeatmapBake" "None" "None" :!class /Script/Engine.KismetMaterialLibrary))
  (Variables|Default|SetMID_Heat _returnvalue_2))

(fn ExportResult
  (Class|ImageWriteBlueprintLibrary|ExporttoDisk (Variables|Default|GetRenderTargetFinal) (Utilities|String|Append (Class|KismetSystemLibrary|GetProjectDirectory) "DesignUtilities/Heatmap") (Utilities|Struct|MakeImageWriteOptions "JPG" "(null).None")))