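; BP_TemporaryPlatform02 is a test-map platform that can vanish after BP_Jammer enters its trigger.
; When the Disappear flag is set, entering waits for Time, then hides the Platform and turns off its collision.
; Leaving the trigger restores visibility and collision immediately, but does not cancel a pending delay, so the platform can still vanish afterwards.
; Both overlap events print debug strings.
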(event OnComponentBeginOverlap(Trigger)
  (params (OverlappedComponent :type Primitive%20Component%20Object%20Reference) (OtherActor :type Actor%20Object%20Reference) (OtherComp :type Primitive%20Component%20Object%20Reference) (OtherBodyIndex :type Integer) (bFromSweep :type Boolean) (SweepResult :type Hit%20Result%20Structure%20%28by%20ref%29))
  (if (and (.bSuccess (Utilities|Casting|CastToBP_Jammer OtherActor)) (Variables|Default|GetDisappear))
    (Development|PrintString "in")
    (Utilities|FlowControl|Delay (Variables|Default|GetTime))
    (Rendering|SetVisibility (Variables|Default|GetPlatform) false false)
    (Collision|SetCollisionEnabled (Variables|Default|GetPlatform) "NoCollision")))

(event OnComponentEndOverlap(Trigger)
  (params (OverlappedComponent :type Primitive%20Component%20Object%20Reference) (OtherActor :type Actor%20Object%20Reference) (OtherComp :type Primitive%20Component%20Object%20Reference) (OtherBodyIndex :type Integer))
  (if (and (.bSuccess (Utilities|Casting|CastToBP_Jammer OtherActor)) (Variables|Default|GetDisappear))
    (Development|PrintString "out")
    (Rendering|SetVisibility (Variables|Default|GetPlatform) true false)
    (Collision|SetCollisionEnabled (Variables|Default|GetPlatform) "QueryAndPhysics")))

(event EventBeginPlay)

(event Collision|EventActorBeginOverlap
  (params (OtherActor :type Actor%20Object%20Reference)))

(event EventTick
  (params (DeltaSeconds :type Float%20%28single-precision%29)))

(fn ConstructionScript)