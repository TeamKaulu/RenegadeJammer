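; BP_TimerFloatingRamp is a placeable floating ramp that vanishes after a player stays on it too long, then returns.
; A BPI_Player actor entering the Box while the ramp is active starts a countdown, and leaving clears it.
; When the countdown ends, Disappear turns off mesh collision, toggles visibility and schedules Respawn after RespawnTime.
; Respawn calls Appear to restore collision, toggle visibility back and reactivate the ramp.
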(event OnComponentEndOverlap(Box)
  (params (OverlappedComponent :type Primitive%20Component%20Object%20Reference) (OtherActor :type Actor%20Object%20Reference) (OtherComp :type Primitive%20Component%20Object%20Reference) (OtherBodyIndex :type Integer))
  (if (Utilities|DoesObjectImplementInterface OtherActor "/Game/RenegadeJammer/Core/Characters/Common/BPI_Player.BPI_Player_C")
    (Utilities|Time|ClearandInvalidateTimerbyHandle (Variables|Default|GetTimerHandle))))

(event OnComponentBeginOverlap(Box)
  (params (OverlappedComponent :type Primitive%20Component%20Object%20Reference) (OtherActor :type Actor%20Object%20Reference) (OtherComp :type Primitive%20Component%20Object%20Reference) (OtherBodyIndex :type Integer) (bFromSweep :type Boolean) (SweepResult :type Hit%20Result%20Structure%20%28by%20ref%29))
  (if (and (Variables|Default|GetIsActive) (Utilities|DoesObjectImplementInterface OtherActor "/Game/RenegadeJammer/Core/Characters/Common/BPI_Player.BPI_Player_C"))
    (bind _returnvalue (Utilities|Time|SetTimerbyEvent (delegate Custom|DisappearEvent) (Variables|Default|GetTime)))
    (Variables|Default|SetTimerHandle _returnvalue)))

(event Custom|DisappearEvent
  (CallFunction|Disappear (delegate Custom|Respawn)))

(event Custom|Respawn
  (CallFunction|Appear))

(fn ConstructionScript)

(fn Disappear
  (params (Delegate :type Delegate))
  (bind _staticmesh (Variables|Default|GetStaticMesh))
  (Variables|Default|SetIsActive false)
  (Collision|SetCollisionEnabled _staticmesh "NoCollision")
  (Rendering|ToggleVisibility _staticmesh false)
  (Utilities|Time|SetTimerbyEvent Delegate (Variables|Default|GetRespawnTime)))

(fn Appear
  (bind _staticmesh (Variables|Default|GetStaticMesh))
  (Variables|Default|SetIsActive true)
  (Collision|SetCollisionEnabled _staticmesh "QueryAndPhysics")
  (Rendering|ToggleVisibility _staticmesh false))