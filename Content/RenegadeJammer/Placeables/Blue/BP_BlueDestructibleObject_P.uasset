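; Blue destructible placeable object that adds a continuously spinning hoop to the behavior it inherits from its parent Blueprint.
; After the parent BeginPlay runs, a fast looping timer applies a small local rotation to the Hoop component on two axes, in place of Tick.
; This file holds no destruction logic of its own, and the construction script only calls the parent.
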(event Custom|HoopRotate
  ;[1 1 1] Rotate Hoop
  (Transformation|AddLocalRotation (Variables|Default|GetHoop) "-1.000000,1.000000,0.000000" false false))

(event EventBeginPlay
  (|CallParentFunction)
  ;[1 1 1] Rotate Hoop
  (Utilities|Time|SetTimerbyEvent (delegate Custom|HoopRotate) 0.01 true))

(event Collision|EventActorBeginOverlap
  (params (OtherActor :type Actor%20Object%20Reference))
  (|CallParentFunction OtherActor) ; This node is disabled and will not be called.\nDrag off pins to build functionality.
)

(event EventTick
  (params (DeltaSeconds :type Float%20%28single-precision%29))
  (|CallParentFunction DeltaSeconds) ; This node is disabled and will not be called.\nDrag off pins to build functionality.
)

(fn ConstructionScript
  (|CallParentFunction))