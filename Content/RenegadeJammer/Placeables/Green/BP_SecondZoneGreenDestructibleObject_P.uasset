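; Green second-zone destructible object placeable that adds a constant spin to its Sphere component.
; On BeginPlay it runs the parent logic, then starts a fast looping timer that applies a small local rotation to the sphere, independent of Tick.
; It contains no destruction logic of its own, and its construction script only calls the parent.
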(event Custom|RotateSphere
  ;[1 1 1] Rotate Sphere
  (Transformation|AddLocalRotation (Variables|Default|GetSphere) "0.000000,-0.300000,0.000000" false false))

(event EventBeginPlay
  (|CallParentFunction)
  ;[1 1 1] Rotate Sphere
  (Utilities|Time|SetTimerbyEvent (delegate Custom|RotateSphere) 0.01 true))

(event Collision|EventActorBeginOverlap
  (params (OtherActor :type Actor%20Object%20Reference))
  (|CallParentFunction OtherActor) ; This node is disabled and will not be called.\nDrag off pins to build functionality.
)

(event EventTick
  (params (DeltaSeconds :type Float%20%28single-precision%29))
  (|CallParentFunction DeltaSeconds) ; This node is disabled and will not be called.\nDrag off pins to build functionality.
)

(fn ConstructionScript
  (|CallParentFunction))