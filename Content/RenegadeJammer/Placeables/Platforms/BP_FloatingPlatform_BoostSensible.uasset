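; Floating platform that is solid or passable depending on how the current boost state compares to its required boost.
; The construction script sets the initial material, and boost-state events toggle collision, with yellow and blue also swapping materials; green always counts as correct.
; Restoring collision waits on a timer re-check while a BP_Jammer overlaps the platform.
; The older overlap-driven Disappear logic is disconnected.
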(event Custom|Disappear
  (Collision|SetCollisionEnabled (Variables|Default|GetPlatform) "NoCollision")
  (Utilities|FlowControl|Delay (Variables|Default|GetDisappearTime))
  (Collision|SetCollisionEnabled (Variables|Default|GetPlatform) "QueryAndPhysics"))

(event EventBeginPlay
  (|CallParentFunction) ; This node is disabled and will not be called.\nDrag off pins to build functionality.
)

(event Collision|EventActorBeginOverlap
  (params (OtherActor :type Actor%20Object%20Reference)))

(event EventTick
  (params (DeltaSeconds :type Float%20%28single-precision%29))
  (|CallParentFunction DeltaSeconds) ; This node is disabled and will not be called.\nDrag off pins to build functionality.
)

(event EventReacttoNoBoostState
  (if (== (Variables|Default|GetBoostRequired) 0)
    (CallFunction|ReacttoCorrectBoost)
    (else
      (CallFunction|ReacttoWrongBoost))))

(event EventReacttoBlueState
  (if (== (Variables|Default|GetBoostRequired) 2)
    (CallFunction|ReacttoCorrectBoost)
    ;[1 1 1] Update Hologram material to opaque
    (Rendering|Material|SetMaterial (Variables|Default|GetPlatform) 0 "/Game/RenegadeJammer/Art/Industrial/Zone02/Ramps/SideBowlFloatingRamp/MI_SideBowlFloatingRampBlue.MI_SideBowlFloatingRampBlue")
    (else
      (CallFunction|ReacttoWrongBoost)
      (Rendering|Material|SetMaterial (Variables|Default|GetPlatform) 0 "/Game/RenegadeJammer/Art/Industrial/Zone02/Ramps/SideBowlFloatingRamp/MI_SideBowlFloatingRampYellowTrans.MI_SideBowlFloatingRampYellowTrans"))))

(event EventReacttoYellowState
  (bind _platform (Variables|Default|GetPlatform))
  (if (== (Variables|Default|GetBoostRequired) 1)
    (CallFunction|ReacttoCorrectBoost)
    ;[1 1 1] Update Hologram material to opaque
    ;;[1 1 1] Check if is Floating Ramp or Curve Ramp
    (if (Utilities|Enum|Equal(Enum) (Variables|Default|GetPlatformType) "NewEnumerator0")
      (Rendering|Material|SetMaterial _platform 0 "/Game/RenegadeJammer/Art/Industrial/Zone02/Ramps/FloatingRamp/MI_FloatingRampYellowOpaque.MI_FloatingRampYellowOpaque")
      (else
        (Rendering|Material|SetMaterial _platform 0 "/Game/RenegadeJammer/Art/Industrial/Zone02/Ramps/SideBowlFloatingRamp/MI_SideBowlFloatingRampYellow.MI_SideBowlFloatingRampYellow")))
    (else
      (CallFunction|ReacttoWrongBoost)
      (Rendering|Material|SetMaterial (Variables|Default|GetPlatform) 0 "/Game/RenegadeJammer/Art/Industrial/Zone02/Ramps/SideBowlFloatingRamp/MI_SideBowlFloatingRampBlueTrans.MI_SideBowlFloatingRampBlueTrans"))))

(event EventReacttoGreenState
  (CallFunction|ReacttoCorrectBoost))

(fn ConstructionScript
  (bind _platform (Variables|Default|GetPlatform))
  (|CallParentFunction)
  (switch Utilities|FlowControl|Switch|SwitchonE_BoostStateEnum (Variables|Default|GetBoostRequired)
    (:NewEnumerator1
      ;[1 1 1] Check if is Floating Ramp or Curve Ramp
      (if (Utilities|Enum|Equal(Enum) (Variables|Default|GetPlatformType) "NewEnumerator0")
        (Rendering|Material|SetMaterial _platform 0 "/Game/RenegadeJammer/Art/Industrial/Zone02/Ramps/FloatingRamp/MI_FloatingRampYellowTrans.MI_FloatingRampYellowTrans")
        (else
          (Rendering|Material|SetMaterial _platform 0 "/Game/RenegadeJammer/Art/Industrial/Zone02/Ramps/SideBowlFloatingRamp/MI_SideBowlFloatingRampYellowTrans.MI_SideBowlFloatingRampYellowTrans"))))
    (:NewEnumerator2
      (Rendering|Material|SetMaterial _platform 0 "/Game/RenegadeJammer/Art/Industrial/Zone02/Ramps/SideBowlFloatingRamp/MI_SideBowlFloatingRampBlueTrans.MI_SideBowlFloatingRampBlueTrans"))
    (:NewEnumerator3
      (Rendering|Material|SetMaterial _platform 0 "/Game/RenegadeJammer/MaterialLibrary/Debug/M_GreenBoostMaterial.M_GreenBoostMaterial"))))

(fn ReacttoCorrectBoost
  (if (> (Utilities|Array|Length (Collision|GetOverlappingActors (Variables|Default|GetPlatform) "/Game/RenegadeJammer/Core/Characters/Jammer/BP_Jammer.BP_Jammer_C" :!class /Script/Engine.PrimitiveComponent)) 0)
    (Utilities|FlowControl|DoOnce false :!label _label
      (:Completed
        (bind _returnvalue (Utilities|Time|SetTimerbyFunctionName 0 "ReactToCorrectBoost" 0.0))
        (Variables|Default|SetComproveJammerOverlapHandle _returnvalue)))
    (else
      (if (and (Utilities|Time|IsValidTimerHandle (Variables|Default|GetComproveJammerOverlapHandle)) (Utilities|Time|IsTimerActivebyHandle (Variables|Default|GetComproveJammerOverlapHandle)))
        (Utilities|Time|ClearandInvalidateTimerbyHandle (Variables|Default|GetComproveJammerOverlapHandle)))
      (Collision|SetCollisionEnabled (Variables|Default|GetPlatform) "QueryAndPhysics")
      (goto _label Reset))))

(fn ReacttoWrongBoost
  (bind _comprovejammeroverlaphandle (Variables|Default|GetComproveJammerOverlapHandle))
  (if (and (Utilities|Time|IsValidTimerHandle _comprovejammeroverlaphandle) (Utilities|Time|IsTimerActivebyHandle _comprovejammeroverlaphandle))
    (Utilities|Time|ClearandInvalidateTimerbyHandle (Variables|Default|GetComproveJammerOverlapHandle)))
  (Collision|SetCollisionEnabled (Variables|Default|GetPlatform) "NoCollision"))