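; Rotating platform placeable for Zone 3 that swings back and forth around its yaw axis.
; A looping timer, rather than Tick, polls the actor's yaw and reverses RotatingMovement's rate past plus or minus MaxRot, with Sign tracking direction.
; An instanced static mesh starts hidden, and ActivateAccess reveals it along with its children and prints a debug message.
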(event Custom|CheckRotate
  (bind _returnvalue (Transformation|GetActorRotation))
  (bind _rotatingmovement (Variables|Default|GetRotatingMovement))
  (if (> (Variables|Default|GetSign) 0)
    (if (> (.yaw _returnvalue) (Variables|Default|GetMaxRot))
      (Variables|/Script/Engine.RotatingMovementComponent|SetRotationRate _rotatingmovement (* (Variables|/Script/Engine.RotatingMovementComponent|GetRotationRate _rotatingmovement) -1.0))
      (Variables|Default|SetSign (* (Variables|Default|GetSign) -1)))
    (elif (< (.yaw _returnvalue) (* (Variables|Default|GetMaxRot) -1))
      (Variables|/Script/Engine.RotatingMovementComponent|SetRotationRate _rotatingmovement (* (Variables|/Script/Engine.RotatingMovementComponent|GetRotationRate _rotatingmovement) -1.0))
      (Variables|Default|SetSign (* (Variables|Default|GetSign) -1)))))

(event EventBeginPlay
  (Rendering|SetVisibility (Variables|Default|GetInstancedStaticMesh1) false false)
  (Utilities|Time|SetTimerbyEvent (delegate Custom|CheckRotate) 1.0 true))

(event Collision|EventActorBeginOverlap
  (params (OtherActor :type Actor%20Object%20Reference)))

(event EventTick
  (params (DeltaSeconds :type Float%20%28single-precision%29)))

(fn ConstructionScript)

(fn ActivateAccess
  (Rendering|SetVisibility (Variables|Default|GetInstancedStaticMesh1) true true)
  (Development|PrintString "Activated" true true "(R=1.000000,G=0.000000,B=0.141483,A=1.000000)"))